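; Knight character Blueprint that handles player input events and uses the Gameplay Ability System.
; On BeginPlay it adds the IMC_Basic Enhanced Input context, then after a short delay sends current and max health attributes to its controller for display.
; Special attack activates GA_WaterBuuurst through the Ability System Component.
; Taunt, basic attack, ultimate and dash only print debug strings, and move is empty.
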(event EventOnMove)

(event EventOnTaunt
  (Development|PrintString "Taunt"))

(event EventOnBasicAttack
  (Development|PrintString "Basic attack"))

(event EventOnSpecialAttack
  (Development|PrintString "Specialattack")
  (Abilities|TryActivateAbilitybyClass (Variables|Default|GetAbilitySystemComponent) "/Game/Programming/Blueprints/GA_WaterBuuurst.GA_WaterBuuurst_C" true))

(event EventOnUltimateAttack
  (Development|PrintString "Ultiamte attack"))

(event EventOnDash
  (Development|PrintString "Dash"))

(event EventBeginPlay
  (bind _abilitysystemcomponent (Variables|Default|GetAbilitySystemComponent))
  (bind _asplayer_controller (Utilities|Casting|CastToPlayerController (Pawn|GetController)))
  (Input|AddMappingContext (PlayerController|LocalPlayerSubsystems|GetEnhancedInputLocalPlayerSubsystem _asplayer_controller) "/Game/Characters/Input/IMC_Basic.IMC_Basic" 0 "(bIgnoreAllPressedKeysUntilRelease=True,bForceImmediately=False,bNotifyUserSettings=False)")
  (Utilities|FlowControl|Delay 0.2)
  (Class|BPIStats|UpdateHealthDisplay(Message) (Pawn|GetController) (.ReturnValue (Class|AbilitySystemComponent|GetGameplayAttributeValue _abilitysystemcomponent "(AttributeName=\"Health\",Attribute=/Script/Proj.RushAttributeSet:Health,AttributeOwner=\"/Script/CoreUObject.Class'/Script/Proj.RushAttributeSet'\")")) (.ReturnValue (Class|AbilitySystemComponent|GetGameplayAttributeValue _abilitysystemcomponent "(AttributeName=\"MaxHealth\",Attribute=/Script/Proj.RushAttributeSet:MaxHealth,AttributeOwner=\"/Script/CoreUObject.Class'/Script/Proj.RushAttributeSet'\")"))))

(fn ConstructionScript)