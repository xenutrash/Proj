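; Playable Plague Doctor character for a 3vs1 mode, using the Gameplay Ability System.
; Basic, special and dash inputs activate the Powder Bomb, Smelling Salts and Dash abilities; ultimate only prints and reports the player dead, while taunt just prints.
; Health changes route through the server, which triggers the client HUD update via the player controller and checks for death.
; Death notifies GM_3vs1 and disables local input.
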(event Custom|Check%20If%20Dead
  (params (Health :type Float%20%28double-precision%29))
  (if (not (Variables|Default|GetIsDead))
    (if (<= Health 0.0)
      (Variables|Default|SetIsDead true)
      (bind _asgm_3vs_1 (Utilities|Casting|CastToGM_3vs1 (Game|GetGameMode)))
      (Default|PlayerDied _asgm_3vs_1 self)
      (CallFunction|DisableController))))

(event Custom|Server%20On%20Health%20Changed
  (Networking|SwitchHasAuthority
    (:Authority
      (Utilities|FlowControl|Sequence
        (:then_0
          (CallFunction|ClientonHealthChanged))
        (:then_1
          (CallFunction|CheckifDead (.ReturnValue (Class|AbilitySystemComponent|GetGameplayAttributeValue (Variables|Default|GetAbilitySystemComponent) "(AttributeName=\"Health\",Attribute=/Script/Proj.RushAttributeSet:Health,AttributeOwner=\"/Script/CoreUObject.Class'/Script/Proj.RushAttributeSet'\")"))))))))

(event Custom|Client%20On%20Health%20Changed
  (bind _abilitysystemcomponent (Variables|Default|GetAbilitySystemComponent))
  (bind _returnvalue (Class|AbilitySystemComponent|GetGameplayAttributeValue _abilitysystemcomponent "(AttributeName=\"Health\",Attribute=/Script/Proj.RushAttributeSet:Health,AttributeOwner=\"/Script/CoreUObject.Class'/Script/Proj.RushAttributeSet'\")"))
  (bind _returnvalue_2 (Class|AbilitySystemComponent|GetGameplayAttributeValue _abilitysystemcomponent "(AttributeName=\"MaxHealth\",Attribute=/Script/Proj.RushAttributeSet:MaxHealth,AttributeOwner=\"/Script/CoreUObject.Class'/Script/Proj.RushAttributeSet'\")"))
  (bind _asbp_proj_player_controller (Utilities|Casting|CastToBP_ProjPlayerController (Game|GetPlayerController 0)))
  (Default|HealthChanged _asbp_proj_player_controller (Utilities|Text|FormatText "Health {0} / {1}" _returnvalue _returnvalue_2) (/ _returnvalue _returnvalue_2)))

(event Custom|Disable%20controller
  (bind _returnvalue (Pawn|GetLocalViewingPlayerController))
  (Utilities|IsValid _returnvalue
    (:Is%20Valid
      (if (Pawn|IsLocalController _returnvalue)
        (Input|DisableInput self _returnvalue)))))

(event EventOnMove)

(event EventOnTaunt
  (Development|PrintString "Taunt"))

(event EventOnBasicAttack
  (Development|PrintString "Basic attack")
  (Abilities|TryActivateAbilitybyClass (Variables|Default|GetAbilitySystemComponent) "/Game/Programming/Blueprints/PlagueDoctor/PowderBomb/GA_PowderBomb.GA_PowderBomb_C" true))

(event EventOnSpecialAttack
  (Development|PrintString "Specialattack")
  (Abilities|TryActivateAbilitybyClass (Variables|Default|GetAbilitySystemComponent) "/Game/Programming/Blueprints/PlagueDoctor/SmellingSalts/GA_SmellingSalts.GA_SmellingSalts_C" true))

(event EventOnUltimateAttack
  (Development|PrintString "Ultiamte attack")
  (bind _asgm_3vs_1 (Utilities|Casting|CastToGM_3vs1 (Game|GetGameMode)))
  (Default|PlayerDied _asgm_3vs_1 self))

(event EventOnHealthChanged
  (params (DeltaValue :type Float%20%28single-precision%29) (EventTags :type Gameplay%20Tag%20Container%20Structure%20%28by%20ref%29))
  (CallFunction|ServeronHealthChanged))

(event EventOnDash
  (Development|PrintString "Dash")
  (Abilities|TryActivateAbilitybyClass (Variables|Default|GetAbilitySystemComponent) "/Game/Programming/Blueprints/GA_Dash.GA_Dash_C" true))

(event EventBeginPlay
  (bind _returnvalue (UserInterface|CreateWidget "/Game/Programming/Blueprints/WBP_Stats.WBP_Stats_C"))
  (Variables|Default|SetHealth%20Widget _returnvalue))

(fn ConstructionScript)

(fn UpdateHealthGUI
  (bind _abilitysystemcomponent (Variables|Default|GetAbilitySystemComponent))
  (bind _returnvalue (Class|AbilitySystemComponent|GetGameplayAttributeValue _abilitysystemcomponent "(AttributeName=\"Health\",Attribute=/Script/Proj.RushAttributeSet:Health,AttributeOwner=\"/Script/CoreUObject.Class'/Script/Proj.RushAttributeSet'\")"))
  (bind _returnvalue_2 (Class|AbilitySystemComponent|GetGameplayAttributeValue _abilitysystemcomponent "(AttributeName=\"MaxHealth\",Attribute=/Script/Proj.RushAttributeSet:MaxHealth,AttributeOwner=\"/Script/CoreUObject.Class'/Script/Proj.RushAttributeSet'\")"))
  (Default|UpdateHealth (Variables|Default|GetWidget%20Ref) (/ _returnvalue _returnvalue_2) (Utilities|Text|FormatText "Health {0} / {1}" _returnvalue _returnvalue_2)))