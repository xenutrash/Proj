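; Training-mode game mode that lets players swap between characters and keeps them from staying dead.
; BeginPlay pre-spawns every DT_CharacaterInfo character at the BP_SpawnFloor point into CachedPlayers; PostLogin possesses the default and registers the player with game state and HUD.
; ChangeCharacter possesses the cached pawn and moves it to the spawn point, while PlayerDied refills health.
; Boss-versus-heroes match logic (countdown, circle, end game, spectator camera) remains but is mostly disconnected.
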(event Custom|Player%20Died
  (params (ActorThatDied :type Actor%20Object%20Reference) (Controller :type BP%20Proj%20Player%20Controller%20Object%20Reference))
  ;[1 1 1] Checks who died and checks if it needs to end the game
  (bind _asbp_rush_character (Utilities|Casting|CastToBP_RushCharacter ActorThatDied))
  (Variables|/Script/Proj.RushAttributeSet|SetHealth (Class|RushCharacter|GetAttributeSet _asbp_rush_character) (Variables|/Script/Proj.RushAttributeSet|GetMaxHealth (Class|RushCharacter|GetAttributeSet _asbp_rush_character))))

(event Custom|End%20Game
  (params (Winner :type String))
  ;[1 1 1] Ends the game
)

(event Custom|StartCircle
  ;[1 1 1] Start the circle with time interval
)

(event Custom|StartCricle
  ;[1 1 1] Start the circle with time interval
)

(event Custom|Find%20Spectator%20Camera
  ;[1 1 1] Find the spectator camera
)

(event Custom|StartCountdown
  ;[1 1 1] Start countdown for match begin
  (bind _ended (CallFunction|UpdateCountdown))
  (if _ended
    _))

(event Custom|SetCamera
  (params (Target :type Player%20Controller%20Object%20Reference)))

(event Custom|ChangeCharacter
  (params (Controller :type BP%20Proj%20Player%20Controller%20Object%20Reference) (CharacterName :type Name))
  (bind _returnvalue (Pawn|GetControlledPawn Controller))
  (bind _cachedplayers (Variables|Default|GetCachedPlayers))
  (bind _value (Utilities|Map|Find _cachedplayers CharacterName))
  (Transformation|SetActorTransform _value (Transformation|GetActorTransform _returnvalue))
  (Pawn|Possess Controller _value)
  (Transformation|SetActorTransform _returnvalue (Transformation|GetWorldTransform (Variables|/Game/Programming/TraningMode/Objects/BP_SpawnFloor.BP_SpawnFloor_C|GetSpawnPoint (Variables|Default|GetSpawnPoint)))))

(event EventBeginPlay
  (bind _returnvalue (Actor|GetActorOfClass "/Game/Programming/TraningMode/Objects/BP_SpawnFloor.BP_SpawnFloor_C"))
  (Variables|Default|SetSpawnPoint _returnvalue)
  (bind _outrownames (DataTable|GetDataTableRowNames "/Game/Programming/Blueprints/DataStructs/DT_CharacaterInfo.DT_CharacaterInfo"))
  (for _array_element _outrownames
    (CallFunction|SpawnCharacter _array_element _array_element (Transformation|GetWorldTransform (Variables|/Game/Programming/TraningMode/Objects/BP_SpawnFloor.BP_SpawnFloor_C|GetSpawnPoint _returnvalue)))))

(event EventOnPlayersSpawned
  (params (GameModeSettings :type Game%20Mode%20Settings%20Structure%20%28by%20ref%29)))

(event EventOnSpawnPlayer
  (params (Controller :type Player%20Controller%20Object%20Reference) (PlayerInfo :type Connected%20Player%20Structure%20%28by%20ref%29) (GameModeSettings :type Game%20Mode%20Settings%20Structure%20%28by%20ref%29)))

(event EventPostLogin
  (params (NewPlayer :type Player%20Controller%20Object%20Reference))
  (bind _defaultcharacter (Variables|Default|GetDefaultCharacter))
  (Pawn|Possess NewPlayer (.Value (Utilities|Map|Find (Variables|Default|GetCachedPlayers) _defaultcharacter)))
  (CallFunction|PostSpawn NewPlayer NewPlayer _defaultcharacter))

(fn ConstructionScript)

(fn CreateEndGameWidget
  (params (NewParam :type String))
  (for _array_element (Variables|/Script/Engine.GameStateBase|GetPlayerArray (Game|GetGameState))
    (bind _asbp_proj_player_controller (Utilities|Casting|CastToBP_ProjPlayerController (Game|GetPlayerController _array_element)))
    (Default|EndGame _asbp_proj_player_controller NewParam)))

(fn RemoveLoadingScreenWidget
  (for _array_element (Variables|/Script/Engine.GameStateBase|GetPlayerArray (Game|GetGameState))
    (bind _asbp_proj_player_controller (Utilities|Casting|CastToBP_ProjPlayerController (Game|GetPlayerController _array_element)))
    (bind _asafgi_instance (Utilities|Casting|CastToAFGI_Instance (Game|GetGameInstance)))
    (Default|SetHudIConsEvent _asbp_proj_player_controller (.SelectedCharacter (Utilities|Struct|BreakConnectedPlayer (Class|AFGIMain|GetPlayerInfo _asafgi_instance (Game|GetPlayerController _array_element)))) (.SelectedSkin (Utilities|Struct|BreakConnectedPlayer (Class|AFGIMain|GetPlayerInfo _asafgi_instance (Game|GetPlayerController _array_element)))))))

(fn AddPlayerDied
  (params (Actor%20That%20Died :type Actor%20Object%20Reference) (ControllerThatDied :type BP%20Proj%20Player%20Controller%20Object%20Reference))
  (Variables|Default|SetActor%20That%20Died Actor%20That%20Died)
  (Variables|Default|SetControllerThatDied ControllerThatDied)
  (Utilities|Array|Add (Variables|Default|GetPeopleDied) (Variables|Default|GetActor%20That%20Died))
  (Default|DisableAllInput (Variables|Default|GetControllerThatDied) true)
  (if (Actor|ActorHasTag (Variables|Default|GetActor%20That%20Died) "Boss")
    (CallFunction|EndGame "Heroes")
    (else
      (bind _output_get (Variables|Default|SetHeroesDeadCount (+ (Variables|Default|GetHeroesDeadCount) 1)))
      (if (>= _output_get (Variables|Default|GetHeroesMaxDeaths))
        (CallFunction|EndGame "Boss")
        (else
          (bind _returnvalue (Actor|GetActorOfClass "/Game/Programming/Blueprints/BP_BattleMusic.BP_BattleMusic_C"))
          (Default|UpdateIntensity _returnvalue (Math|Conversions|ToFloat(Integer) _output_get)))))))

(fn GetSpawnPoint
  (params (Boss :type Boolean))
  (if (< (Utilities|Array|Length (Variables|Default|GetSpawnPoints)) 1)
    (bind _outactors (Actor|GetAllActorsOfClass "/Script/Engine.PlayerStart"))
    (for (_array_element _array_index) _outactors
      (if Boss
        (if (Actor|ActorHasTag _array_element "BossSpawnpoint")
          (Variables|Default|SetSpawnPoints _outactors :!label _label)
          (LocalVariables|SetReturnValue (Transformation|GetActorTransform (Utilities|Array|Get(acopy) (Variables|Default|GetSpawnPoints) _array_index)))
          (Utilities|Array|RemoveIndex (Variables|Default|GetSpawnPoints) _array_index)
          (return (LocalVariables|GetReturnValue)))
        (elif (not (Actor|ActorHasTag _array_element "BossSpawnpoint"))
          (goto _label))))
    (else
      (LocalVariables|SetReturnValue (Transformation|GetActorTransform (Utilities|Array|Get(acopy) (Variables|Default|GetSpawnPoints) _array_index)))
      (Utilities|Array|RemoveIndex (Variables|Default|GetSpawnPoints) _array_index)
      (return (LocalVariables|GetReturnValue)))))

(fn SlowDownTime
  (params (Time%20Dialation :type Float%20%28single-precision%29))
  (Utilities|Time|SetGlobalTimeDilation Time%20Dialation))

(fn SetSpectatorCamera
  (params (Controller :type Player%20Controller%20Object%20Reference))
  (Game|Player|SetViewTargetwithBlend Controller (Variables|Default|GetSpectatorCamera) 0.5 "VTBlend_Linear" 0.0 false))

(fn UpdateCountdown
  (if (< (Variables|Default|GetCountdown) 1)
    (for _array_element (Variables|Default|GetPlayerControllers)
      (Default|DisableAllInput _array_element false)
      (Default|UpdateCountdown _array_element))
    (return true)
    (else
      (for _array_element_2 (Variables|Default|GetPlayerControllers)
        (Default|UpdateCountdown _array_element_2 (Utilities|Text|ToText(Integer) (Variables|Default|GetCountdown))))
      (Variables|Default|SetCountdown (- (Variables|Default|GetCountdown) 1))
      (return false))))

(fn PostSpawn
  (params (Object :type Object%20Object%20Reference) (self2 :type Controller%20Object%20Reference) (CharacetrName :type Name))
  (bind _asbp_3vs_1game_state (Utilities|Casting|CastToBP_3vs1GameState (Game|GetGameState)))
  (bind _asmythbreak_player_state (Utilities|Casting|CastToMythbreakPlayerState (Variables|/Script/Engine.Controller|GetPlayerState self2)))
  (Default|AddPlayer _asbp_3vs_1game_state _asmythbreak_player_state)
  (bind _asbp_proj_player_controller (Utilities|Casting|CastToBP_ProjPlayerController Object))
  (Default|SetHudIConsEvent _asbp_proj_player_controller CharacetrName "None"))

(fn SpawnCharacter
  (params (RowName :type Name) (Key :type Name%20%28by%20ref%29) (SpawnTransform :type Transform) (Owner :type Actor%20Object%20Reference))
  (bind _returnvalue (Utilities|GetDataTableRow "/Game/Programming/Blueprints/DataStructs/DT_CharacaterInfo.DT_CharacaterInfo" RowName)
    (:then
      (bind _returnvalue_2 (Game|SpawnActorfromClass (.Character (Utilities|Struct|BreakS_CharacterInformastion _returnvalue)) SpawnTransform "AdjustIfPossibleButAlwaysSpawn" "MultiplyWithRoot" Owner 0))
      (Utilities|Map|Add (Variables|Default|GetCachedPlayers) Key _returnvalue_2))))