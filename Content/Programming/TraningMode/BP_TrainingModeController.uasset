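; Player controller for training mode that lets the player pick and swap their character.
; It creates a WBP_CharacterPickerGUI widget at BeginPlay, reuses it, and makes it visible again when H is pressed.
; A ChangeCharacter event forwards the chosen character name to LobbyGameMode, which changes the player's character.
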(event Custom|ChangeCharacter
  (params (NameOfCharacter :type Name))
  (bind _aslobby_game_mode (Utilities|Casting|CastToLobbyGameMode (Game|GetGameMode)))
  (Class|LobbyGameMode|ChangePlayerCharacter _aslobby_game_mode self NameOfCharacter))

(event Custom|Show%20Character%20picker
  (CallFunction|CreateCharacterPickerWidget)
  (if (not (Widget|IsVisible (Variables|Default|GetGUI)))
    (Widget|SetVisibility (Variables|Default|GetGUI) "Visible")))

(event EventBeginPlay
  (|CallParentFunction)
  (CallFunction|CreateCharacterPickerWidget))

(event EventTick
  (params (DeltaSeconds :type Float%20%28single-precision%29))
  (|CallParentFunction DeltaSeconds) ; This node is disabled and will not be called.\nDrag off pins to build functionality.
)

(event Input|KeyboardEvents|H
  (params (Key :type Key%20Structure :default "None"))
  (:Pressed
    (CallFunction|ShowCharacterPicker)))

(fn ConstructionScript
  (|CallParentFunction))

(fn CreateCharacterPickerWidget
  (Utilities|IsValid (Variables|Default|GetGUI)
    (:Is%20Valid
      _)
    (:Is%20Not%20Valid
      (bind _returnvalue (UserInterface|CreateWidget "/Game/Programming/TraningMode/Widgets/WBP_CharacterPickerGUI.WBP_CharacterPickerGUI_C" self))
      (bind _output_get (Variables|Default|SetGUI _returnvalue))
      (UserInterface|Viewport|AddtoViewport _output_get 0)))
  (return (Variables|Default|GetGUI)))