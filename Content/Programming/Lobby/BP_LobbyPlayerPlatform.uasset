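; BP_LobbyPlayerPlatform is a lobby platform that spawns and holds a player's preview character.
; SpawnCharacter links the player controller to the platform, spawns a BP_Lobby_Character at the spawn transform if none exists, and marks the platform occupied.
; ChangeCharacter cycles through DT_Bosses or DT_Heroes rows by character type, wrapping the index and passing each row's mesh to the character's SetMeshOnServer.
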(event Custom|SpawnCharacter
  (params (PC :type PC%20Lobby%20Controller%20Object%20Reference))
  (Development|PrintString "Hello")
  (Default|SetPlayerPlatform PC self)
  (Variables|Default|SetPC PC)
  (Utilities|IsValid (Variables|Default|GetCharacter)
    (:Is%20Not%20Valid
      (bind _returnvalue (Game|SpawnActorfromClass "/Game/Programming/Lobby/BP_Lobby_Character.BP_Lobby_Character_C" (Transformation|GetWorldTransform (Variables|Default|GetPlayerSpawnTransform)) "Undefined" "MultiplyWithRoot" 0 0))
      (Variables|Default|SetCharacter _returnvalue)
      (Variables|Default|SetIsOccupied true))))

(event Custom|ChangeCharacter
  (switch name (Variables|Default|GetCharacterType)
    (:Boss
      (bind _returnvalue (Utilities|GetDataTableRow "/Game/Programming/Lobby/DT_Bosses.DT_Bosses" (Utilities|Array|Get(acopy) (Variables|Default|GetDataTableRowNamesBoss) (Variables|Default|GetCurrentRowIndex)))
        (:then
          (CallFunction|ChangeCharacterVisible (.Mesh (Utilities|Struct|BreakS_Lobby_Characters _returnvalue)))
          (Math|Integer|IncrementInt (Variables|Default|GetCurrentRowIndex)
            (:%20%20
              (if (not (Utilities|Array|IsValidIndex (Variables|Default|GetDataTableRowNamesBoss) (Variables|Default|GetCurrentRowIndex)))
                (Variables|Default|SetCurrentRowIndex 0)))))))
    (:Hero
      (bind _returnvalue_2 (Utilities|GetDataTableRow "/Game/Programming/Lobby/DT_Heroes.DT_Heroes" (Utilities|Array|Get(acopy) (Variables|Default|GetDataTableRowNamesHeroes) (Variables|Default|GetCurrentRowIndex)))
        (:then
          (CallFunction|ChangeCharacterVisible (.Mesh (Utilities|Struct|BreakS_Lobby_Characters _returnvalue_2)))
          (Math|Integer|IncrementInt (Variables|Default|GetCurrentRowIndex)
            (:%20%20
              (if (not (Utilities|Array|IsValidIndex (Variables|Default|GetDataTableRowNamesHeroes) (Variables|Default|GetCurrentRowIndex)))
                (Variables|Default|SetCurrentRowIndex 0)))))))))

(event EventBeginPlay
  (bind _outrownames (DataTable|GetDataTableRowNames "/Game/Programming/Lobby/DT_Bosses.DT_Bosses"))
  (Variables|Default|SetDataTableRowNamesBoss _outrownames)
  (bind _outrownames_2 (DataTable|GetDataTableRowNames "/Game/Programming/Lobby/DT_Heroes.DT_Heroes"))
  (Variables|Default|SetDataTableRowNamesHeroes _outrownames_2)
  (Variables|Default|SetCurrentRowIndex 0))

(fn ConstructionScript)

(fn ChangeCharacterVisible
  (params (NewMesh :type Skeletal%20Mesh%20Object%20Reference))
  (Default|SetMeshonServer (Variables|Default|GetCharacter) NewMesh))