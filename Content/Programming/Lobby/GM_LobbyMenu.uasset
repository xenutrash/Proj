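; Game mode for the lobby menu that registers joining players, seats them on platforms and assigns their roles.
; Each new player is added to the AFGI_Main game instance.
; In the lobby map, after a short delay, lobby controllers are tracked and their pawns teleported to the first free BP_LobbyPlayerPlatform cached at BeginPlay.
; The lobby pawn becomes Boss for the first connected player and Hero for later ones.
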(event EventHandleStartingNewPlayer
  (params (NewPlayer :type Player%20Controller%20Object%20Reference))
  (bind _asafgi_main (Utilities|Casting|CastToAFGI_Main (Game|GetGameInstance)))
  (Default|AddNewPlayer _asafgi_main NewPlayer)
  (|CallParentFunction NewPlayer)
  (bind _returnvalue (Game|GetCurrentLevelName true))
  (switch string _returnvalue
    (:LobbyMenuMap
      (bind _aspc_lobby_controller (Utilities|Casting|CastToPC_LobbyController NewPlayer))
      (Utilities|FlowControl|Delay 0.05)
      (Utilities|Array|Add (Variables|Default|GetAllConnectedPlayers) _aspc_lobby_controller)
      (CallFunction|AssignPlayerPlatform _aspc_lobby_controller)
      (CallFunction|GiveType _aspc_lobby_controller))))

(event EventBeginPlay
  (bind _outactors (Actor|GetAllActorsOfClass "/Game/Programming/Lobby/BP_LobbyPlayerPlatform.BP_LobbyPlayerPlatform_C"))
  (Variables|Default|SetPlatforms _outactors))

(fn ConstructionScript)

(fn ChoosePlayerStart
  (params (Player :type Controller%20Object%20Reference))
  (return 0))

(fn AssignPlayerPlatform
  (params (Player :type PC%20Lobby%20Controller%20Object%20Reference))
  ;[1 1 1] Checks the available platforms and teleports player to the first not occupied
  (bind _array_element (Utilities|Array|ForEachLoopwithBreak (Variables|Default|GetPlatforms) :!label _label)
    (:LoopBody
      (if (not (Variables|/Game/Programming/Lobby/BP_LobbyPlayerPlatform.BP_LobbyPlayerPlatform_C|GetIsOccupied _array_element))
        (Variables|/Game/Programming/Lobby/BP_LobbyPlayerPlatform.BP_LobbyPlayerPlatform_C|SetIsOccupied _array_element true)
        (Transformation|SetActorLocation (Pawn|GetControlledPawn Player) (Transformation|GetSocketLocation (Variables|/Game/Programming/Lobby/BP_LobbyPlayerPlatform.BP_LobbyPlayerPlatform_C|GetPlayerSpawnTransform _array_element) "None") false true)
        (goto _label Break)))))

(fn GiveType
  (params (Player :type PC%20Lobby%20Controller%20Object%20Reference))
  (bind _asbp_lobby_character_pawn (Utilities|Casting|CastToBP_Lobby_Character_Pawn (Pawn|GetControlledPawn Player)))
  (if (== (Utilities|Array|Length (Variables|Default|GetAllConnectedPlayers)) 1)
    (Variables|/Game/Programming/Lobby/BP_Lobby_Character_Pawn.BP_Lobby_Character_Pawn_C|SetType _asbp_lobby_character_pawn "Boss")
    (else
      (Variables|/Game/Programming/Lobby/BP_Lobby_Character_Pawn.BP_Lobby_Character_Pawn_C|SetType _asbp_lobby_character_pawn "Hero"))))