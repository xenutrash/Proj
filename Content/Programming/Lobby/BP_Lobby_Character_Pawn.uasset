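; Lobby pawn that displays a player's selected hero or boss and stores that character choice.
; ChangeCharacter looks up a row in DT_Heroes or DT_Bosses, and UpdateCharacter reapplies it after a delay.
; SetCharacter feeds mesh, character, animation, height and name into paired server/client events, which apply each change on authority and remotes.
; On BeginPlay, the locally controlled pawn switches the view to the lobby camera.
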(event Custom|Set%20Mesh%20On%20Server
  (params (NewMesh :type Skeletal%20Mesh%20Object%20Reference))
  ;[1 1 1] Change visible mesh
  (Networking|SwitchHasAuthority
    (:Authority
      (Utilities|FlowControl|Sequence
        (:then_0
          (CallFunction|SetMeshonClient NewMesh))
        (:then_1
          (Components|SkeletalMesh|SetSkeletalMeshAsset (Variables|Default|GetCharacterMesh) (stale Custom|Set%20Mesh%20On%20Client New%20Mesh)))))))

(event Custom|ChangeCharacter
  (params (NameOfCharacter :type Name) (IsBoss :type Boolean))
  (Variables|Default|SetName%20Of%20Character NameOfCharacter)
  (bind _output_get (Variables|Default|SetIs%20Boss IsBoss))
  (if _output_get
    (bind _returnvalue (Utilities|GetDataTableRow "/Game/Programming/Lobby/DataSets/DT_Bosses.DT_Bosses" (Variables|Default|GetName%20Of%20Character))
      (:then
        (CallFunction|SetCharacter _returnvalue)))
    (else
      (bind _returnvalue_2 (Utilities|GetDataTableRow "/Game/Programming/Lobby/DataSets/DT_Heroes.DT_Heroes" (Variables|Default|GetName%20Of%20Character))
        (:then
          (CallFunction|SetCharacter _returnvalue_2))))))

(event Custom|SetCharacterNameClients
  (params (Value :type Text%20%28by%20ref%29))
  (Networking|SwitchHasAuthority
    (:Remote
      (Rendering|Components|TextRender|SetText (Variables|Default|GetCharacterName) Value))))

(event Custom|Set%20Height%20Mesh%20Server
  (params (New%20Location%20Z :type Float%20%28double-precision%29))
  (Networking|SwitchHasAuthority
    (:Authority
      (Utilities|FlowControl|Sequence
        (:then_0
          (CallFunction|SetHeightMeshClients New%20Location%20Z))
        (:then_1
          (Transformation|SetRelativeLocation (Variables|Default|GetCharacterMesh) (Math|Vector|MakeVector 0.0 0.0 (stale Custom|Set%20Height%20Mesh%20Clients New%20Location%20Z)) false true))))))

(event Custom|Set%20Height%20Mesh%20Clients
  (params (New%20Location%20Z :type Float%20%28double-precision%29))
  (Networking|SwitchHasAuthority
    (:Remote
      (Transformation|SetRelativeLocation (Variables|Default|GetCharacterMesh) (Math|Vector|MakeVector 0.0 0.0 New%20Location%20Z) false true))))

(event Custom|Set%20Mesh%20On%20Client
  (params (New%20Mesh :type Skeletal%20Mesh%20Object%20Reference))
  ;[1 1 1] Change visible mesh
  (Networking|SwitchHasAuthority
    (:Remote
      (Components|SkeletalMesh|SetSkeletalMeshAsset (Variables|Default|GetCharacterMesh) New%20Mesh))))

(event Custom|Set%20Animation%20Server
  (params (NewAnimToPlay :type Animation%20Asset%20Object%20Reference))
  (Networking|SwitchHasAuthority
    (:Authority
      (Utilities|FlowControl|Sequence
        (:then_0
          (CallFunction|SetAnimationClients NewAnimToPlay))
        (:then_1
          (Components|Animation|PlayAnimation (Variables|Default|GetCharacterMesh) (stale Custom|Set%20Animation%20Clients NewAnimToPlay) true))))))

(event Custom|Set%20Animation%20Clients
  (params (NewAnimToPlay :type Animation%20Asset%20Object%20Reference))
  (Networking|SwitchHasAuthority
    (:Remote
      (Components|Animation|PlayAnimation (Variables|Default|GetCharacterMesh) NewAnimToPlay true))))

(event Custom|UpdateCharacter
  (Utilities|FlowControl|Delay 1.0)
  (if (Variables|Default|GetIs%20Boss)
    (bind _returnvalue (Utilities|GetDataTableRow "/Game/Programming/Lobby/DataSets/DT_Bosses.DT_Bosses" (Variables|Default|GetName%20Of%20Character))
      (:then
        (CallFunction|SetCharacter _returnvalue)))
    (else
      (bind _returnvalue_2 (Utilities|GetDataTableRow "/Game/Programming/Lobby/DataSets/DT_Heroes.DT_Heroes" (Variables|Default|GetName%20Of%20Character))
        (:then
          (CallFunction|SetCharacter _returnvalue_2))))))

(event Custom|SetCharacterNameServer
  (params (Value :type Text%20%28by%20ref%29))
  (Networking|SwitchHasAuthority
    (:Authority
      (Utilities|FlowControl|Sequence
        (:then_0
          (CallFunction|SetCharacterNameClients Value))
        (:then_1
          (Rendering|Components|TextRender|SetText (Variables|Default|GetCharacterName) (stale Custom|SetCharacterNameClients Value)))))))

(event Custom|Set%20Character%20On%20Client
  (params (SelectedCharacter :type Rush%20Character%20Class%20Reference))
  ;[1 1 1] Change to selected character
  (Networking|SwitchHasAuthority
    (:Remote
      (Variables|Default|SetSelectedCharacter SelectedCharacter))))

(event Custom|Set%20Character%20On%20Server
  (params (SelectedCharacter :type Rush%20Character%20Class%20Reference))
  ;[1 1 1] Change to selected character
  (Networking|SwitchHasAuthority
    (:Authority
      (Utilities|FlowControl|Sequence
        (:then_0
          (CallFunction|SetCharacteronClient SelectedCharacter))
        (:then_1
          (Variables|Default|SetSelectedCharacter (stale Custom|Set%20Character%20On%20Client SelectedCharacter)))))))

(event EventBeginPlay
  (if (Pawn|IsLocallyControlled)
    (bind _outactors (Actor|GetAllActorsOfClass "/Game/Programming/Lobby/BP_Lobby_Camera.BP_Lobby_Camera_C"))
    (for _array_element _outactors
      (Game|Player|SetViewTargetwithBlend (Game|GetPlayerController 0) _array_element 0.0 "VTBlend_Linear" 0.0 false))))

(fn ConstructionScript)

(fn SetPlayerName
  (bind _returnvalue (Game|GetPlayerController 0))
  (bind _playerstate (Variables|/Script/Engine.Controller|GetPlayerState _returnvalue))
  (Utilities|IsValid _playerstate
    (:Is%20Valid
      (Rendering|Components|TextRender|SetText (Variables|Default|GetPlayerName) (Utilities|Text|ToText(String) (PlayerState|GetPlayerName _playerstate)))
      (return))))

(fn SetupDataTables
  (bind _outrownames (DataTable|GetDataTableRowNames "/Game/Programming/Lobby/DataSets/DT_Bosses.DT_Bosses"))
  (Variables|Default|SetDataTableRowNamesBoss _outrownames)
  (bind _outrownames_2 (DataTable|GetDataTableRowNames "/Game/Programming/Lobby/DataSets/DT_Heroes.DT_Heroes"))
  (Variables|Default|SetDataTableRowNamesHeroes _outrownames_2)
  (Variables|Default|SetCurrentRowIndex 0))

(fn GetSelectedCharacter
  (return (Variables|Default|GetSelectedCharacter)))

(fn SetCharacter
  (params (S_Lobby_Characters :type S%20Lobby%20Characters%20Structure%20%28by%20ref%29))
  (bind (_name _mesh _realcharacter _animation _heightmesh) (Utilities|Struct|BreakS_Lobby_Characters S_Lobby_Characters))
  (CallFunction|SetMeshonServer _mesh)
  (CallFunction|SetCharacteronServer _realcharacter)
  (CallFunction|SetAnimationServer _animation)
  (CallFunction|SetHeightMeshServer _heightmesh)
  (CallFunction|SetCharacterNameServer _name))

(fn CreateCharacter
  (params (CharacterInfo :type S%20Lobby%20Characters%20Structure%20%28by%20ref%29) (Controller :type PC%20Lobby%20Controller%20Object%20Reference))
  (bind _returnvalue (Game|SpawnActorfromClass "BP_Lobby_Character_Pawn_C" (Math|Transform|MakeTransform "0, 0, 0") "AdjustIfPossibleButDontSpawnIfColliding" "MultiplyWithRoot" Controller 0))
  (Components|SkeletalMesh|SetSkeletalMeshAsset (Variables|BP_Lobby_Character_Pawn_C|GetCharacterMesh _returnvalue) "/Game/Characters/Mannequin_UE4/Meshes/SK_Mannequin.SK_Mannequin"))