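; Lobby player controller that manages the lobby menu, loading screen and exit from a multiplayer session.
; On BeginPlay it creates the lobby widget, hidden on MainMenuMap, shows the cursor, caches the game instance and plays a loading screen in reverse.
; Events replay that animation forward for the local controller, forward character changes to the lobby pawn, and destroy the session before opening the main menu.
; Helper functions show or hide the menu and return player name and selected character.
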(event Custom|EndClientSession
  (|DestroySession self
    (:then
      (Game|OpenLevel(byObjectReference) "/Game/Programming/Lobby/Maps/MainMenuMap.MainMenuMap"))))

(event Custom|PlayLoadingANimastion
  (if (Pawn|IsLocalController)
    (Default|PlayEverything (Variables|Default|GetLoadingScreen) "Forward")
    (Development|PrintString "Running")
    (else
      (Development|PrintString "UNREAL IS CRINGE"))))

(event Custom|ChangeCharacter
  ;[1 1 1] Change character from dataset
  (bind _asbp_lobby_character_pawn (Utilities|Casting|CastToBP_Lobby_Character_Pawn (Game|Player|GetPlayerPawn 0)))
  (Default|ChangeCharacter _asbp_lobby_character_pawn)
  (Default|GetSelectedCharacter _asbp_lobby_character_pawn))

(event EventBeginPlay
  (CallFunction|UIShowLobbyMenu))

(fn ConstructionScript)

(fn GetPlayerName
  (return (PlayerState|GetPlayerName (Variables|/Script/Engine.Controller|GetPlayerState (Game|GetPlayerController 0)))))

(fn UIShowLobbyMenu
  (Utilities|IsValid (Variables|Default|GetWB_LobbyMenu)
    (:Is%20Valid
      _)
    (:Is%20Not%20Valid
      (bind _returnvalue (UserInterface|CreateWidget "/Game/Programming/Lobby/Widgets/WBP_Lobby.WBP_Lobby_C" (Game|GetPlayerController 0)))
      (bind _output_get (Variables|Default|SetWB_LobbyMenu _returnvalue))
      (bind _returnvalue_2 (Game|GetCurrentLevelName true))
      (if (Utilities|Enum|NotEqual(Enum) _returnvalue_2 "MainMenuMap")
        _
        (else
          (Widget|SetVisibility _output_get "Hidden")))))
  (UserInterface|Viewport|AddtoViewport (Variables|Default|GetWB_LobbyMenu) 0)
  (Variables|Default|SetbShowMouseCursor true)
  (bind _asafgi_main (Utilities|Casting|CastToAFGI_Main (Game|GetGameInstance)))
  (Variables|Default|SetRef_AFGI_Main _asafgi_main)
  (bind _returnvalue_3 (UserInterface|CreateWidget "/Game/Programming/Lobby/Widgets/WBP_LoadingScreen.WBP_LoadingScreen_C" (Game|GetPlayerController 0)))
  (bind _output_get_2 (Variables|Default|SetLoadingScreen _returnvalue_3))
  (UserInterface|Viewport|AddtoViewport _output_get_2 0)
  (Default|PlayEverythingReverse _output_get_2)
  (return))

(fn GetSelectedCharacter
  (return (Variables|Default|GetSelectedCharacter)))

(fn UiShowLobbyMenuFr
  (bind _wb_lobbymenu (Variables|Default|GetWB_LobbyMenu))
  (if (Utilities|IsValid _wb_lobbymenu)
    (Widget|SetVisibility _wb_lobbymenu "Visible")
    (else
      (Development|PrintString "Invalid hud ref"))))

(fn UiHideLobbyGUI
  (bind _wb_lobbymenu (Variables|Default|GetWB_LobbyMenu))
  (if (Utilities|IsValid _wb_lobbymenu)
    (Widget|SetVisibility _wb_lobbymenu "Hidden")
    (else
      (Development|PrintString "No valid GUI "))))