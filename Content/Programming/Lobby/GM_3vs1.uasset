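; Game mode for the 3vs1 Boss versus Heroes match, handling spawning, match flow and win conditions.
; Spawns and possesses DataTable-selected characters at PlayerStarts, gives spectators an input-disabled camera-positioned pawn, and locks player input until a timer countdown ends.
; Once players spawn, it clears loading screens and runs a recurring mushroom circle.
; Deaths and logouts update battle music or end the match with brief slow motion and end-game widgets.
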(event Custom|Player%20Died
  (params (ActorThatDied :type Actor%20Object%20Reference) (Controller :type BP%20Proj%20Player%20Controller%20Object%20Reference))
  ;[1 1 1] Checks who died and checks if it needs to end the game
  (if (not (Utilities|Array|ContainsItem (Variables|Default|GetPeopleDied) ActorThatDied))
    (CallFunction|AddPlayerDied ActorThatDied Controller)))

(event Custom|End%20Game
  (params (Winner :type String))
  ;[1 1 1] Ends the game
  (if (not (Variables|Default|GetGameEnded))
    (Variables|Default|SetGameEnded true)
    (CallFunction|SlowDownTime 0.5)
    (Utilities|FlowControl|Delay 1.5)
    (CallFunction|SlowDownTime 1.0)
    (CallFunction|CreateEndGameWidget Winner)
    (bind _returnvalue (Actor|GetActorOfClass "/Game/Programming/Blueprints/BP_BattleMusic.BP_BattleMusic_C"))
    (Default|EndMusic _returnvalue)))

(event Custom|StartCircle
  ;[1 1 1] Start the circle with time interval
  (bind _returnvalue (Actor|GetActorOfClass "/Game/Programming/Blueprints/Gameplay/LevelEffects/BP_MushroomCircle.BP_MushroomCircle_C"))
  (if (Utilities|IsValid _returnvalue)
    (Default|StartCircle _returnvalue 1.0 0.1 15.0)
    (Utilities|Time|SetTimerbyEvent (delegate Custom|StartCricle) 2e+01 true)))

(event Custom|StartCricle
  ;[1 1 1] Start the circle with time interval
  (Default|StartCircle (stale Custom|StartCircle _returnvalue) 0.4 6.0 6.0))

(event Custom|Find%20Spectator%20Camera
  ;[1 1 1] Find the spectator camera
  (bind _outactors (Actor|GetAllActorsOfClass "/Script/Engine.CameraActor"))
  (for _array_element _outactors
    (if (Actor|ActorHasTag _array_element "SpectatorCamera")
      (Variables|Default|SetSpectatorCamera _array_element))))

(event Custom|SpawnCharacters
  ;[1 1 1] Spawns in the correct characters and make players posses them
  (bind _outactors (Actor|GetAllActorsOfClass "/Script/Engine.PlayerStart"))
  (bind _asafgi_main (Utilities|Casting|CastToAFGI_Main (Game|GetGameInstance)))
  (for (_array_element _array_index) (Variables|/Game/Programming/Lobby/AFGI_Main.AFGI_Main_C|GetSelectCombo _asafgi_main)
    (bind _returnvalue (Game|SpawnActorfromClass (.Character (Utilities|Struct|BreakS_CharacterSets _array_element)) (Transformation|GetActorTransform (Utilities|Array|Get(acopy) _outactors _array_index)) "AdjustIfPossibleButDontSpawnIfColliding" "MultiplyWithRoot" (Game|GetPlayerController _array_index) 0))
    (Pawn|Possess (Game|GetPlayerController _array_index) _returnvalue)
    (Development|PrintString "Is valid")
    (bind _asbp_proj_player_controller (Utilities|Casting|CastToBP_ProjPlayerController (Game|GetPlayerController _array_index)))
    (switch string (Utilities|String|ToString(Name) (.CharacterName (Utilities|Struct|BreakS_CharacterSets _array_element)))
      (:Alchemist
        (Default|SetHudIConsEvent _asbp_proj_player_controller "Alchemist" "None"))
      (:Slayer
        (Default|SetHudIConsEvent _asbp_proj_player_controller "Nixa" "None" :!label _label))
      (:Nixa
        (goto _label)))))

(event Custom|StartCountdown
  ;[1 1 1] Start countdown for match begin
  (bind _ended (CallFunction|UpdateCountdown))
  (if _ended
    (Utilities|Time|ClearandInvalidateTimerbyHandle (stale EventBeginPlay _returnvalue))))

(event Custom|SetCamera
  (params (Target :type Player%20Controller%20Object%20Reference))
  (Game|Player|SetViewTargetwithBlend Target (Variables|Default|GetSpectatorCamera) 0.5 "VTBlend_Linear" 0.0 false))

(event EventBeginPlay
  (CallFunction|FindSpectatorCamera)
  (Utilities|FlowControl|Delay 0.2)
  ;[1 1 1] Start countdown for match begin
  (for _array_element (Variables|Default|GetPlayerControllers)
    (Default|DisableAllInput _array_element true))
  (bind _returnvalue (Utilities|Time|SetTimerbyEvent (delegate Custom|StartCountdown) 1.0 true)))

(event EventOnPlayersSpawned
  (params (GameModeSettings :type Game%20Mode%20Settings%20Structure%20%28by%20ref%29))
  (bind _outactors (Actor|GetAllActorsOfClasswithTag "/Game/Programming/Blueprints/BP_RushCharacter.BP_RushCharacter_C" "Hero"))
  (Variables|Default|SetHeroesMaxDeaths (Utilities|Array|Length _outactors))
  (Utilities|FlowControl|Delay 3.0)
  (CallFunction|RemoveLoadingScreenWidget)
  (CallFunction|StartCircle))

(event EventOnSpawnPlayer
  (params (Controller :type Player%20Controller%20Object%20Reference) (PlayerInfo :type Connected%20Player%20Structure%20%28by%20ref%29) (GameModeSettings :type Game%20Mode%20Settings%20Structure%20%28by%20ref%29))
  (bind (_selectedcharacter _selectedskin _playerindex _isboss) (Utilities|Struct|BreakConnectedPlayer PlayerInfo))
  (bind _returnvalue (Utilities|GetDataTableRow "/Game/Programming/Blueprints/DataStructs/DT_CharacaterInfo.DT_CharacaterInfo" _selectedcharacter)
    (:then
      (bind _pos (CallFunction|GetSpawnPoint _isboss))
      (bind _returnvalue_2 (Game|SpawnActorfromClass (.Character (Utilities|Struct|BreakS_CharacterInformastion _returnvalue)) _pos "AdjustIfPossibleButDontSpawnIfColliding" "MultiplyWithRoot" Controller 0))
      (Pawn|Possess Controller _returnvalue_2)
      (bind _asbp_proj_player_controller (Utilities|Casting|CastToBP_ProjPlayerController Controller))
      (Default|DisableAllInput _asbp_proj_player_controller true)
      (Utilities|Array|AddUnique (Variables|Default|GetPlayerControllers) _asbp_proj_player_controller)
      (bind _asbp_3vs_1game_state (Utilities|Casting|CastToBP_3vs1GameState (Game|GetGameState)))
      (bind _asmythbreak_player_state (Utilities|Casting|CastToMythbreakPlayerState (Variables|/Script/Engine.Controller|GetPlayerState Controller)))
      (Default|AddPlayer _asbp_3vs_1game_state _asmythbreak_player_state))))

(event EventOnSpawnSpectator
  (params (Controller :type Player%20Controller%20Object%20Reference) (PlayerInfo :type Connected%20Player%20Structure%20%28by%20ref%29))
  (bind _asbp_proj_player_controller (Utilities|Casting|CastToBP_ProjPlayerController Controller))
  (Default|SetSpecator _asbp_proj_player_controller)
  (CallFunction|FindSpectatorCamera)
  (bind _returnvalue (Game|SpawnActorfromClass "/Script/Engine.SpectatorPawn" (Transformation|GetActorTransform (Variables|Default|GetSpectatorCamera)) "AdjustIfPossibleButAlwaysSpawn" "MultiplyWithRoot" _asbp_proj_player_controller 0))
  (Pawn|Possess Controller _returnvalue)
  (Input|DisableInput _returnvalue Controller))

(event EventOnLogout
  (params (ExitingController :type Controller%20Object%20Reference))
  (bind _outactors (Actor|GetAllActorsOfClasswithTag "/Game/Programming/Blueprints/BP_RushCharacter.BP_RushCharacter_C" "Hero"))
  (bind _output_get (Variables|Default|SetHeroesMaxDeaths (Utilities|Array|Length _outactors)))
  (if (< _output_get 1)
    (CallFunction|EndGame "Boss")))

(fn ConstructionScript)

(fn CreateEndGameWidget
  (params (NewParam :type String))
  (for _array_element (Variables|/Script/Engine.GameStateBase|GetPlayerArray (Game|GetGameState))
    (bind _asbp_proj_player_controller (Utilities|Casting|CastToBP_ProjPlayerController (Game|GetPlayerController _array_element)))
    (Default|EndGame _asbp_proj_player_controller NewParam)))

(fn RemoveLoadingScreenWidget
  (for _array_element (Variables|Default|GetPlayerControllers)
    (Default|SetPlayerName _array_element))
  (for _array_element_2 (Variables|/Script/Engine.GameStateBase|GetPlayerArray (Game|GetGameState))
    (bind _asbp_proj_player_controller (Utilities|Casting|CastToBP_ProjPlayerController (Game|GetPlayerController _array_element_2)))
    (bind _asafgi_instance (Utilities|Casting|CastToAFGI_Instance (Game|GetGameInstance)))
    (Default|SetHudIConsEvent _asbp_proj_player_controller (.SelectedCharacter (Utilities|Struct|BreakConnectedPlayer (Class|AFGIMain|GetPlayerInfo _asafgi_instance (Game|GetPlayerController _array_element_2)))) (.SelectedSkin (Utilities|Struct|BreakConnectedPlayer (Class|AFGIMain|GetPlayerInfo _asafgi_instance (Game|GetPlayerController _array_element_2)))))))

(fn AddPlayerDied
  (params (Actor%20That%20Died :type Actor%20Object%20Reference) (ControllerThatDied :type BP%20Proj%20Player%20Controller%20Object%20Reference))
  (Variables|Default|SetActor%20That%20Died Actor%20That%20Died)
  (Variables|Default|SetControllerThatDied ControllerThatDied)
  (Utilities|Array|Add (Variables|Default|GetPeopleDied) (Variables|Default|GetActor%20That%20Died))
  (Default|DisableAllInput (Variables|Default|GetControllerThatDied) true)
  (if (Actor|ActorHasTag (Variables|Default|GetActor%20That%20Died) "Boss")
    (CallFunction|EndGame "Heroes")
    (else
      (bind _output_get (Variables|Default|SetHeroesDeadCount (+ (Variables|Default|GetHeroesDeadCount) 1)))
      (if (>= _output_get (Variables|Default|GetHeroesMaxDeaths))
        (CallFunction|EndGame "Boss")
        (else
          (bind _returnvalue (Actor|GetActorOfClass "/Game/Programming/Blueprints/BP_BattleMusic.BP_BattleMusic_C"))
          (Default|UpdateIntensity _returnvalue (Math|Conversions|ToFloat(Integer) _output_get)))))))

(fn GetSpawnPoint
  (params (Boss :type Boolean))
  (if (< (Utilities|Array|Length (Variables|Default|GetSpawnPoints)) 1)
    (bind _outactors (Actor|GetAllActorsOfClass "/Script/Engine.PlayerStart"))
    (for (_array_element _array_index) _outactors
      (if Boss
        (if (Actor|ActorHasTag _array_element "BossSpawnpoint")
          (Variables|Default|SetSpawnPoints _outactors :!label _label)
          (LocalVariables|SetReturnValue (Transformation|GetActorTransform (Utilities|Array|Get(acopy) (Variables|Default|GetSpawnPoints) _array_index)))
          (Utilities|Array|RemoveIndex (Variables|Default|GetSpawnPoints) _array_index)
          (return (LocalVariables|GetReturnValue)))
        (elif (not (Actor|ActorHasTag _array_element "BossSpawnpoint"))
          (goto _label))))
    (else
      (LocalVariables|SetReturnValue (Transformation|GetActorTransform (Utilities|Array|Get(acopy) (Variables|Default|GetSpawnPoints) _array_index)))
      (Utilities|Array|RemoveIndex (Variables|Default|GetSpawnPoints) _array_index)
      (return (LocalVariables|GetReturnValue)))))

(fn SlowDownTime
  (params (Time%20Dialation :type Float%20%28single-precision%29))
  (Utilities|Time|SetGlobalTimeDilation Time%20Dialation))

(fn SetSpectatorCamera
  (params (Controller :type Player%20Controller%20Object%20Reference))
  (Game|Player|SetViewTargetwithBlend Controller (Variables|Default|GetSpectatorCamera) 0.5 "VTBlend_Linear" 0.0 false))

(fn UpdateCountdown
  (if (< (Variables|Default|GetCountdown) 1)
    (for _array_element (Variables|Default|GetPlayerControllers)
      (Default|DisableAllInput _array_element false)
      (Default|UpdateCountdown _array_element))
    (return true)
    (else
      (for _array_element_2 (Variables|Default|GetPlayerControllers)
        (Default|UpdateCountdown _array_element_2 (Utilities|Text|ToText(Integer) (Variables|Default|GetCountdown))))
      (Variables|Default|SetCountdown (- (Variables|Default|GetCountdown) 1))
      (return false))))