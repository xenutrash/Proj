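; BP_RushCharacter is a networked player character that turns toward the mouse cursor and relays its rotation to other clients.
; Damage, shield, max health and ultimate charge run through GAS SetByCaller effects, with damage passing through shield reduction and logging to MythbreakPlayerState.
; Health changes trigger an authority-side death check with GM_3vs1 and an overhead-widget refresh.
; Loose gameplay tags provide timed invulnerability and temporary ability blocking, while max speed edits CharacterMovement directly.
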(event Custom|Check%20If%20Dead
  (params (Health :type Float%20%28double-precision%29))
  ;[1 1 1] Checks if player has below 0 hp, then calls gamemode
  (if (<= Health 0.0)
    (bind _asgm_3vs_1 (Utilities|Casting|CastToGM_3vs1 (Game|GetGameMode)))
    (bind _asbp_proj_player_controller (Utilities|Casting|CastToBP_ProjPlayerController (Pawn|GetController)))
    (Default|PlayerDied _asgm_3vs_1 self _asbp_proj_player_controller)))

(event Custom|Server%20On%20Health%20Changed
  ;[1 1 1] Update health when changed
  (Networking|SwitchHasAuthority
    (:Authority
      (CallFunction|CheckifDead (.ReturnValue (Class|AbilitySystemComponent|GetGameplayAttributeValue (Variables|Default|GetAbilitySystemComponent) "(AttributeName=\"Health\",Attribute=/Script/Proj.RushAttributeSet:Health,AttributeOwner=\"/Script/CoreUObject.Class'/Script/Proj.RushAttributeSet'\")")))
      (CallFunction|OnHealthChangedAllClients))))

(event Custom|RotateCharacter
  (bind _returnvalue (Utilities|Time|GetWorldDeltaSeconds))
  (bind _returnvalue_2 (Game|GetPlayerController 0))
  (bind _returnvalue_3 (Transformation|GetActorLocation))
  (bind _returnvalue_4 (Transformation|GetActorRotation))
  (bind _hitresult (Game|Player|GetHitResultUnderCursorbyChannel _returnvalue_2 "TraceTypeQuery1" true))
  (bind _returnvalue_5 (Math|Rotator|FindLookatRotation (Math|Vector|MakeVector (.x _returnvalue_3) (.y _returnvalue_3) (.z _returnvalue_3)) (Math|Vector|MakeVector (.x (.location _hitresult)) (.y (.location _hitresult)) (.z _returnvalue_3))))
  (bind _returnvalue_6 (Math|Interpolation|RInterpTo _returnvalue_4 _returnvalue_5 _returnvalue 1e+01))
  ;[1 1 1] Rotate character to mouse position
  (Transformation|SetActorRotation _returnvalue_6)
  (CallFunction|RotateAllClients _returnvalue_6))

(event Custom|Add%20To%20Max%20Health
  (params (Health%20Amount :type Float%20%28double-precision%29))
  ;[1 1 1] Add max health
  (bind _returnvalue (Ability|GameplayEffect|AssignTagSetbyCallerMagnitude (GameplayEffects|MakeOutgoingSpec :self (Variables|Default|GetAbilitySystemComponent) :GameplayEffectClass "/Game/Programming/Blueprints/GeneralAbilities/GE_SetMaxHealth.GE_SetMaxHealth_C") "(TagName=\"MaxHealth\")" Health%20Amount))
  (GameplayEffects|ApplyGameplayEffectSpecToSelf (Variables|Default|GetAbilitySystemComponent) _returnvalue))

(event Custom|ResetUltimateServer
  ;[1 1 1] Reset ultimate and UI
  (bind _returnvalue (Ability|GameplayEffect|AssignTagSetbyCallerMagnitude (GameplayEffects|MakeOutgoingSpec :self (Variables|Default|GetAbilitySystemComponent) :GameplayEffectClass "/Game/Programming/Blueprints/GeneralAbilities/GE_GiveUltimateCharge.GE_GiveUltimateCharge_C") "(TagName=\"Attack.Ultimate\")" (* (.ReturnValue (Class|AbilitySystemBlueprintLibrary|GetFloatAttributeBasefromAbilitySystemComponent (Variables|Default|GetAbilitySystemComponent) "(AttributeName=\"UltimateCharge\",Attribute=/Script/Proj.RushAttributeSet:UltimateCharge,AttributeOwner=\"/Script/CoreUObject.Class'/Script/Proj.RushAttributeSet'\")")) -1.0)))
  (GameplayEffects|ApplyGameplayEffectSpecToSelf (Variables|Default|GetAbilitySystemComponent) _returnvalue))

(event Custom|ActivateInvulernability
  (params (Duration :type Float%20%28single-precision%29))
  ;[1 1 1] Invulnerability for a limited time
  (if (not (Utilities|Array|ContainsItem (.gameplaytags (GameplayTags|GetOwnedGameplayTags (Variables|Default|GetAbilitySystemComponent) :!class /Script/GameplayTags.GameplayTagAssetInterface)) "(TagName=\"Defense.Invincibility\")"))
    (Ability|GameplayEffect|AddLooseGameplayTags self (GameplayTags|MakeGameplayTagContainerfromTag "(TagName=\"Defense.Invincibility\")"))
    (Utilities|FlowControl|Delay Duration)
    (Ability|GameplayEffect|RemoveLooseGameplayTags self (GameplayTags|MakeGameplayTagContainerfromTag "(TagName=\"Defense.Invincibility\")"))))

(event Custom|PlayLoadingTemp
  (bind _returnvalue (Game|GetPlayerController 0))
  (if (Pawn|IsLocalController _returnvalue)
    (bind _asbp_proj_player_controller (Utilities|Casting|CastToBP_ProjPlayerController _returnvalue))
    (Default|PlayLoadingANimastionReverse _asbp_proj_player_controller)
    (else
      (Utilities|String|LogString "NOT EXECUTED LOCALLY "))))

(event Custom|Take%20Damage
  (params (DamageAmount :type Float%20%28single-precision%29))
  (bind _returnvalue (Transformation|GetActorTransform))
  ;[1 1 1] Take damage
  (CallFunction|AddDamageTakentoScore DamageAmount)
  (bind _returnvalue_2 (CallFunction|ReduceShield DamageAmount))
  (bind _returnvalue_3 (Ability|GameplayEffect|AssignTagSetbyCallerMagnitude (GameplayEffects|MakeOutgoingSpec :self (Variables|Default|GetAbilitySystemComponent) :GameplayEffectClass "/Game/Programming/Blueprints/GeneralAbilities/GE_TakeDamage.GE_TakeDamage_C") "(TagName=\"Health\")" _returnvalue_2))
  (GameplayEffects|ApplyGameplayEffectSpecToSelf (Variables|Default|GetAbilitySystemComponent) _returnvalue_3)
  (Default|PlaySoundLocally (Variables|Default|GetSoundSystem) "/Game/FMOD/Events/InWorld/LocalPlayer/Local_Hit.Local_Hit" _returnvalue false)
  (Default|PlaySoundAllClientsExcludeOwner (Variables|Default|GetSoundSystem) 0 _returnvalue (Game|GetPlayerController 0) false))

(event Custom|MultiCastApplyRotation
  (params (NewRotation :type Rotator))
  ;[1 1 1] Rotate character to mouse position
  (if (not (Pawn|IsLocallyControlled))
    (Transformation|SetActorRotation NewRotation true)))

(event Custom|AddDamageTakenToScore
  (params (DamageTaken :type Float%20%28single-precision%29))
  ;[1 1 1] Updates the score on the player
  (bind _asmythbreak_player_state (Utilities|Casting|CastToMythbreakPlayerState (Variables|/Script/Engine.Controller|GetPlayerState (Game|GetPlayerController 0))))
  (Class|MythbreakPlayerState|AddDamageTaken _asmythbreak_player_state DamageTaken))

(event Custom|Client%20On%20Health%20Changed
  ;[1 1 1] Update health when changed
)

(event Custom|On%20health%20changed%20All%20clients
  (bind _abilitysystemcomponent (Variables|Default|GetAbilitySystemComponent))
  (bind _returnvalue (Class|AbilitySystemComponent|GetGameplayAttributeValue _abilitysystemcomponent "(AttributeName=\"Health\",Attribute=/Script/Proj.RushAttributeSet:Health,AttributeOwner=\"/Script/CoreUObject.Class'/Script/Proj.RushAttributeSet'\")"))
  (bind _returnvalue_2 (Class|AbilitySystemComponent|GetGameplayAttributeValue _abilitysystemcomponent "(AttributeName=\"MaxHealth\",Attribute=/Script/Proj.RushAttributeSet:MaxHealth,AttributeOwner=\"/Script/CoreUObject.Class'/Script/Proj.RushAttributeSet'\")"))
  ;[1 1 1] Update health when changed
  (Utilities|FlowControl|Delay 0.2)
  (bind _aswbp_stats (Utilities|Casting|CastToWBP_Stats (UserInterface|GetUserWidgetObject (Variables|Default|GetHealthbar))))
  (Default|UpdateHealth _aswbp_stats (/ _returnvalue _returnvalue_2) (Utilities|Text|FormatText "Health {0} / {1}" _returnvalue _returnvalue_2)))

(event Custom|Give%20Shield
  (params (Shield%20Amount :type Float%20%28double-precision%29))
  ;[1 1 1] Give shield
  (if (<= (.ReturnValue (Class|AbilitySystemComponent|GetGameplayAttributeValue (Variables|Default|GetAbilitySystemComponent) "(AttributeName=\"Armour\",Attribute=/Script/Proj.RushAttributeSet:Armour,AttributeOwner=\"/Script/CoreUObject.Class'/Script/Proj.RushAttributeSet'\")")) 5e+01)
    (bind _returnvalue (Ability|GameplayEffect|AssignTagSetbyCallerMagnitude (GameplayEffects|MakeOutgoingSpec :self (Variables|Default|GetAbilitySystemComponent) :GameplayEffectClass "/Game/Programming/Blueprints/GeneralAbilities/GE_GiveShield.GE_GiveShield_C") "(TagName=\"Shield\")" Shield%20Amount))
    (GameplayEffects|ApplyGameplayEffectSpecToSelf (Variables|Default|GetAbilitySystemComponent) _returnvalue)))

(event Custom|RotateAllClients
  (params (NewRotation :type Rotator))
  ;[1 1 1] Rotate character to mouse position
  (CallFunction|MultiCastApplyRotation NewRotation))

(event Custom|ChargeUltimate
  (params (ChargeAmount :type Float%20%28single-precision%29))
  ;[1 1 1] Charge ultimate
  (bind _returnvalue (Ability|GameplayEffect|AssignTagSetbyCallerMagnitude (GameplayEffects|MakeOutgoingSpec :self (Variables|Default|GetAbilitySystemComponent) :GameplayEffectClass "/Game/Programming/Blueprints/GeneralAbilities/GE_GiveUltimateCharge.GE_GiveUltimateCharge_C") "(TagName=\"Attack.Ultimate\")" ChargeAmount))
  (GameplayEffects|ApplyGameplayEffectSpecToSelf (Variables|Default|GetAbilitySystemComponent) _returnvalue)
  (if (Pawn|IsLocallyControlled)
    (Default|AddUltimateCharge (Variables|Default|GetPlayerController) ChargeAmount)))

(event Custom|AddDamageToScore
  (params (Damage :type Float%20%28single-precision%29))
  ;[1 1 1] Updates the score on the player
  (bind _asmythbreak_player_state (Utilities|Casting|CastToMythbreakPlayerState (Variables|/Script/Engine.Controller|GetPlayerState (Game|GetPlayerController 0))))
  (Class|MythbreakPlayerState|AddDamageDealt _asmythbreak_player_state (* Damage -1.0)))

(event Custom|ResetUltimate
  ;[1 1 1] Reset ultimate and UI
  (if (Pawn|IsLocallyControlled)
    (Default|ResetUltimate (Variables|Default|GetPlayerController))
    (CallFunction|ResetUltimateServer)))

(event Custom|Add%20To%20Max%20Speed
  (params (Speed%20amount :type Float%20%28double-precision%29))
  (bind _charactermovement (Variables|Character|GetCharacterMovement))
  ;[1 1 1] Add to max speed SHOULD BE FIXED WITH ATTRIBUTE SET
  (Variables|/Script/Engine.CharacterMovementComponent|SetMaxWalkSpeed _charactermovement (+ Speed%20amount (Variables|/Script/Engine.CharacterMovementComponent|GetMaxWalkSpeed _charactermovement))))

(event EventOnAttributeSetInited
  ;[1 1 1] Update health when changed
  (CallFunction|ServeronHealthChanged))

(event EventOnHealthChanged
  (params (DeltaValue :type Float%20%28single-precision%29) (EventTags :type Gameplay%20Tag%20Container%20Structure%20%28by%20ref%29))
  ;[1 1 1] Update health when changed
  (CallFunction|ServeronHealthChanged))

(fn ConstructionScript)

(fn GetMouseLocation
  (return (.location (.HitResult (Game|Player|GetHitResultUnderCursorbyChannel (Game|GetPlayerController 0) "TraceTypeQuery2" true)))))

(fn ReduceShield
  (params (Damage%20Amount :type Float%20%28single-precision%29))
  (bind _returnvalue (Math|Float|Absolute(Float) Damage%20Amount))
  (bind _abilitysystemcomponent (Variables|Default|GetAbilitySystemComponent))
  (bind _returnvalue_2 (Class|AbilitySystemComponent|GetGameplayAttributeValue _abilitysystemcomponent "(AttributeName=\"Armour\",Attribute=/Script/Proj.RushAttributeSet:Armour,AttributeOwner=\"/Script/CoreUObject.Class'/Script/Proj.RushAttributeSet'\")"))
  (bind _returnvalue_3 (- _returnvalue_2 _returnvalue))
  ;[1 1 1] Checks how much the shield absorbs the damage
  (if (<= _returnvalue_3 0.0)
    (bind _returnvalue_4 (Ability|GameplayEffect|AssignTagSetbyCallerMagnitude (GameplayEffects|MakeOutgoingSpec :self (Variables|Default|GetAbilitySystemComponent) :GameplayEffectClass "/Game/Programming/Blueprints/GeneralAbilities/GE_GiveShield.GE_GiveShield_C") "(TagName=\"Shield\")" (* _returnvalue_2 -1.0)))
    (GameplayEffects|ApplyGameplayEffectSpecToSelf (Variables|Default|GetAbilitySystemComponent) _returnvalue_4)
    (else
      (bind _returnvalue_5 (Ability|GameplayEffect|AssignTagSetbyCallerMagnitude (GameplayEffects|MakeOutgoingSpec :self (Variables|Default|GetAbilitySystemComponent) :GameplayEffectClass "/Game/Programming/Blueprints/GeneralAbilities/GE_GiveShield.GE_GiveShield_C") "(TagName=\"Shield\")" Damage%20Amount))
      (GameplayEffects|ApplyGameplayEffectSpecToSelf (Variables|Default|GetAbilitySystemComponent) _returnvalue_5)))
  (return _returnvalue_3))

(fn BlockAbilityInputTemp
  (if (Utilities|Array|ContainsItem (.gameplaytags (GameplayTags|GetOwnedGameplayTags (Variables|Default|GetAbilitySystemComponent) :!class /Script/GameplayTags.GameplayTagAssetInterface)) "(TagName=\"Attack.Block.All\")")
    (return true)
    (else
      (Ability|GameplayEffect|AddLooseGameplayTags self (GameplayTags|MakeGameplayTagContainerfromTag "(TagName=\"Attack.Block.All\")") true)
      (return true))))

(fn RemoveBlockTemp
  (bind _returnvalue (Ability|GameplayEffect|RemoveLooseGameplayTags self (GameplayTags|MakeGameplayTagContainerfromTag "(TagName=\"Attack.Block.All\")") true))
  (if _returnvalue
    (Development|PrintString "Removed?")
    (else
      (Development|PrintString "No remove?"))))