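; Alchemist powder bomb projectile that applies a Gameplay Effect to RushCharacters it overlaps, skipping actors tagged Hero.
; Each Tick, a vertical line trace from the hit plane checks for ground until the first hit.
; On impact it stops moving, sets its hit collider to query-only, fires a Niagara ring and expires shortly after.
; Overlapped actors are recorded so each receives the GAS effect only once.
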(event Collision|EventActorBeginOverlap
  (params (OtherActor :type Actor%20Object%20Reference))
  (bind _collidedwith (Variables|Default|GetCollidedWith))
  (if (not (Actor|ActorHasTag OtherActor "Hero"))
    (if (not (Utilities|Array|ContainsItem _collidedwith OtherActor))
      (Utilities|Array|Add _collidedwith OtherActor)
      (CallFunction|ApplyEffect OtherActor))))

(event EventTick
  (params (DeltaSeconds :type Float%20%28single-precision%29))
  (if (not (Variables|Default|GetGroundHit))
    (bind _iscontact (Utilities|DetectGround (Variables|Default|GetSM_HitPlane))
      (:Out
        (if _iscontact
          (Variables|Default|SetGroundHit true)
          (Development|PrintString "I hit the thing")
          (CallFunction|StopProjectileMovement)
          (Collision|SetCollisionEnabled (Variables|Default|GetHitCollider) "QueryOnly")
          (Actor|SetLifeSpan 0.2)
          (Components|Activation|Activate (Variables|Default|GetNs_HitRIng) true))))))

(fn ConstructionScript)

(fn StopProjectileMovement
  (bind _projectilemovement (Variables|Default|GetProjectileMovement))
  (Game|Components|ProjectileMovement|SetVelocityinLocalSpace _projectilemovement "0, 0, 0")
  (Variables|/Script/Engine.ProjectileMovementComponent|SetProjectileGravityScale _projectilemovement 0.0))

(fn ApplyEffect
  (params (Object :type Object%20Object%20Reference))
  (bind _asrush_character (Utilities|Casting|CastToRushCharacter Object)
    (:then
      (GameplayEffects|ApplyGameplayEffectToSelf :self (Ability|GetAbilitySystemComponent _asrush_character) :GameplayEffectClass "/Game/Programming/Blueprints/Alchemist/PowderBomb/GE_PowderBomb_effect.GE_PowderBomb_effect_C")
      (Development|PrintString "Effect applied"))
    (:CastFailed
      (Development|PrintString "Not a RushCharacter"))))