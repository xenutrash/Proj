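; GA_PowderBomb is a Gameplay Ability that throws a powder bomb projectile, filed under the Alchemist.
; On activation it plays the throw montage and waits for an Attack.Basic gameplay event to time the release.
; That event spawns BP_PowderBombProjectile at the hand_r socket with the avatar's rotation and forces the cooldown commit.
; The ability ends when the montage completes, blends out, is interrupted or is cancelled, printing a debug message.
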(event Ability|EventActivateAbility
  (bind _returnvalue (Ability|GetAvatarActorfromActorInfo))
  (|PlayMontageandWaitProxy "None" "/Game/Characters/PlagueDoctor/PlaceHolders/AM_ThrowAttack.AM_ThrowAttack" 1.0 "None" true 1.0 0.0 false
    (:then
      (Ability|Tasks|WaitGameplayEvent "(TagName=\"Attack.Basic\")" 0
        (:EventReceived
          (Game|SpawnActorfromClass "/Game/Programming/Blueprints/Alchemist/PowderBomb/BP_PowderBombProjectile.BP_PowderBombProjectile_C" (Math|Transform|MakeTransform (Transformation|GetSocketLocation (Actor|GetComponentbyClass _returnvalue "/Script/Engine.SkeletalMeshComponent") "hand_r") (Transformation|GetActorRotation _returnvalue) "1.000000,1.000000,1.000000") "Undefined" "MultiplyWithRoot" _returnvalue 0)
          (Ability|CommitAbilityCooldown false true))))
    (:OnCompleted
      (Ability|EndAbility :!label _label))
    (:OnBlendOut
      (goto _label))
    (:OnInterrupted
      (goto _label))
    (:OnCancelled
      (goto _label))))

(event Ability|EventOnEndAbility
  (params (bWasCancelled :type Boolean))
  (Development|PrintString "Ability ended"))