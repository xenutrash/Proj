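; GA_AlchemistPrimaryFire is the Gameplay Ability for the Alchemist's primary fire attack.
; On the server it plays the fire montage and waits for the Attack.Basic gameplay event.
; That event spawns BP_Alchemist_PrimaryFire at the avatar's gun hand socket facing the actor's rotation, commits the cooldown and ends the ability.
; The montage completing, blending out, or being interrupted or cancelled also ends it.
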(event Ability|EventActivateAbility
  (bind _returnvalue (Ability|GetAvatarActorfromActorInfo))
  (if (Networking|IsServer)
    (|PlayMontageandWaitProxy "None" "/Game/Characters/PlagueDoctor/PlaceHolders/AM_Alchemist_PrimaryFire.AM_Alchemist_PrimaryFire" 1.0 "None" true 1.0 0.0 false
      (:then
        (Ability|Tasks|WaitGameplayEvent "(TagName=\"Attack.Basic\")" 0
          (:EventReceived
            (Game|SpawnActorfromClass "/Game/Programming/Blueprints/Alchemist/PrimaryFire/BP_Alchemist_PrimaryFire.BP_Alchemist_PrimaryFire_C" (Math|Transform|MakeTransform (Transformation|GetSocketLocation (Actor|GetComponentbyClass _returnvalue "/Script/Engine.SkeletalMeshComponent") "ik_hand_gun") (Transformation|GetActorRotation _returnvalue) "1.000000,1.000000,1.000000") "Undefined" "MultiplyWithRoot" _returnvalue 0)
            (Ability|CommitAbilityCooldown false true)
            (Ability|EndAbility))))
      (:OnCompleted
        (Ability|EndAbility :!label _label))
      (:OnBlendOut
        (goto _label))
      (:OnInterrupted
        (goto _label))
      (:OnCancelled
        (goto _label)))))

(event Ability|EventOnEndAbility
  (params (bWasCancelled :type Boolean)))