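; Alchemist primary fire actor that damages bosses on overlap, ignoring its owner.
; Overlapped actors tagged Boss are cast to RushCharacter, and GE_TakeDamage is applied through the target's own Ability System Component.
; Any other non-owner overlap hides the actor and destroys it after a short delay, while a Boss overlap leaves it in place.
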(event Collision|EventActorBeginOverlap
  (params (OtherActor :type Actor%20Object%20Reference))
  (if (not (== OtherActor (Components|GetOwner)))
    (if (Actor|ActorHasTag OtherActor "Boss")
      (CallFunction|ApplyEffect OtherActor)
      (else
        (Rendering|SetActorHiddenInGame true)
        (Utilities|FlowControl|Delay 1.0)
        (Actor|DestroyActor)))))

(fn ConstructionScript)

(fn ApplyEffect
  (params (Object :type Object%20Object%20Reference))
  (bind _asrush_character (Utilities|Casting|CastToRushCharacter Object)
    (:then
      (GameplayEffects|ApplyGameplayEffectToSelf :self (Ability|GetAbilitySystemComponent _asrush_character) :GameplayEffectClass "/Game/Programming/Blueprints/GE_TakeDamage.GE_TakeDamage_C"))
    (:CastFailed
      (Development|PrintString "Not a RushCharacter"))))