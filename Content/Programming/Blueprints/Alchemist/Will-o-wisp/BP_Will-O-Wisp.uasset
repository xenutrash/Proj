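; Alchemist's Will-o'-Wisp area effect, which shields heroes and damages bosses inside its sphere.
; Two looping timers poll sphere overlaps and filter by actor tag: a fast one refreshes brief invulnerability with VFX on heroes, a slower one damages bosses.
; Boss damage is also added to the owning character's score.
; One second before its lifespan ends, it sets an Alchemist sound parameter, likely cueing the ending audio.
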(event Custom|DealDamage
  ;[1 1 1] Apply damage to boss in zone
  (for _array_element (Collision|GetOverlappingActors (Variables|Default|GetSphere) "/Game/Programming/Blueprints/BP_RushCharacter.BP_RushCharacter_C" :!class /Script/Engine.PrimitiveComponent)
    (if (Actor|ActorHasTag _array_element "Boss")
      (bind _asbp_rush_character (Utilities|Casting|CastToBP_RushCharacter _array_element))
      (Default|TakeDamage _asbp_rush_character (Variables|Default|GetDamage))
      (Default|AddDamagetoScore (Variables|Default|GetOwnerCharacter) (Variables|Default|GetDamage)))))

(event Custom|GiveArmor
  ;[1 1 1] Give invulnerability to heroes in zone
  (for _array_element (Collision|GetOverlappingActors (Variables|Default|GetSphere) "/Game/Programming/Blueprints/BP_RushCharacter.BP_RushCharacter_C" :!class /Script/Engine.PrimitiveComponent)
    (if (Actor|ActorHasTag _array_element "Hero")
      (bind _asbp_rush_character (Utilities|Casting|CastToBP_RushCharacter _array_element))
      (Default|ActivateInvulernability _asbp_rush_character 0.05 true))))

(event EventBeginPlay
  (bind _asbp_rush_character (Utilities|Casting|CastToBP_RushCharacter (Components|GetOwner)))
  (Variables|Default|SetOwnerCharacter _asbp_rush_character)
  (Utilities|Time|SetTimerbyEvent (delegate Custom|DealDamage) 0.2 true)
  (Utilities|Time|SetTimerbyEvent (delegate Custom|GiveArmor) 0.05 true)
  (Utilities|FlowControl|Delay (- (Variables|Actor|GetInitialLifeSpan) 1.0))
  (bind _asbp_alchemist (Utilities|Casting|CastToBP_Alchemist (Components|GetOwner)))
  (Default|EventInstanceSetParameter (Variables|/Game/Programming/Blueprints/BP_RushCharacter.BP_RushCharacter_C|GetSoundSystem _asbp_alchemist) "Alchemist_WillOfTheWisp" 1.0 (Utilities|String|MakeLiteralString "Alchemist_WillOfTheWisp")))

(fn ConstructionScript)