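; Gameplay Ability for the Alchemist's Smelling Salts special, which spawns a BP_SmellingSalt actor during an attack animation.
; On activation it force-commits the cooldown and plays a random montage from AnimationArray.
; The first Attack.Special gameplay event spawns the salt at the avatar's location, owned by the avatar and yawed 180 degrees from its facing.
; The ability ends when the montage completes, blends out, is interrupted or is cancelled.
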(event Ability|EventActivateAbility
  (bind _animationarray (Variables|Default|GetAnimationArray))
  (Ability|CommitAbilityCooldown false true)
  (|PlayMontageandWaitProxy "None" (Utilities|Array|Get(acopy) _animationarray (Math|Random|RandomInteger (Utilities|Array|Length _animationarray))) 1.0 "None" true 1.0 0.0 false
    (:then
      (Ability|Tasks|WaitGameplayEvent "(TagName=\"Attack.Special\")" 0 true
        (:EventReceived
          (CallFunction|SpawnProjectile))))
    (:OnCompleted
      (Ability|EndAbility :!label _label))
    (:OnBlendOut
      (goto _label))
    (:OnInterrupted
      (goto _label))
    (:OnCancelled
      (goto _label))))

(event Ability|EventOnEndAbility
  (params (bWasCancelled :type Boolean)))

(fn SpawnProjectile
  (bind _returnvalue (Ability|GetAvatarActorfromActorInfo))
  (bind _returnvalue_2 (Transformation|GetActorRotation _returnvalue))
  (Game|SpawnActorfromClass "/Game/Programming/Blueprints/Alchemist/SmellingSalts/BP_SmellingSalt.BP_SmellingSalt_C" (Math|Transform|MakeTransform (Transformation|GetActorLocation _returnvalue) (Math|Rotator|MakeRotator (.roll _returnvalue_2) (.pitch _returnvalue_2) (- (.yaw _returnvalue_2) 1.8e+02)) "1.000000,1.000000,1.000000") "Undefined" "MultiplyWithRoot" _returnvalue 0))