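; Smelling salt actor for the Alchemist that applies a gameplay effect to non-hero characters entering its HitRange.
; Overlapping actors tagged Hero only trigger a debug print; others are recorded in ActorsHit so each is processed once.
; ApplyEffect casts to BP_RushCharacter and applies GE_SmellingSaltOverTime through that character's Ability System Component, with debug prints along the way.
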(event OnComponentBeginOverlap(HitRange)
  (params (OverlappedComponent :type Primitive%20Component%20Object%20Reference) (OtherActor :type Actor%20Object%20Reference) (OtherComp :type Primitive%20Component%20Object%20Reference) (OtherBodyIndex :type Integer) (bFromSweep :type Boolean) (SweepResult :type Hit%20Result%20Structure%20%28by%20ref%29))
  (bind _actorshit (Variables|Default|GetActorsHit))
  (if (Actor|ActorHasTag OtherActor "Hero")
    (Development|PrintString "hit a hero")
    (elif (not (Utilities|Array|ContainsItem _actorshit OtherActor))
      (Utilities|Array|Add _actorshit OtherActor)
      (CallFunction|ApplyEffect OtherActor))))

(fn ConstructionScript)

(fn ApplyEffect
  (params (Object :type Object%20Object%20Reference))
  (Development|PrintString "HIT SOMETHING")
  (bind _asbp_rush_character (Utilities|Casting|CastToBP_RushCharacter Object))
  (GameplayEffects|ApplyGameplayEffectToSelf :self (Ability|GetAbilitySystemComponent _asbp_rush_character) :GameplayEffectClass "/Game/Programming/Blueprints/Alchemist/SmellingSalts/GE_SmellingSaltOverTime.GE_SmellingSaltOverTime_C")
  (Development|PrintString "Effect applied"))