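; Alchemist player character that turns attack and dash input events into GAS abilities: primary fire, Smelling Salts, Will-O-Wisp ultimate and dash.
; Primary, special and dash drive player controller cooldowns, though primary starts its cooldown even if activation fails.
; Successful attacks play networked sounds (primary, special) or reset ultimate charge, which gates Will-O-Wisp.
; Dash briefly shows an i-frame overlay with an effect; key 7 triggers ult-ready visuals.
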(event EventOnHealthChanged
  (params (DeltaValue :type Float%20%28single-precision%29) (EventTags :type Gameplay%20Tag%20Container%20Structure%20%28by%20ref%29))
  (|CallParentFunction DeltaValue EventTags))

(event EventBeginPlay
  (|CallParentFunction))

(event EventOnBasicAttack
  (CallFunction|AbilityPrimaryAttack))

(event EventOnSpecialAttack
  (CallFunction|AbilitySpecialAttack))

(event EventOnUltimateAttack
  (CallFunction|AbilityUltimateAttack))

(event EventOnDash
  (Development|PrintString "Dash")
  (bind _returnvalue (Abilities|TryActivateAbilitybyClass (Variables|Default|GetAbilitySystemComponent) "/Game/Programming/Blueprints/GeneralAbilities/GA_Dash.GA_Dash_C" true))
  (if _returnvalue
    (Components|Activation|Activate (Variables|Default|GetDashEffect) false)
    (Rendering|Material|SetOverlayMaterial (Variables|Character|GetMesh) "/Game/Material/M_IFrame.M_IFrame" :!class /Script/Engine.MeshComponent)
    (bind _asbp_proj_player_controller (Utilities|Casting|CastToBP_ProjPlayerController (Game|GetPlayerController 0)))
    (Default|StartCooldownSpace _asbp_proj_player_controller)
    (Utilities|FlowControl|Delay 0.2)
    (Rendering|Material|SetOverlayMaterial (Variables|Character|GetMesh) 0 :!class /Script/Engine.MeshComponent)))

(event Input|KeyboardEvents|7
  (params (Key :type Key%20Structure :default "None"))
  (:Pressed
    (Components|Activation|Activate (Variables|Default|GetNS_Ultready) false)
    (Rendering|Material|SetOverlayMaterial (Variables|Character|GetMesh) "/Game/Material/M_UltReady.M_UltReady" :!class /Script/Engine.MeshComponent)))

(fn ConstructionScript
  (|CallParentFunction))

(fn AbilityPrimaryAttack
  (bind _returnvalue (Transformation|GetActorTransform))
  (Development|PrintString "Basic attack")
  (bind _returnvalue_2 (Abilities|TryActivateAbilitybyClass (Variables|Default|GetAbilitySystemComponent) "/Game/Programming/Blueprints/Alchemist/PrimaryFire/GA_AlchemistPrimaryFire.GA_AlchemistPrimaryFire_C" true))
  (bind _asbp_proj_player_controller (Utilities|Casting|CastToBP_ProjPlayerController (Game|GetPlayerController 0)))
  (Default|StartCoolDownM1 _asbp_proj_player_controller)
  (if _returnvalue_2
    (Default|PlaySoundLocally (Variables|Default|GetSoundSystem) "/Game/FMOD/Events/InWorld/LocalPlayer/Hero/Alchemist/Local_Alchemist_MainAttack.Local_Alchemist_MainAttack" _returnvalue false)
    (Default|PlaySoundAllClientsExcludeOwner (Variables|Default|GetSoundSystem) "/Game/FMOD/Events/InWorld/NonLocalPlayer/Hero/Alchemist/NonLocal_Alchemist_MainAttack.NonLocal_Alchemist_MainAttack" _returnvalue (Game|GetPlayerController 0) false)))

(fn AbilitySpecialAttack
  (bind _returnvalue (Transformation|GetActorTransform))
  (Development|PrintString "Specialattack")
  (bind _returnvalue_2 (Abilities|TryActivateAbilitybyClass (Variables|Default|GetAbilitySystemComponent) "/Game/Programming/Blueprints/Alchemist/SmellingSalts/GA_SmellingSalts.GA_SmellingSalts_C" true))
  (if _returnvalue_2
    (bind _asbp_proj_player_controller (Utilities|Casting|CastToBP_ProjPlayerController (Game|GetPlayerController 0)))
    (Default|StartCooldownE _asbp_proj_player_controller)
    (Default|PlaySoundLocally (Variables|Default|GetSoundSystem) "/Game/FMOD/Events/InWorld/LocalPlayer/Hero/Alchemist/Local_Alchemist_SmellingSalt.Local_Alchemist_SmellingSalt" _returnvalue false)
    (Default|PlaySoundAllClientsExcludeOwner (Variables|Default|GetSoundSystem) "/Game/FMOD/Events/InWorld/LocalPlayer/Hero/Alchemist/Local_Alchemist_SmellingSalt.Local_Alchemist_SmellingSalt" _returnvalue (Game|GetPlayerController 0) false)))

(fn AbilityUltimateAttack
  (if (<= 1e+02 (.ReturnValue (Class|AbilitySystemBlueprintLibrary|GetFloatAttributeBasefromAbilitySystemComponent (Variables|Default|GetAbilitySystemComponent) "(AttributeName=\"UltimateCharge\",Attribute=/Script/Proj.RushAttributeSet:UltimateCharge,AttributeOwner=\"/Script/CoreUObject.Class'/Script/Proj.RushAttributeSet'\")")))
    (Development|PrintString "Ultiamte attack")
    (bind _returnvalue (Abilities|TryActivateAbilitybyClass (Variables|Default|GetAbilitySystemComponent) "/Game/Programming/Blueprints/Alchemist/Will-o-wisp/GA_Will-O-Wisp.GA_Will-O-Wisp_C" true))
    (if _returnvalue
      (CallFunction|ResetUltimate))))