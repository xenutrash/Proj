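; Player-controlled raid boss Nixa, with boosted health, reduced speed and Bite, Waterburst, Whirlpool and Submerge attacks.
; Inputs activate GAS abilities by tag, starting controller cooldowns and local/remote sounds; failed activations handle bite chaining, whirlpool cancel and reemerge.
; Helper events drive replicated VFX, camera boom lerp and mesh/collision toggling.
; Submerge fades a dynamic post-process material on the top-down camera, while damage briefly flashes an overlay.
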(event Custom|ToggleVisable
  ;[1 0.5873 0.9109 0.3] Helper functions
  ;;[1 0.2118 0.851] Toggle Vision (for submerge)
  (CallFunction|ToggleVisionFunc))

(event Custom|EffectsAllClients
  (params (Target :type Actor%20Component%20Object%20Reference))
  (Components|Activation|Activate Target false))

(event Custom|ActivateSubmergeVFX
  (params (Condition :type Boolean))
  (CallFunction|ActivateSubmergeVFXAllClients Condition))

(event Custom|ActivateSubmergeVFXAllClients
  (params (Condition :type Boolean))
  (bind _submergevfx (Variables|Default|GetSubmergeVFX))
  (if Condition
    (Components|Activation|Activate _submergevfx false)
    (else
      (Components|Activation|Deactivate _submergevfx))))

(event Custom|LerpGroundTarget
  ;[1 0.5873 0.9109 0.3] Helper functions
  ;;[1 0.2118 0.851] Camera Lerp In and Out
  (Utilities|FlowControl|FlipFlop
    (:A
      (Variables|Default|SetLerpIn? true)
      (bind _alpha (Timeline|LerpCamera PlayFromStart)
        (:Update
          (if (Variables|Default|GetLerpIn?)
            (Transformation|SetRelativeLocation (.CameraBoom (Utilities|NewMacro _alpha _alpha)) (Math|Vector|MakeVector (.RelativeLocation_X (Utilities|NewMacro _alpha _alpha)) (.RelativeLocation_Y (Utilities|NewMacro _alpha _alpha)) (.ReturnValue (Utilities|NewMacro _alpha _alpha))) false false)
            (else
              (Transformation|SetRelativeLocation (.CameraBoom (Utilities|NewMacro _alpha _alpha)) (Math|Vector|MakeVector (.RelativeLocation_X (Utilities|NewMacro _alpha _alpha)) (.RelativeLocation_Y (Utilities|NewMacro _alpha _alpha)) (.ReturnValue2 (Utilities|NewMacro _alpha _alpha))) false false))))))
    (:B
      (Variables|Default|SetLerpIn? false)
      (Timeline|LerpCamera PlayFromStart))))

(event Custom|Spawn%20Niagara%20System%20Multicast
  (params (SystemTemplate :type Niagara%20System%20Object%20Reference) (Location :type Vector))
  (Niagara|SpawnSystematLocation SystemTemplate Location))

(event Custom|SetWhirlPoolLocationMultiCast
  (params (Target :type BP%20Water%20Object%20Reference) (Location :type Vector))
  (Default|SetWhirlpoolLocation Target Location))

(event Custom|WhirlPoolAnimate
  (params (Target :type BP%20Water%20Object%20Reference))
  (bind _returnvalue (Transformation|GetActorTransform Target))
  (Default|AnimateRadius Target 0.0)
  (Default|PlaySoundLocally (Variables|Default|GetSoundSystem) "/Game/FMOD/Events/InWorld/LocalPlayer/Boss/Nixa/Local_Nixa_Whirlpool.Local_Nixa_Whirlpool" _returnvalue false)
  (Default|PlaySoundAllClientsExcludeOwner (Variables|Default|GetSoundSystem) "/Game/FMOD/Events/InWorld/NonLocalPlayer/Boss/Nixa/NonLocal_Nixa_Whirlpool.NonLocal_Nixa_Whirlpool" _returnvalue (Game|GetPlayerController 0) false))

(event Custom|PlayBiteVFX
  (params (Stage :type Integer))
  (bind _nixabiteready (Variables|Default|GetNixaBiteReady))
  (bind _slasheffect (Variables|Default|GetSlashEffect))
  (bind _slasheffect_2 (Variables|Default|GetSlashEffect))
  ;[1 1 1] Nixa bite vfx play
  (Math|Integer|CompareInt Stage 1
    (:>
      (Components|Activation|Deactivate _nixabiteready))
    (:==
      (Effects|Components|ParticleSystem|SetIntParameter _slasheffect "Slash Direction" -1)
      (Effects|Components|ParticleSystem|SetVectorParameter _slasheffect_2 "Splash Direction" "1.000000,1.000000,1.000000")
      (Components|Activation|Activate _slasheffect_2 true)
      (Components|Activation|Activate _nixabiteready true)
      (CallFunction|EffectsAllClients _nixabiteready))
    (:<
      (Effects|Components|ParticleSystem|SetIntParameter _slasheffect "Slash Direction" 1)
      (Effects|Components|ParticleSystem|SetVectorParameter _slasheffect_2 "Splash Direction" "1.000000,-1.000000,1.000000")
      (Components|Activation|Activate _slasheffect_2 true)
      (CallFunction|EffectsAllClients (Variables|Default|GetSlashEffect)))))

(event Custom|SubmergeReemergeCooldown
  ;[1 0.5873 0.9109 0.3] Helper functions
  (Utilities|FlowControl|FlipFlop
    (:A
      (Variables|Default|SetCanReemerge? true))
    (:B
      (Variables|Default|SetCanReemerge? false))))

(event Custom|Fade%20In%20Submerge%20PP
  ;[0 1 0.9931] Submerge VFX
  (bind _fade (Timeline|Fade%20Submerge Play)
    (:Update
      (Rendering|Material|SetScalarParameterValue (Variables|Default|GetPP_Submerge) "On/Off" _fade :!class /Script/Engine.MaterialInstanceDynamic))))

(event Custom|Fade%20Out%20Submerge%20PP
  ;[0 1 0.9931] Submerge VFX
  (bind _fade (Timeline|Fade%20Submerge Reverse)
    (:Update
      (Rendering|Material|SetScalarParameterValue (Variables|Default|GetPP_Submerge) "On/Off" _fade :!class /Script/Engine.MaterialInstanceDynamic))))

(event Input|EnhancedActionEvents|EnhancedInputActionIA_ConfirmAction
  (params (ActionValue :type Boolean) (ElapsedSeconds :type Float%20%28double-precision%29) (TriggeredSeconds :type Float%20%28double-precision%29) (InputAction :type Input%20Action%20Object%20Reference :default "/Game/Characters/Input/Inputs/IA_ConfirmAction.IA_ConfirmAction"))
  (Abilities|TryActivateAbilitiesbyTag (Variables|Default|GetAbilitySystemComponent) (GameplayTags|MakeLiteralGameplayTagContainer "(GameplayTags=((TagName=\"Event.Input.Confirm\")))") true))

(event EventOnHealthChanged
  (params (DeltaValue :type Float%20%28single-precision%29) (EventTags :type Gameplay%20Tag%20Container%20Structure%20%28by%20ref%29))
  (|CallParentFunction DeltaValue EventTags))

(event EventOnTaunt
  ;[0 0 0 0.3] Abilities
  ;;[0.003922 0.003922 0.003922] Kog ult
)

(event EventOnBasicAttack
  (bind _rootcomponent (Variables|Transformation|GetRootComponent))
  (bind _soundsystem (Variables|Default|GetSoundSystem))
  ;[0 0 0 0.3] Abilities
  ;;[0.003922 0.003922 0.003922] Bite
  (bind _returnvalue (Abilities|TryActivateAbilitiesbyTag (Variables|Default|GetAbilitySystemComponent) (GameplayTags|MakeGameplayTagContainerfromTag "(TagName=\"Attack.Active.Bite\")") true :!label _label))
  (if _returnvalue
    (Default|PlayEventAttachedLocally _soundsystem "/Game/FMOD/Events/InWorld/LocalPlayer/Boss/Nixa/Local_Nixa_NormalAttack.Local_Nixa_NormalAttack" _rootcomponent false)
    (Default|PlayEventAttachedAllClientsExcludeOwner _soundsystem "/Game/FMOD/Events/InWorld/NonLocalPlayer/Boss/Nixa/NonLocal_Nixa_NormalAttack.NonLocal_Nixa_NormalAttack" _rootcomponent (Game|GetPlayerController 0) false)
    (else
      (Ability|SendGameplayEventtoActor self "(TagName=\"Event.Bite.Trigger\")")
      (Ability|Async|WaitGameplayEventToActor 0 "(TagName=\"Event.Bite.BiteAgain\")"
        (:EventReceived
          (Utilities|FlowControl|Delay 0.05)
          (goto _label))))))

(event EventBeginPlay
  (|CallParentFunction)
  ;[1 1 1] Change max hp
  (CallFunction|AddtoMaxHealth 9e+02)
  (CallFunction|AddtoMaxSpeed -1.5e+02)
  (CallFunction|CreateDynamicSubmergePP))

(event EventTakeDamage
  (params (DamageAmount :type Float%20%28single-precision%29))
  (CallFunction|ChangeOverlayMaterialServer "/Game/Material/OverlayMaterial/M_Playerhit_Nixa_Inst.M_Playerhit_Nixa_Inst")
  (Utilities|FlowControl|Delay 0.1)
  (CallFunction|ChangeOverlayMaterialServer)
  (|CallParentFunction DamageAmount))

(event EventOnSpecialAttack
  (bind _soundsystem (Variables|Default|GetSoundSystem))
  (bind _rootcomponent (Variables|Transformation|GetRootComponent))
  ;[0 0 0 0.3] Abilities
  ;;[0.003922 0.003922 0.003922] Waterburst
  (bind _returnvalue (Abilities|TryActivateAbilitiesbyTag (Variables|Default|GetAbilitySystemComponent) (GameplayTags|MakeLiteralGameplayTagContainer "(GameplayTags=((TagName=\"Attack.Active.Waterburst\")))") true))
  (if _returnvalue
    (bind _asbp_proj_player_controller (Utilities|Casting|CastToBP_ProjPlayerController (Game|GetPlayerController 0)))
    (Default|StartCooldownE _asbp_proj_player_controller 2)
    (Default|PlayEventAttachedLocally _soundsystem "/Game/FMOD/Events/InWorld/LocalPlayer/Boss/Nixa/Local_Nixa_WaterOrbs.Local_Nixa_WaterOrbs" _rootcomponent false)
    (Default|PlayEventAttachedAllClientsExcludeOwner _soundsystem "/Game/FMOD/Events/InWorld/NonLocalPlayer/Boss/Nixa/NonLocal_Nixa_WaterOrbs.NonLocal_Nixa_WaterOrbs" _rootcomponent (Game|GetPlayerController 0) false)))

(event EventOnUltimateAttack
  ;[0 0 0 0.3] Abilities
  ;;[0.003922 0.003922 0.003922] Whirlpool
  (bind _returnvalue (Abilities|TryActivateAbilitiesbyTag (Variables|Default|GetAbilitySystemComponent) (GameplayTags|MakeLiteralGameplayTagContainer "(GameplayTags=((TagName=\"Attack.Active.Whirlpool\")))") true))
  (if _returnvalue
    (bind _asbp_proj_player_controller (Utilities|Casting|CastToBP_ProjPlayerController (Game|GetPlayerController 0)))
    (Default|StartCooldownQ _asbp_proj_player_controller 12)
    (else
      (Utilities|FlowControl|Delay 0.3)
      (Ability|SendGameplayEventtoActor self "(TagName=\"Event.Cancel.Whirlpool\")"))))

(event EventOnDash
  (bind _soundsystem (Variables|Default|GetSoundSystem))
  (bind _rootcomponent (Variables|Transformation|GetRootComponent))
  ;[0 0 0 0.3] Abilities
  ;;[0.003922 0.003922 0.003922] Submerge
  (bind _returnvalue (Abilities|TryActivateAbilitiesbyTag (Variables|Default|GetAbilitySystemComponent) (GameplayTags|MakeLiteralGameplayTagContainer "(GameplayTags=((TagName=\"Attack.Active.Submerge\")))") true))
  (if _returnvalue
    (bind _asbp_proj_player_controller (Utilities|Casting|CastToBP_ProjPlayerController (Game|GetPlayerController 0)))
    (Default|StartCooldownSpace _asbp_proj_player_controller 15)
    (Default|PlayEventAttachedLocally _soundsystem "/Game/FMOD/Events/InWorld/LocalPlayer/Boss/Nixa/Local_Nixa_Dive.Local_Nixa_Dive" _rootcomponent true "NixaDive")
    (Default|PlayEventAttachedAllClientsExcludeOwner _soundsystem "/Game/FMOD/Events/InWorld/NonLocalPlayer/Boss/Nixa/NonLocal_Nixa_Dive.NonLocal_Nixa_Dive" _rootcomponent (Game|GetPlayerController 0) true "NixaDive")
    (CallFunction|FadeinSubmergePP)
    (elif (Variables|Default|GetCanReemerge?)
      (Abilities|TryActivateAbilitiesbyTag (Variables|Default|GetAbilitySystemComponent) (GameplayTags|MakeLiteralGameplayTagContainer "(GameplayTags=((TagName=\"Event.Input.Confirm\")))") true)
      (CallFunction|SubmergeReemergeCooldown))))

(event Input|KeyboardEvents|DebugKeyC
  (params (Key :type Key%20Structure :default "None") (ActionValue :type Input%20Action%20Value%20Structure))
  (:Pressed
    (Abilities|TryActivateAbilitybyClass (Variables|Default|GetAbilitySystemComponent) "/Game/Programming/Blueprints/NixaRaidBoss/GA_FlowingTides.GA_FlowingTides_C" true)))

(fn ConstructionScript
  (|CallParentFunction))

(fn ToggleVisionFunc
  (bind _mesh (Variables|Character|GetMesh))
  (bind _mesh_2 (Variables|Character|GetMesh))
  (Utilities|FlowControl|FlipFlop
    (:A
      (Rendering|ToggleVisibility _mesh false)
      (Collision|SetCollisionEnabled _mesh_2 "NoCollision"))
    (:B
      (Rendering|ToggleVisibility _mesh true)
      (Collision|SetCollisionEnabled _mesh_2 "QueryAndPhysics"))))

(fn CreateDynamicSubmergePP
  (bind _returnvalue (Rendering|Material|CreateDynamicMaterialInstance "/Game/Material/PostProcess/PP_Submerge.PP_Submerge" "None" "None" :!class /Script/Engine.KismetMaterialLibrary))
  (bind _output_get (Variables|Default|SetPP_Submerge _returnvalue))
  (Variables|/Script/Engine.CameraComponent|SetPostProcessSettings (Variables|Default|GetTopDownCameraComponent) (Utilities|Struct|MakePostProcessSettings (Utilities|Struct|MakeWeightedBlendables (Utilities|Array|MakeArray (Utilities|Struct|MakeWeightedBlendable 1.0 _output_get))))))