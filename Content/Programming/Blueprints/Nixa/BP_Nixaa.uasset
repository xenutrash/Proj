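; BP_Nixaa is the Nixa player character, a child Blueprint that raises max health and speed and maps attack and dash inputs to Gameplay Ability System activations.
; Basic, special and ultimate attacks trigger abilities by class or tag, with successful special and submerge activations starting player-controller cooldowns.
; Dash alternates between submerging and sending a confirm tag via a boolean.
; Tick syncs walk speed to the Speed attribute, while FlipFlops toggle mesh visibility and timeline-driven camera boom height.
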(event Custom|ToggleVisable
  (bind _mesh (Variables|Character|GetMesh))
  (Utilities|FlowControl|FlipFlop
    (:A
      (Rendering|ToggleVisibility _mesh false)
      (Collision|SetCollisionEnabled (Variables|Character|GetMesh) "NoCollision"))
    (:B
      (Rendering|ToggleVisibility _mesh true)
      (Components|Activation|Activate (Variables|Default|GetSwirl) false))))

(event Custom|LerpGroundTarget
  (bind _cameraboom (Variables|Default|GetCameraBoom))
  (bind _relativelocation (Variables|/Script/Engine.SceneComponent|GetRelativeLocation _cameraboom))
  (Development|PrintString "Flip flop")
  (Utilities|FlowControl|FlipFlop
    (:A
      (bind _output_get (Variables|Default|SetLerpIn? true))
      (Development|PrintString (Utilities|String|ToString(Boolean) _output_get))
      (bind _alpha (Timeline|LerpCamera PlayFromStart)
        (:Update
          (if (Variables|Default|GetLerpIn?)
            (Development|PrintString "Lerp In")
            (Transformation|SetRelativeLocation _cameraboom (Math|Vector|MakeVector (.x _relativelocation) (.y _relativelocation) (Math|Float|Lerp (.z _relativelocation) (+ (.z _relativelocation) 5e+02) _alpha)) false false)
            (else
              (Development|PrintString "Lerp Out")
              (Transformation|SetRelativeLocation _cameraboom (Math|Vector|MakeVector (.x _relativelocation) (.y _relativelocation) (Math|Float|Lerp (.z _relativelocation) (- (.z _relativelocation) 5e+02) _alpha)) false false))))))
    (:B
      (bind _output_get_2 (Variables|Default|SetLerpIn? false))
      (Development|PrintString (Utilities|String|ToString(Boolean) _output_get_2))
      (Timeline|LerpCamera PlayFromStart))))

(event EventOnHealthChanged
  (params (DeltaValue :type Float%20%28single-precision%29) (EventTags :type Gameplay%20Tag%20Container%20Structure%20%28by%20ref%29))
  (|CallParentFunction DeltaValue EventTags))

(event EventOnTaunt
  (Development|PrintString "Taunt"))

(event EventOnBasicAttack
  ;[1 1 1] Bite
  (Abilities|TryActivateAbilitybyClass (Variables|Default|GetAbilitySystemComponent) "/Game/Programming/Blueprints/Nixa/Abilities/Bite/GA_Bite.GA_Bite_C" true)
  (Components|Activation|Activate (Variables|Default|GetBiteEffect) false))

(event EventBeginPlay
  (|CallParentFunction)
  ;[1 1 1] Change max hp
  (CallFunction|AddtoMaxHealth 9e+02)
  (CallFunction|AddtoMaxSpeed 1.5e+02))

(event EventTick
  (params (DeltaSeconds :type Float%20%28single-precision%29))
  ;[1 1 1] que?
  (Variables|/Script/Engine.CharacterMovementComponent|SetMaxWalkSpeed (Variables|Character|GetCharacterMovement) (.currentvalue (Variables|/Script/Proj.RushAttributeSet|GetSpeed (Variables|Default|GetAttributes)))))

(event EventOnSpecialAttack
  ;[1 1 1] Secondary E = Waterburst
  (bind _returnvalue (Abilities|TryActivateAbilitiesbyTag (Variables|Default|GetAbilitySystemComponent) (GameplayTags|MakeLiteralGameplayTagContainer "(GameplayTags=((TagName=\"Attack.Boss.Main\")))") true))
  (if _returnvalue
    (bind _asbp_proj_player_controller (Utilities|Casting|CastToBP_ProjPlayerController (Game|GetPlayerController 0)))
    (Default|StartCooldownE _asbp_proj_player_controller 2)))

(event EventOnUltimateAttack
  (Abilities|TryActivateAbilitybyClass (Variables|Default|GetAbilitySystemComponent) "/Game/Programming/Blueprints/Nixa/Abilities/Bite/GA_KogUlt.GA_KogUlt_C" true))

(event EventOnDash
  (if (Variables|Default|GetCanReactivateSubmerge)
    (Variables|Default|SetCanReactivateSubmerge false)
    (Abilities|TryActivateAbilitiesbyTag (Variables|Default|GetAbilitySystemComponent) (GameplayTags|MakeLiteralGameplayTagContainer "(GameplayTags=((TagName=\"Event.Input.Confirm\")))") true)
    (else
      (Variables|Default|SetCanReactivateSubmerge true)
      (bind _returnvalue (Abilities|TryActivateAbilitiesbyTag (Variables|Default|GetAbilitySystemComponent) (GameplayTags|MakeLiteralGameplayTagContainer "(GameplayTags=((TagName=\"Attack.Submerge\")))") true))
      (if _returnvalue
        (bind _asbp_proj_player_controller (Utilities|Casting|CastToBP_ProjPlayerController (Game|GetPlayerController 0)))
        (Default|StartCooldownSpace _asbp_proj_player_controller 15)))))

(event EventOnMove)

(fn ConstructionScript
  (|CallParentFunction))