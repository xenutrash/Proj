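; Gameplay Ability for Nixa's Water Burst, which fires a fan of burst projectiles on a cooldown.
; On authority, it plays a montage and waits for the Bite1 gameplay event to spawn the projectiles in front of the avatar.
; Yaw steps by Spread per projectile from an Offset, with pitch flattened and spawn height fixed.
; The ability ends when the montage completes, blends out or is interrupted or cancelled.
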(event Ability|EventActivateAbility
  (bind _returnvalue (Ability|GetAvatarActorfromActorInfo))
  (bind _returnvalue_2 (Ability|GetAvatarActorfromActorInfo))
  (bind _returnvalue_3 (Ability|GetAvatarActorfromActorInfo))
  (bind _returnvalue_4 (Ability|GetAvatarActorfromActorInfo))
  (bind _returnvalue_5 (Transformation|GetActorRotation _returnvalue))
  (bind _returnvalue_6 (Transformation|GetActorRotation _returnvalue_2))
  (bind _returnvalue_7 (Transformation|GetActorLocation _returnvalue_4))
  (bind (_roll _pitch _yaw) (Math|Rotator|BreakRotator _returnvalue_5))
  (bind _returnvalue_8 (Math|Vector|GetForwardVector _returnvalue_6))
  (bind _returnvalue_9 (* _returnvalue_8 "100.000000,100.000000,100.000000"))
  (bind _returnvalue_10 (+ _returnvalue_9 _returnvalue_7))
  (Variables|Default|SetCooldown 1e+01)
  (Utilities|Casting|CastToPawn (Ability|GetAvatarActorfromActorInfo)
    (:then
      (Ability|CommitAbilityCooldown false)
      (Ability|HasAuthority
        (:True
          (|PlayMontageandWaitProxy "None" 0 1.0 "None" true 1.0 0.0 false
            (:then
              (if (Networking|IsServer)
                (Ability|Tasks|WaitGameplayEvent "(TagName=\"Event.Montage.Bite1\")" 0
                  (:EventReceived
                    (for _index (range 1 (Variables|Default|GetProjectileCount))
                      (bind _returnvalue_11 (Game|SpawnActorfromClass "/Game/Programming/Blueprints/Nixa/Abilities/WaterBurst/BP_NixaBurstProjectile.BP_NixaBurstProjectile_C" (Math|Transform|MakeTransform (Math|Vector|MakeVector (.x _returnvalue_10) (.y _returnvalue_10) 35.0) (Math|Rotator|CombineRotators (Math|Rotator|MakeRotator _roll 0.0 (+ _yaw (Variables|Default|Getoffset))) (* (Math|Rotator|MakeRotator 0.0 0.0 (Variables|Default|GetSpread)) _index)) "1.000000,1.000000,1.000000") "Undefined" "MultiplyWithRoot" _returnvalue_3 0))
                      (Actor|SetOwner _returnvalue_11 _returnvalue_3))))
                (else
                  (Ability|EndAbility))))
            (:OnCompleted
              (Ability|EndAbility :!label _label))
            (:OnBlendOut
              (goto _label))
            (:OnInterrupted
              (goto _label))
            (:OnCancelled
              (goto _label))))))
    (:CastFailed
      (Development|PrintString "Pawn cast failed"))))

(event Ability|EventOnEndAbility
  (params (bWasCancelled :type Boolean)))