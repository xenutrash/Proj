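; Nixa's Water Burst projectile, which damages Hero-tagged characters on overlap and breaks on static meshes.
; Hit logic runs on the server, spawning a splash through a multicast, damaging and scoring for the owner, then destroying the projectile.
; Damage derives from time since creation, though the formula as written yields negative values and BaseDamage is never read.
; The box-growing IncreaseSize event has its looping timer disconnected.
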(event OnComponentBeginOverlap(Box)
  (params (OverlappedComponent :type Primitive%20Component%20Object%20Reference) (OtherActor :type Actor%20Object%20Reference) (OtherComp :type Primitive%20Component%20Object%20Reference) (OtherBodyIndex :type Integer) (bFromSweep :type Boolean) (SweepResult :type Hit%20Result%20Structure%20%28by%20ref%29))
  (bind _returnvalue (Actor|GetGameTimeSinceCreation))
  (bind _returnvalue_2 (Actor|GetGameTimeSinceCreation))
  (bind _returnvalue_3 (* _returnvalue_2 13.0))
  (bind _returnvalue_4 (- _returnvalue _returnvalue_3))
  (if (Networking|IsServer)
    (if (not (Variables|Default|GetDisableHits))
      (if (Actor|ActorHasTag OtherActor "Hero")
        (Variables|Default|SetDisableHits true)
        (CallFunction|CreateWaterImpactEffect)
        (if (not (Utilities|Array|ContainsItem (Variables|Default|GetCharactersHit) OtherActor))
          (Utilities|Array|Add (Variables|Default|GetCharactersHit) OtherActor)
          (bind _asbp_rush_character (Utilities|Casting|CastToBP_RushCharacter OtherActor))
          (Default|TakeDamage _asbp_rush_character _returnvalue_4)
          (Default|UpdateScore _asbp_rush_character (Components|GetOwner) _returnvalue_4)
          (Actor|SetLifeSpan 0.1)
          (Actor|DestroyActor))
        (else
          (Utilities|Casting|CastToStaticMeshActor OtherActor)
          (Variables|Default|SetDisableHits true)
          (CallFunction|CreateWaterImpactEffect)
          (Rendering|SetActorHiddenInGame true)
          (Utilities|FlowControl|Delay 2.0)
          (Actor|DestroyActor))))))

(event Custom|IncreaseSize
  (bind _box (Variables|Default|GetBox))
  ;[1 1 1] Increases the size of the projectile
  (Transformation|SetWorldScale3D _box (+ (Transformation|GetWorldScale _box) "0.060000,0.060000,0.060000")))

(event Custom|CreateWaterImpactEffect
  (CallFunction|CreateWaterImpactEffectMulticast))

(event Custom|CreateWaterImpactEffectMulticast
  (Niagara|SpawnSystematLocation "/Game/Niagara/NS_SplashImpact.NS_SplashImpact" (Transformation|GetActorLocation)))

(event EventBeginPlay
  (Variables|Default|SetBaseDamage (Actor|GetGameTimeSinceCreation)))

(fn ConstructionScript)