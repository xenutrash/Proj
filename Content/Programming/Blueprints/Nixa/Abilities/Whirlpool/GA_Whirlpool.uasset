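; Gameplay ability for Nixa that places a ground-targeted whirlpool and knocks back pawns caught in it.
; A mouse-location actor feeds target-data confirmation, while a parallel four-second timer ends the ability.
; Confirming plays a montage, moves the whirlpool on the level's BP_Water through Nixa's multicasts and shows a Niagara indicator.
; After a delay, a sphere trace activates GA_KnockBackWhirlpool on hit actors and sends them the location by gameplay event.
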(event Ability|EventOnEndAbility
  (params (bWasCancelled :type Boolean))
  (Development|PrintString "Ability ended lerping in")
  (Default|LerpGroundTarget (stale Ability|EventActivateAbility _asbp_nixaa)))

(event Ability|EventActivateAbility
  (bind _returnvalue (Ability|GetAvatarActorfromActorInfo))
  (Utilities|Array|Clear (Variables|Default|GetHit%20Actor))
  (Ability|GameplayEffect|AddLooseGameplayTags (Ability|GetAvatarActorfromActorInfo) (GameplayTags|MakeLiteralGameplayTagContainer "(GameplayTags=((TagName=\"Attack.Block.Bite\")))"))
  (Ability|CommitAbilityCooldown false)
  (bind _asbp_nixaa (Utilities|Casting|CastToBP_Nixaa (Ability|GetAvatarActorfromActorInfo)))
  (Default|LerpGroundTarget _asbp_nixaa)
  (bind _returnvalue_2 (Game|SpawnActorfromClass "/Game/Meshes/BP_MouseLocation.BP_MouseLocation_C" (Math|Transform|MakeTransform (Transformation|GetActorLocation (Ability|GetAvatarActorfromActorInfo)) "0, 0, 0" "1.000000,1.000000,1.000000") "Undefined" "MultiplyWithRoot" 0 0))
  (|WaitTargetData :ConfirmationType "UserConfirmed" :Class "/Game/Programming/Blueprints/Nixa/Abilities/Submerge/BP_WhirlPoolGroundTrace.BP_WhirlPoolGroundTrace_C" :bTraceAffectsAimPitch false :StartLocation (Utilities|Struct|MakeGameplayAbilityTargetingLocationInfo "ActorTransform" "0.000000,0.000000,0.000000|0.000000,0.000000,-0.000000|1.000000,1.000000,1.000000" _returnvalue_2) :ReticleClass "/Script/GameplayAbilities.GameplayAbilityWorldReticle" :Filter (Filter|MakeFilterHandle (Utilities|Struct|MakeGameplayTargetDataFilter 0 "TDFS_Any") 0)
    (:then
      (Utilities|FlowControl|Delay 4.0)
      (Default|DestoryMouseActor _returnvalue_2)
      (Ability|CommitAbilityCooldown false)
      (Ability|EndAbility))
    (:ValidData
      (|PlayMontageandWaitProxy "None" "/Game/Animation/Nixa/Montages/Joel.Joel" 1.0 "None" false 1.0 0.0 false
        (:then
          (Ability|CommitAbilityCooldown false)
          (bind _output_get (Variables|Default|SetMouse%20Location (Transformation|GetActorLocation _returnvalue_2)))
          (CallFunction|SpawnWhirlpoolatLocation _output_get)
          (bind _asbp_nixaa_2 (Utilities|Casting|CastToBP_Nixaa _returnvalue))
          (Default|WhirlPoolAnimate _asbp_nixaa_2 (Variables|Default|GetSpawnedWater))
          (bind _asbp_nixaa_3 (Utilities|Casting|CastToBP_Nixaa _returnvalue))
          (Default|SpawnNiagaraSystemMulticast _asbp_nixaa_3 "/Game/Niagara/NS_Whirlpool_Indicator.NS_Whirlpool_Indicator" _output_get)
          (Utilities|FlowControl|Delay (Variables|Default|GetDuration))
          (Default|PlaySoundLocally (Variables|/Game/Programming/Blueprints/BP_RushCharacter.BP_RushCharacter_C|GetSoundSystem _asbp_nixaa_3) "/Game/FMOD/Events/InWorld/LocalPlayer/Boss/Nixa/Local_Nixa_Whirlpool.Local_Nixa_Whirlpool" (Math|Conversions|ToTransform(Vector) _output_get) false)
          (Default|PlaySoundAllClientsExcludeOwner (Variables|/Game/Programming/Blueprints/BP_RushCharacter.BP_RushCharacter_C|GetSoundSystem _asbp_nixaa_3) "/Game/FMOD/Events/InWorld/NonLocalPlayer/Boss/Nixa/NonLocal_Nixa_Whirlpool.NonLocal_Nixa_Whirlpool" (Math|Conversions|ToTransform(Vector) _output_get) (Game|GetPlayerController 0) false)
          (bind (_outhits _returnvalue_3) (Collision|MultiSphereTraceForObjects _output_get _output_get 3.8e+02 (Utilities|Array|MakeArray "ObjectTypeQuery3") false 0 "ForDuration" true "(R=1.000000,G=0.000000,B=0.000000,A=1.000000)" "(R=0.000000,G=1.000000,B=0.000000,A=1.000000)" 1.0))
          (if _returnvalue_3
            (for _array_element _outhits
              (Utilities|Array|AddUnique (Variables|Default|GetHit%20Actor) (.HitActor (Collision|BreakHitResult _array_element))))
            (for _array_element_2 (Variables|Default|GetHit%20Actor)
              (Utilities|IsValid (Ability|GetAbilitySystemComponent _array_element_2)
                (:Is%20Valid
                  (Abilities|TryActivateAbilitybyClass (Ability|GetAbilitySystemComponent _array_element_2) "/Game/Programming/Blueprints/Nixa/Abilities/Bite/GA_KnockBackWhirlpool.GA_KnockBackWhirlpool_C" true)
                  (Ability|SendGameplayEventtoActor _array_element_2 "(TagName=\"GameplayCue.Test\")" (Utilities|Struct|MakeGameplayEventData "(TagName=\"\")" 0 _array_element_2 0 0 "()" "(GameplayTags=)" "(GameplayTags=)" 1e+01 (Class|AbilitySystemBlueprintLibrary|AbilityTargetDatafromLocations (Utilities|Struct|MakeGameplayAbilityTargetingLocationInfo "LiteralTransform" (Math|Transform|MakeTransform _output_get)) (Utilities|Struct|MakeGameplayAbilityTargetingLocationInfo "LiteralTransform" (Math|Transform|MakeTransform _output_get)))))
                  (Utilities|FlowControl|Delay 0.05)
                  (Ability|SendGameplayEventtoActor _array_element_2 "(TagName=\"GameplayCue.Test\")" (Utilities|Struct|MakeGameplayEventData "(TagName=\"\")" 0 _array_element_2 0 0 "()" "(GameplayTags=)" "(GameplayTags=)" 1e+01 (Class|AbilitySystemBlueprintLibrary|AbilityTargetDatafromLocations (Utilities|Struct|MakeGameplayAbilityTargetingLocationInfo "LiteralTransform" (Math|Transform|MakeTransform _output_get)) (Utilities|Struct|MakeGameplayAbilityTargetingLocationInfo "LiteralTransform" (Math|Transform|MakeTransform _output_get))))))))
            (Utilities|FlowControl|Delay 1.0)
            (Ability|EndAbility)
            (else
              (Development|PrintString "Ability Ended no hits")
              (Ability|EndAbility))))))))

(fn SpawnWhirlpoolatLocation
  (params (Pos :type Vector))
  (if (Utilities|IsValid (Variables|Default|GetSpawnedWater))
    _
    (else
      (bind _returnvalue (Actor|GetActorOfClass "/Game/Programming/Blueprints/Gameplay/LevelEffects/BP_Water.BP_Water_C"))
      (Variables|Default|SetSpawnedWater _returnvalue)))
  (bind _asbp_nixaa (Utilities|Casting|CastToBP_Nixaa (Ability|GetAvatarActorfromActorInfo)))
  (Default|SetWhirlPoolLocationMultiCast _asbp_nixaa (Variables|Default|GetSpawnedWater) Pos))