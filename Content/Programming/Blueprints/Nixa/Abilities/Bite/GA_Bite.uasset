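; Gameplay ability for a bite attack that cycles through a three-step combo counter, playing the same bite montage at each step.
; On the Bite1 montage event, a sphere trace for pawns, apparently in front of the avatar, collects targets with ability systems.
; The first two steps call TakeDamage on BP_RushCharacter targets, while the third activates GA_Knockback on the target.
; An end-ability macro advances and wraps the counter.
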(event Ability|EventActivateAbility
  (bind (_start_x _start_y _start_z _end_x _end_y _end_z) (|Sphereinputs))
  (|PlayMontageandWaitProxy "None" (Utilities|Select :Index (Variables|Default|GetIntCounter) :Option%200 "/Game/Animation/Nixa/Montages/Bite_Montage.Bite_Montage" :Option%201 "/Game/Animation/Nixa/Montages/Bite_Montage.Bite_Montage" :Option%202 "/Game/Animation/Nixa/Montages/Bite_Montage.Bite_Montage") 0.8 "None" true 1.0 0.0 false
    (:then
      (Ability|Tasks|WaitGameplayEvent "(TagName=\"Event.Montage.Bite1\")" 0
        (:EventReceived
          (bind (_outhits _returnvalue) (Collision|MultiSphereTraceForObjects (Math|Vector|MakeVector _start_x _start_y _start_z) (Math|Vector|MakeVector _end_x _end_y _end_z) 1.8e+02 (Utilities|Array|MakeArray "ObjectTypeQuery3") false 0 "None"))
          (if _returnvalue
            (for _array_element _outhits
              (Utilities|Array|AddUnique (Variables|Default|GetHit%20Actor) (.HitActor (Collision|BreakHitResult _array_element))))
            (for _array_element_2 (Variables|Default|GetHit%20Actor)
              (Utilities|IsValid (Ability|GetAbilitySystemComponent _array_element_2)
                (:Is%20Valid
                  (switch int (Variables|Default|GetIntCounter)
                    (:Default
                      (bind _asbp_rush_character (Utilities|Casting|CastToBP_RushCharacter _array_element_2 :!label _label)
                        (:then
                          (Default|TakeDamage _asbp_rush_character -1e+01)
                          (Ability|EndAbility :!label _label_2))
                        (:CastFailed
                          (Development|PrintString "failed to cast"))))
                    (:0
                      (goto _label))
                    (:1
                      (goto _label))
                    (:2
                      (bind _returnvalue_2 (Abilities|TryActivateAbilitybyClass (Ability|GetAbilitySystemComponent _array_element_2) "/Game/Programming/Blueprints/Nixa/GA_Knockback.GA_Knockback_C" true))
                      (Development|PrintString (Utilities|String|ToString(Boolean) _returnvalue_2))
                      (goto _label_2))))))
            (Utilities|EndAbilityMacro)))))
    (:OnCompleted
      (Utilities|EndAbilityMacro :!label _label_3))
    (:OnBlendOut
      (goto _label_3))
    (:OnInterrupted
      (goto _label_3))
    (:OnCancelled
      (goto _label_3))))

(event Ability|EventOnEndAbility
  (params (bWasCancelled :type Boolean)))