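; Gameplay Ability for Nixa's Kog ultimate, a ground-targeted cast that spawns BP_KogUlt at a chosen location.
; On activation it calls LerpGroundTarget on BP_Nixaa, then after a short delay spawns a mouse-location helper actor as the source for user-confirmed WaitTargetData.
; Confirming spawns the ult at the helper, destroys it and ends after a delay; cancelling cleans up and ends immediately.
; Ending the ability calls LerpGroundTarget again.
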(event Ability|EventActivateAbility
  (bind _returnvalue (Ability|GetAvatarActorfromActorInfo))
  (bind _asbp_nixaa (Utilities|Casting|CastToBP_Nixaa (Ability|GetAvatarActorfromActorInfo)))
  (Default|LerpGroundTarget _asbp_nixaa)
  (Utilities|FlowControl|Delay 0.2)
  (bind _returnvalue_2 (Game|SpawnActorfromClass "/Game/Meshes/BP_MouseLocation.BP_MouseLocation_C" (Math|Transform|MakeTransform (Transformation|GetActorLocation _returnvalue) "0, 0, 0" "1.000000,1.000000,1.000000") "Undefined" "MultiplyWithRoot" 0 0))
  (|WaitTargetData :ConfirmationType "UserConfirmed" :Class "/Game/Programming/Blueprints/Nixa/Abilities/Submerge/BP_SubmergeGroundTrace.BP_SubmergeGroundTrace_C" :TraceProfile "(Name=\"Spectator\")" :bTraceAffectsAimPitch false :StartLocation (Utilities|Struct|MakeGameplayAbilityTargetingLocationInfo "ActorTransform" "0.000000,0.000000,0.000000|0.000000,0.000000,-0.000000|1.000000,1.000000,1.000000" _returnvalue_2) :ReticleClass "/Script/GameplayAbilities.GameplayAbilityWorldReticle" :Filter (Filter|MakeFilterHandle (Utilities|Struct|MakeGameplayTargetDataFilter 0 "TDFS_Any") 0)
    (:ValidData
      (Game|SpawnActorfromClass "/Game/Programming/Blueprints/Nixa/Abilities/Bite/BP_KogUlt.BP_KogUlt_C" (Math|Transform|MakeTransform (Transformation|GetActorLocation _returnvalue_2) "0, 0, 0" "1.000000,1.000000,1.000000") "Undefined" "MultiplyWithRoot" _returnvalue 0)
      (Default|DestoryMouseActor _returnvalue_2)
      (Utilities|FlowControl|Delay 4.0)
      (Ability|EndAbility))
    (:Cancelled
      (Default|DestoryMouseActor _returnvalue_2)
      (Ability|EndAbility))))

(event Ability|EventOnEndAbility
  (params (bWasCancelled :type Boolean))
  (Default|LerpGroundTarget (stale Ability|EventActivateAbility _asbp_nixaa)))