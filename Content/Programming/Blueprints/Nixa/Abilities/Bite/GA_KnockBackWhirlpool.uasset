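; Gameplay ability for a whirlpool effect that drags a rush character toward a point and temporarily slows movement.
; On activation it computes a slow from the avatar's max walk speed, then waits once for a GameplayCue.Test event.
; The event prints debug text and applies root-motion force toward the target data's origin.
; It then reduces the payload target's max speed, restores it after a delay, and ends.
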(event Ability|EventActivateAbility
  (bind _asbp_rush_character (Utilities|Casting|CastToBP_RushCharacter (Ability|GetAvatarActorfromActorInfo)))
  (Variables|Default|SetSlow (* (Variables|Default|GetSlowPercentAmount) (Variables|/Script/Engine.CharacterMovementComponent|GetMaxWalkSpeed (Variables|/Script/Engine.Character|GetCharacterMovement _asbp_rush_character))))
  (bind _payload (Ability|Tasks|WaitGameplayEvent "(TagName=\"GameplayCue.Test\")" 0 true)
    (:EventReceived
      (Development|PrintString "KNOCKED" true true "(R=1.000000,G=0.159240,B=0.079553,A=1.000000)" 2345.0)
      (Ability|Tasks|ApplyRootMotionConstantForce "None" (Math|Vector|GetForwardVector (Math|Rotator|FindLookatRotation (Transformation|GetActorLocation (Ability|GetAvatarActorfromActorInfo)) (.location (Class|AbilitySystemBlueprintLibrary|GetTargetDataOrigin (.TargetData (Utilities|Struct|BreakGameplayEventData _payload)))))) 1.1e+03 0.3 false 0 "MaintainLastRootMotionVelocity"
        (:then
          (bind _asbp_rush_character_2 (Utilities|Casting|CastToBP_RushCharacter (.Target (Utilities|Struct|BreakGameplayEventData _payload))))
          (Default|AddtoMaxSpeed _asbp_rush_character_2 (* -1.0 (Variables|Default|GetSlow)))
          ;[1 1 1] Slow length after dragged in?
          (Utilities|FlowControl|Delay (Variables|Default|GetTimeSlowed))
          (Default|AddtoMaxSpeed _asbp_rush_character_2 (Variables|Default|GetSlow))
          (Ability|EndAbility))))))