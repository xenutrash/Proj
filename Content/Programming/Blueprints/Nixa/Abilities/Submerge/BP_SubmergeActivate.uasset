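; Short-lived area-damage actor for Nixa's Submerge ability that hits Hero-tagged characters once, then destroys itself.
; Shortly after spawning, it gathers overlapping BP_RushCharacters from its Sphere in a single query rather than through overlap events.
; Each unique target with an Ability System Component takes damage through TakeDamage, with UpdateScore crediting the actor's owner.
; The GA_Knockback activation is disconnected and marked as removed.
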(event OnComponentBeginOverlap(Sphere)
  (params (OverlappedComponent :type Primitive%20Component%20Object%20Reference) (OtherActor :type Actor%20Object%20Reference) (OtherComp :type Primitive%20Component%20Object%20Reference) (OtherBodyIndex :type Integer) (bFromSweep :type Boolean) (SweepResult :type Hit%20Result%20Structure%20%28by%20ref%29)))

(event Custom|GetCharactersInHitbox
  (for _array_element (Collision|GetOverlappingActors (Variables|Default|GetSphere) "/Game/Programming/Blueprints/BP_RushCharacter.BP_RushCharacter_C" :!class /Script/Engine.PrimitiveComponent)
    (if (Actor|ActorHasTag _array_element "Hero")
      (Utilities|Array|AddUnique (Variables|Default|GetOther%20Actor) _array_element)))
  (CallFunction|DealDamage))

(event Custom|DealDamage
  (for _array_element (Variables|Default|GetOther%20Actor)
    (if (Utilities|Array|ContainsItem (Variables|Default|GetPlayersAlreadyHit) _array_element)
      (Development|PrintString "Already hit")
      (else
        (Utilities|IsValid (Ability|GetAbilitySystemComponent _array_element)
          (:Is%20Valid
            (bind _asbp_rush_character (Utilities|Casting|CastToBP_RushCharacter _array_element))
            (Default|TakeDamage _asbp_rush_character (Variables|Default|GetDamageToDeal))
            (Default|UpdateScore _asbp_rush_character (Components|GetOwner) (Variables|Default|GetDamageToDeal))
            (Utilities|Array|AddUnique (Variables|Default|GetPlayersAlreadyHit) _array_element))))))
  (Actor|DestroyActor))

(event EventBeginPlay
  (Utilities|FlowControl|Delay 0.15)
  (CallFunction|GetCharactersinHitbox))

(fn ConstructionScript)