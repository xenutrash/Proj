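; Gameplay ability for Nixa's submerge: she dives out of sight with a speed boost, then emerges with an attack.
; A random dive montage leads into hidden mesh, disabled collision and overlaps, VFX and a passive effect.
; A 3.5-second timer or Confirm input, which also removes the effect, triggers the emerge montage and damage-actor spawn.
; The Attack.Submerge event reverts boost, VFX, audio and post-process, then ends the ability.
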(event Ability|EventActivateAbility
  (if (Variables|Default|GetSubmerged)
    (Development|PrintString "REACTIVATED")
    (else
      (CallFunction|StartSequence)
      (|PlayMontageandWaitProxy "None" (CallFunction|GetRandomMontage) 1.0 "None" true 1.0 0.0 false
        (:OnBlendOut
          (bind _returnvalue (CallFunction|MiddleSequence))
          (CallFunction|ToggleCollison)
          (Ability|Tasks|WaitGameplayEvent "(TagName=\"Event.Input.Confirm\")" (Variables|Default|GetNixa%20Character) true
            (:then
              (Utilities|FlowControl|Delay 3.5)
              (Variables|Default|SetSubmerged false :!label _label)
              (|PlayMontageandWaitProxy "None" "/Game/Animation/Nixa/Montages/Emerge_1_Montage.Emerge_1_Montage" 1.0 "None" false 1.0 0.0 false
                (:then
                  (Ability|Tasks|WaitGameplayEvent "(TagName=\"Attack.Submerge\")" 0 true
                    (:then
                      (Utilities|FlowControl|Delay 0.1)
                      (CallFunction|ToogleVisability)
                      (CallFunction|SpawnDamage))
                    (:EventReceived
                      (CallFunction|EndSequence)
                      (Utilities|FlowControl|Delay 0.15)
                      (CallFunction|SetGenerateOverlapEvents true (Variables|Default|GetNixa%20Character))
                      (Ability|EndAbility))))
                (:OnInterrupted
                  (Ability|EndAbility :!label _label_2))
                (:OnCancelled
                  (goto _label_2))))
            (:EventReceived
              (GameplayEffects|RemoveActiveGameplayEffect (Ability|GetAbilitySystemComponent (Variables|Default|GetNixa%20Character)) _returnvalue -1)
              (if (Variables|Default|GetSubmerged)
                (goto _label)))))))))

(event Ability|EventOnEndAbility
  (params (bWasCancelled :type Boolean))
  (bind _nixa_character (Variables|Default|GetNixa%20Character))
  (Variables|Default|SetSubmerged false)
  (CallFunction|ToogleVisability)
  (CallFunction|SetGenerateOverlapEvents true (Variables|Default|GetNixa%20Character))
  (if (<= (Variables|Default|GetSpeed) 0.0)
    _
    (else
      (Variables|/Script/Engine.CharacterMovementComponent|SetMaxWalkSpeed (Variables|/Script/Engine.Character|GetCharacterMovement _nixa_character) (Variables|Default|GetSpeed))))
  (CallFunction|StopAudio _nixa_character)
  (Default|ActivateSubmergeVFX (Variables|Default|GetNixa%20Character) false))

(fn SetGenerateOverlapEvents
  (params (Generate%20Overlap%20Events :type Boolean) (Actor :type Actor%20Object%20Reference))
  (bind _asbp_nixaa (Utilities|Casting|CastToBP_Nixaa Actor))
  (Default|SetOverlapping _asbp_nixaa Generate%20Overlap%20Events))

(fn GetNixaReference
  (Utilities|IsValid (Variables|Default|GetNixa%20Character)
    (:Is%20Not%20Valid
      (bind _asbp_nixaa (Utilities|Casting|CastToBP_Nixaa (Ability|GetAvatarActorfromActorInfo)))
      (Variables|Default|SetNixa%20Character _asbp_nixaa))))

(fn GetRandomMontage
  (bind _animationlist (Variables|Default|GetAnimationList))
  (return (Utilities|Array|Get(acopy) _animationlist (Math|Random|RandomInteger (Utilities|Array|Length _animationlist)))))

(fn ToogleVisability
  (bind _nixa_character (Variables|Default|GetNixa%20Character))
  (bind _mesh (Variables|/Script/Engine.Character|GetMesh _nixa_character))
  (if (Variables|Default|GetSubmerged)
    (Rendering|SetVisibility _mesh false false)
    (else
      (Rendering|SetVisibility _mesh true true))))

(fn SpawnDamage
  (Utilities|IsValid (Variables|Default|GetSpawnedObject)
    (:Is%20Valid
      (Development|PrintString "I already exis"))
    (:Is%20Not%20Valid
      (bind _returnvalue (Game|SpawnActorfromClass "/Game/Programming/Blueprints/Nixa/Abilities/Submerge/BP_SubmergeActivate.BP_SubmergeActivate_C" (Math|Transform|MakeTransform (Transformation|GetActorLocation (Ability|GetAvatarActorfromActorInfo)) "0, 0, 0" "1.000000,1.000000,1.000000") "Undefined" "MultiplyWithRoot" (Variables|Default|GetNixa%20Character) 0))
      (Variables|Default|SetSpawnedObject _returnvalue))))

(fn EndSequence
  (bind _nixa_character (Variables|Default|GetNixa%20Character))
  (Default|ActivateSubmergeVFX (Variables|Default|GetNixa%20Character) false)
  (Default|AddtoMaxSpeed _nixa_character -3e+02)
  (Default|EventInstanceAttatchedSetParameter (Variables|/Game/Programming/Blueprints/BP_RushCharacter.BP_RushCharacter_C|GetSoundSystem _nixa_character) "Nixa_Dive" 1.0 "NixaDive")
  (Default|FadeOutSubmergePP (Variables|Default|GetNixa%20Character)))

(fn MiddleSequence
  (bind _nixa_character (Variables|Default|GetNixa%20Character))
  (Default|ActivateSubmergeVFX _nixa_character true)
  (Default|AddtoMaxSpeed _nixa_character 3e+02)
  (CallFunction|ToogleVisability)
  (CallFunction|SetGenerateOverlapEvents false _nixa_character)
  (bind _returnvalue (GameplayEffects|ApplyGameplayEffectToSelf :self (Ability|GetAbilitySystemComponent _nixa_character) :GameplayEffectClass "/Game/Programming/Blueprints/Nixa/Abilities/Submerge/GE_NixaSubmergePassive.GE_NixaSubmergePassive_C"))
  (return _returnvalue))

(fn StartSequence
  (Ability|CommitAbilityCooldown false)
  (Ability|HasAuthority
    (:True
      (CallFunction|GetNixaReference)
      (Variables|Default|SetSpeed (Variables|/Script/Engine.CharacterMovementComponent|GetMaxWalkSpeed (Variables|/Script/Engine.Character|GetCharacterMovement (Variables|Default|GetNixa%20Character))))
      (Variables|Default|SetSubmerged true))))

(fn ToggleCollison
  (bind _nixa_character (Variables|Default|GetNixa%20Character))
  (bind _mesh (Variables|/Script/Engine.Character|GetMesh _nixa_character))
  (if (Variables|Default|GetSubmerged)
    (Collision|SetCollisionEnabled _mesh "NoCollision")
    (Development|PrintString "YOU CAN'T SEE ME ANYMORE :3")
    (else
      (Collision|SetCollisionEnabled _mesh "QueryAndPhysics")
      (Development|PrintString "YOU CAN SEE ME NOW"))))

(fn StopAudio
  (params (self2 :type BP%20Rush%20Character%20Object%20Reference))
  (bind _soundsystem (Variables|/Game/Programming/Blueprints/BP_RushCharacter.BP_RushCharacter_C|GetSoundSystem self2))
  (Default|EventInstanceAttachedStop _soundsystem "NixaDive")
  (Default|EventInstanceStop _soundsystem "NixaDive"))