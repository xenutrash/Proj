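; BP_NixaBurstProjectile is Nixa's burst projectile, which damages actors tagged Hero on overlap.
; Its box overlap ignores the owner and Projectile-tagged actors, and only prints debug text for Boss or other actors.
; A Hero with a valid Ability System Component receives GE_TakeDamage on itself, then the projectile hides and destroys itself after a short delay.
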(event OnComponentBeginOverlap(Box)
  (params (OverlappedComponent :type Primitive%20Component%20Object%20Reference) (OtherActor :type Actor%20Object%20Reference) (OtherComp :type Primitive%20Component%20Object%20Reference) (OtherBodyIndex :type Integer) (bFromSweep :type Boolean) (SweepResult :type Hit%20Result%20Structure%20%28by%20ref%29))
  (bind _returnvalue (Ability|GetAbilitySystemComponent OtherActor))
  (if (not (== OtherActor (Components|GetOwner)))
    (if (Actor|ActorHasTag OtherActor "Boss")
      (Development|PrintString "Hit boss")
      (elif (not (Actor|ActorHasTag OtherActor "Projectile"))
        (if (Actor|ActorHasTag OtherActor "Hero")
          (Utilities|IsValid _returnvalue
            (:Is%20Valid
              (GameplayEffects|ApplyGameplayEffectToSelf :self _returnvalue :GameplayEffectClass "/Game/Programming/Blueprints/GE_TakeDamage.GE_TakeDamage_C")
              (Rendering|SetActorHiddenInGame true)
              (Utilities|FlowControl|Delay 1.0)
              (Actor|DestroyActor)))
          (else
            (Development|PrintString "Hit actor not Hero Boss or Projectile")
            (Development|PrintString (Utilities|GetDisplayName OtherActor) true true "(R=1.000000,G=0.000000,B=0.124420,A=1.000000)" 23452345.0)))))))

(fn ConstructionScript)