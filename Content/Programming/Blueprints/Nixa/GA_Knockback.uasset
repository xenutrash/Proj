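; GA_Knockback is a gameplay ability that knocks its own avatar back when a Boss-tagged pawn is nearby.
; After a short delay, it runs a debug-drawn multi-sphere trace for Pawns at the avatar's location.
; For Boss hits, it applies a constant root motion force along the hit normal.
; The ability ends only when that force finishes, so it has no end path without a Boss hit.
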(event Ability|EventActivateAbility
  (bind _returnvalue (Ability|GetAvatarActorfromActorInfo))
  (bind _returnvalue_2 (Transformation|GetActorLocation _returnvalue))
  (Utilities|FlowControl|Delay 0.2)
  (Development|PrintString "I WILL TRY TO KNOCK BACK MYSELF")
  (bind _outhits (Collision|MultiSphereTraceForObjects _returnvalue_2 _returnvalue_2 2e+02 (Utilities|Array|MakeArray "ObjectTypeQuery3") false 0 "ForDuration"))
  (for _array_element _outhits
    (if (Actor|ActorHasTag (.HitActor (Collision|BreakHitResult _array_element)) "Boss")
      (Development|PrintString (Utilities|GetDisplayName (.HitActor (Collision|BreakHitResult _array_element))) true true "(R=0.000000,G=0.122660,B=1.000000,A=1.000000)" 32.0)
      (Ability|Tasks|ApplyRootMotionConstantForce "None" (.Normal (Collision|BreakHitResult _array_element)) 7e+02 0.4 false 0 "MaintainLastRootMotionVelocity"
        (:OnFinish
          (Ability|EndAbility))))))

(event Ability|EventOnEndAbility
  (params (bWasCancelled :type Boolean)))