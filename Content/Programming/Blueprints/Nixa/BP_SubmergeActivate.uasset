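; BP_SubmergeActivate is a Nixa actor that damages Hero-tagged actors entering its sphere, then destroys itself.
; On sphere overlap it adds the hero to an array and waits briefly before looping over the collected actors.
; It applies GE_TakeDamage through each valid Ability System Component, calling DestroyActor inside the loop after each application.
; Print strings trace the overlap and the target for debugging.
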(event OnComponentBeginOverlap(Sphere)
  (params (OverlappedComponent :type Primitive%20Component%20Object%20Reference) (OtherActor :type Actor%20Object%20Reference) (OtherComp :type Primitive%20Component%20Object%20Reference) (OtherBodyIndex :type Integer) (bFromSweep :type Boolean) (SweepResult :type Hit%20Result%20Structure%20%28by%20ref%29))
  (Development|PrintString (Utilities|GetDisplayName OtherActor))
  (if (Actor|ActorHasTag OtherActor "Hero")
    (Development|PrintString "Hero found")
    (Utilities|Array|Add (Variables|Default|GetOther%20Actor) OtherActor)
    (Utilities|FlowControl|Delay 0.1)
    (for _array_element (Variables|Default|GetOther%20Actor)
      (Utilities|IsValid (Ability|GetAbilitySystemComponent _array_element)
        (:Is%20Valid
          (Development|PrintString (Utilities|GetDisplayName (Ability|GetAbilitySystemComponent _array_element)))
          (GameplayEffects|ApplyGameplayEffectToSelf :self (Ability|GetAbilitySystemComponent _array_element) :GameplayEffectClass "/Game/Programming/Blueprints/GE_TakeDamage.GE_TakeDamage_C")
          (Actor|DestroyActor))))))

(fn ConstructionScript)