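; Gameplay Ability, under Nixa's folder, that casts a whirlpool.
; On activation it turns the avatar toward the visibility-channel hit under the cursor, then spawns BP_Whirlpool at the avatar's location with the avatar as owner.
; It commits only the cooldown, not the cost, and ends immediately, printing a debug string on end.
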(event Ability|EventOnEndAbility
  (params (bWasCancelled :type Boolean))
  (Development|PrintString "whirlpool finished"))

(event Ability|EventActivateAbility
  (bind _returnvalue (Ability|GetAvatarActorfromActorInfo))
  (bind _returnvalue_2 (Transformation|GetActorLocation _returnvalue))
  (Transformation|SetActorRotation (Ability|GetAvatarActorfromActorInfo) (Math|Rotator|FindLookatRotation _returnvalue_2 (.location (.HitResult (Game|Player|GetHitResultUnderCursorbyChannel (Pawn|GetLocalViewingPlayerController (Variables|/Script/Engine.Actor|GetInstigator (Ability|GetAvatarActorfromActorInfo))) "TraceTypeQuery1" true)))))
  (bind _returnvalue_3 (Game|SpawnActorfromClass "/Game/Programming/Blueprints/Nixa/BP_Whirlpool.BP_Whirlpool_C" (Math|Transform|MakeTransform _returnvalue_2 "0, 0, 0" "1.000000,1.000000,1.000000") "Undefined" "MultiplyWithRoot" 0 0))
  (Actor|SetOwner _returnvalue_3 (Ability|GetAvatarActorfromActorInfo))
  (Ability|CommitAbilityCooldown false)
  (Ability|EndAbility))