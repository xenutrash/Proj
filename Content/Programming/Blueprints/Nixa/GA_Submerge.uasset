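; Gameplay ability that submerges Nixa for four seconds, then surfaces the character.
; On authority it toggles visibility, applies a passive effect, plays local or non-local dive audio, commits cooldown and starts a slowed water-burst montage.
; A ground-trace WaitTargetData runs alongside the delay, but its valid data only prints.
; After the delay, only the locally controlled branch replays the montage, spawns BP_SubmergeActivate, restores visibility and ends the ability.
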(event Ability|EventActivateAbility
  (bind _returnvalue (Class|GameplayAbility|MakeTargetLocationInfofromOwnerActor))
  (bind _returnvalue_2 (Ability|GetAvatarActorfromActorInfo))
  (bind _returnvalue_3 (Ability|GetAvatarActorfromActorInfo))
  (bind _returnvalue_4 (Class|GameplayAbility|GetOwningComponentfromActorInfo))
  (bind (_locationtype _literaltransform _sourceactor _sourcecomponent _sourceability _sourcesocketname) (Utilities|Struct|BreakGameplayAbilityTargetingLocationInfo _returnvalue))
  (Ability|HasAuthority
    (:True
      (bind _asbp_nixaa (Utilities|Casting|CastToBP_Nixaa (Ability|GetAvatarActorfromActorInfo)))
      (Default|ToggleVisable _asbp_nixaa)
      (GameplayEffects|ApplyGameplayEffectToSelf :self (Ability|GetAbilitySystemComponent _returnvalue_3) :GameplayEffectClass "/Game/Programming/Blueprints/Nixa/GE_NixaSubmergePassive.GE_NixaSubmergePassive_C")
      (if (Pawn|IsLocallyControlled _asbp_nixaa)
        (bind _returnvalue_5 (Class|FMODBlueprintStatics|PlayEventAttached "/Game/FMOD/Events/InWorld/LocalPlayer/Boss/Nixa/Local_Nixa_Dive.Local_Nixa_Dive" _returnvalue_4 "None" "0, 0, 0" "KeepRelativeOffset"))
        (else
          (bind _returnvalue_6 (Class|FMODBlueprintStatics|PlayEventAttached "/Game/FMOD/Events/InWorld/NonLocalPlayer/Boss/Nixa/NonLocal_Nixa_Dive.NonLocal_Nixa_Dive" _returnvalue_4 "None" "0, 0, 0" "KeepRelativeOffset"))))
      (Ability|CommitAbilityCooldown false)
      (|PlayMontageandWaitProxy "None" "/Game/Programming/Blueprints/Nixa/Animtest/AM_NixaWaterBurst.AM_NixaWaterBurst" 0.2 "None" true 1.0 0.0 false
        (:then
          (|WaitTargetData :ConfirmationType "UserConfirmed" :Class "/Game/Programming/Blueprints/Nixa/BP_SubmergeGroundTrace.BP_SubmergeGroundTrace_C" :StartLocation (Utilities|Struct|MakeGameplayAbilityTargetingLocationInfo _locationtype (Math|Transform|MakeTransform (+ (Transformation|GetActorForwardVector _returnvalue_3) (.location _literaltransform)) (.rotation _literaltransform) (.scale _literaltransform)) _sourceactor _sourcecomponent _sourceability _sourcesocketname) :ReticleClass 0 :bDebug true
            (:then
              (Utilities|FlowControl|Delay 4.0)
              (Development|PrintString "NOW I POPPED UP")
              (Input|DisableInput _returnvalue_2 0)
              (if (Pawn|IsLocallyControlled _asbp_nixaa)
                (Class|FMODAudioComponent|SetParameter _returnvalue_5 "Nixa_Dive" 1.0)
                (|PlayMontageandWaitProxy "None" "/Game/Programming/Blueprints/Nixa/Animtest/AM_NixaWaterBurst.AM_NixaWaterBurst" 1.0 "None" true 1.0 0.0 false
                  (:then
                    (bind _returnvalue_7 (Game|SpawnActorfromClass "/Game/Programming/Blueprints/Nixa/BP_SubmergeActivate.BP_SubmergeActivate_C" (Math|Transform|MakeTransform (Transformation|GetActorLocation _returnvalue_2) "0, 0, 0" "1.000000,1.000000,1.000000") "Undefined" "MultiplyWithRoot" 0 0))
                    (Actor|SetOwner _returnvalue_7 (Ability|GetAvatarActorfromActorInfo))
                    (Default|ToggleVisable _asbp_nixaa)
                    (Input|EnableInput _returnvalue_2 0)
                    (Ability|EndAbility)))
                (else
                  (Class|FMODAudioComponent|SetParameter _returnvalue_6 "Nixa_Dive" 1.0))))
            (:ValidData
              (Development|PrintString "valid data"))))))))

(event Ability|EventOnEndAbility
  (params (bWasCancelled :type Boolean))
  (Development|PrintString "USED SUBMURGE"))