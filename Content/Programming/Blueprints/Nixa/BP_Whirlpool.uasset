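; Whirlpool hazard that pulls player-tagged characters toward its center and destroys itself after a few seconds.
; Sphere overlaps track players and their movement components in parallel arrays, lowering walk speed inside and resetting it to a fixed value on exit.
; Tick adds a constant center-directed impulse to each tracked character's velocity every frame, without delta-time scaling.
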(event OnComponentBeginOverlap(Sphere)
  (params (OverlappedComponent :type Primitive%20Component%20Object%20Reference) (OtherActor :type Actor%20Object%20Reference) (OtherComp :type Primitive%20Component%20Object%20Reference) (OtherBodyIndex :type Integer) (bFromSweep :type Boolean) (SweepResult :type Hit%20Result%20Structure%20%28by%20ref%29))
  (if (Actor|ActorHasTag OtherActor "player")
    (Utilities|Array|Add (Variables|Default|GetOther%20Actor) OtherActor)
    (Variables|Default|SetPlayerInVortex? true)
    (for _array_element (Variables|Default|GetOther%20Actor)
      (Utilities|Array|AddUnique (Variables|Default|GetCharacter%20Movement%20Ref) (Actor|GetComponentbyClass _array_element "/Script/Engine.CharacterMovementComponent"))
      (for _array_element_2 (Variables|Default|GetCharacter%20Movement%20Ref)
        ;[1 1 1] Hur snabb movementspeed innuti whirlpool
        (Variables|/Script/Engine.CharacterMovementComponent|SetMaxWalkSpeed _array_element_2 3e+02)))
    (else
      (Development|PrintString "not a player"))))

(event OnComponentEndOverlap(Sphere)
  (params (OverlappedComponent :type Primitive%20Component%20Object%20Reference) (OtherActor :type Actor%20Object%20Reference) (OtherComp :type Primitive%20Component%20Object%20Reference) (OtherBodyIndex :type Integer))
  (if (Actor|ActorHasTag OtherActor "player")
    (for (_array_element _array_index) (Variables|Default|GetOther%20Actor)
      (if (== _array_element OtherActor)
        (Utilities|Array|RemoveItem (Variables|Default|GetOther%20Actor) _array_element)
        (Variables|/Script/Engine.CharacterMovementComponent|SetMaxWalkSpeed (Utilities|Array|Get(acopy) (Variables|Default|GetCharacter%20Movement%20Ref) _array_index) 6e+02)
        (Utilities|Array|RemoveIndex (Variables|Default|GetCharacter%20Movement%20Ref) _array_index)))))

(event EventTick
  (params (DeltaSeconds :type Float%20%28single-precision%29))
  (if (not (Utilities|Array|IsEmpty (Variables|Default|GetOther%20Actor)))
    (for (_array_element _array_index) (Variables|Default|GetCharacter%20Movement%20Ref)
      (Variables|/Script/Engine.MovementComponent|SetVelocity _array_element (+ (* (Math|Vector|GetForwardVector (Math|Rotator|FindLookatRotation (Transformation|GetActorLocation (Utilities|Array|Get(acopy) (Variables|Default|GetOther%20Actor) _array_index)) (Transformation|GetWorldLocation (Variables|Default|GetCenter)))) "35.000000,35.000000,35.000000") (Variables|/Script/Engine.MovementComponent|GetVelocity _array_element))))))

(event EventBeginPlay
  (Utilities|FlowControl|Delay 5.0)
  (Actor|DestroyActor))

(fn ConstructionScript)