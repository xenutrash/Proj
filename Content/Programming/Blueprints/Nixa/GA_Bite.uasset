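; GA_Bite is a gameplay ability that performs a melee bite toward the mouse cursor.
; On activation it commits its cooldown, turns the avatar to where the cursor ray meets the plane at its height, then disables input.
; It plays a sped-up bite montage with scaled root motion.
; On completion, a forward box trace applies GE_TakeDamage to the hit actor's ability system, then input returns and the ability ends.
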(event Ability|EventActivateAbility
  (bind _returnvalue (Ability|GetAvatarActorfromActorInfo))
  (bind _returnvalue_2 (Ability|GetAvatarActorfromActorInfo))
  (bind _returnvalue_3 (Transformation|GetActorLocation _returnvalue_2))
  (Ability|CommitAbilityCooldown false)
  (bind _aspawn (Utilities|Casting|CastToPawn (Ability|GetAvatarActorfromActorInfo)))
  (bind _asplayer_controller (Utilities|Casting|CastToPlayerController (Pawn|GetController _aspawn)))
  (Transformation|SetActorRotation _returnvalue (Math|Rotator|FindLookatRotation (Transformation|GetActorLocation (Ability|GetAvatarActorfromActorInfo)) (.Intersection (Class|KismetMathLibrary|LinePlaneIntersectionOriginNormal (.WorldLocation (Game|Player|ConvertMouseLocationToWorldSpace _asplayer_controller)) (+ (.WorldLocation (Game|Player|ConvertMouseLocationToWorldSpace _asplayer_controller)) (* (.WorldDirection (Game|Player|ConvertMouseLocationToWorldSpace _asplayer_controller)) 1e+04)) (Transformation|GetWorldLocation (Variables|/Script/Engine.Actor|GetRootComponent (Ability|GetAvatarActorfromActorInfo))) "0.000000,0.000000,1.000000"))) true)
  (Variables|Default|SetRotation (Transformation|GetActorRotation _returnvalue))
  (Input|DisableInput _returnvalue 0)
  (|PlayMontageandWaitProxy "None" "/Game/Animation/Nixa/WhiteboxAnimations/Bite_Montage.Bite_Montage" 3.0 "None" true 5.0 0.0 false
    (:OnCompleted
      (bind _outhit (Collision|BoxTraceByChannel _returnvalue_3 (+ (* (Math|Vector|GetForwardVector (Variables|Default|GetRotation)) "100.000000,100.000000,100.000000") _returnvalue_3) "50.000000,50.000000,50.000000" "0, 0, 0" "TraceTypeQuery2" true 0 "ForDuration"))
      (Utilities|IsValid (Ability|GetAbilitySystemComponent (.HitActor (Collision|BreakHitResult _outhit)))
        (:Is%20Valid
          (GameplayEffects|ApplyGameplayEffectToSelf :self (Ability|GetAbilitySystemComponent (.HitActor (Collision|BreakHitResult _outhit))) :GameplayEffectClass "/Game/Programming/Blueprints/GE_TakeDamage.GE_TakeDamage_C"))
        (:Is%20Not%20Valid
          _))
      (Input|EnableInput _returnvalue 0)
      (Ability|EndAbility))))