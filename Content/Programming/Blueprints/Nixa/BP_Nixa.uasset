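; BP_Nixa is a playable character Blueprint built on the Gameplay Ability System, with several actions still print-only stubs.
; BeginPlay adds the input mapping context, creates the stats widget and applies a base-stats effect.
; Basic and special attacks activate abilities by gameplay tag, while the boss attack applies a damage effect to Nixa herself.
; OnHealthChanged pushes health attribute values to the widget as percentage and text.
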(event EventOnTaunt
  (Development|PrintString "Taunt"))

(event EventOnBasicAttack
  (Development|PrintString "Basic attack")
  (Abilities|TryActivateAbilitiesbyTag (Variables|Default|GetAbilitySystemComponent) (GameplayTags|MakeLiteralGameplayTagContainer "(GameplayTags=((TagName=\"Attack.Basic\")))") true))

(event EventOnSpecialAttack
  (Development|PrintString "Specialattack")
  (Abilities|TryActivateAbilitiesbyTag (Variables|Default|GetAbilitySystemComponent) (GameplayTags|MakeLiteralGameplayTagContainer "(GameplayTags=((TagName=\"Attack.Special\")))") true))

(event EventOnUltimateAttack
  (Development|PrintString "Ultiamte attack"))

(event EventOnBossAttack
  (Development|PrintString "Boss attack")
  (GameplayEffects|ApplyGameplayEffectToSelf :self (Variables|Default|GetAbilitySystemComponent) :GameplayEffectClass "/Game/Programming/Blueprints/GE_TakeDamage.GE_TakeDamage_C")
  (Development|PrintString (Utilities|String|ToString(Float) (.basevalue (Variables|/Script/Proj.RushAttributeSet|GetHealth (Variables|Default|GetAttributes))))))

(event EventOnDash
  (Development|PrintString "Dash"))

(event EventOnHealthChanged
  (params (DeltaValue :type Float%20%28single-precision%29) (EventTags :type Gameplay%20Tag%20Container%20Structure%20%28by%20ref%29))
  (bind _abilitysystemcomponent (Variables|Default|GetAbilitySystemComponent))
  (bind _returnvalue (Class|AbilitySystemComponent|GetGameplayAttributeValue _abilitysystemcomponent "(AttributeName=\"Health\",Attribute=/Script/Proj.RushAttributeSet:Health,AttributeOwner=\"/Script/CoreUObject.Class'/Script/Proj.RushAttributeSet'\")"))
  (bind _returnvalue_2 (Class|AbilitySystemComponent|GetGameplayAttributeValue _abilitysystemcomponent "(AttributeName=\"MaxHealth\",Attribute=/Script/Proj.RushAttributeSet:MaxHealth,AttributeOwner=\"/Script/CoreUObject.Class'/Script/Proj.RushAttributeSet'\")"))
  (bind _returnvalue_3 (/ _returnvalue _returnvalue_2))
  ;[1 1 1] Updaterar HP på widgeten genom ett bpi till playercontroller
  (Development|PrintString (Utilities|String|ToString(Float) _returnvalue_3))
  (Default|UpdateHealth (Variables|Default|GetWidgetRef) _returnvalue_3 (Utilities|Text|FormatText "Health ({0}) / ({1})" _returnvalue _returnvalue_2)))

(event EventOnMove)

(event EventBeginPlay
  (Utilities|FlowControl|Sequence
    (:then_0
      (bind _asplayer_controller (Utilities|Casting|CastToPlayerController (Pawn|GetController)))
      (Input|AddMappingContext (PlayerController|LocalPlayerSubsystems|GetEnhancedInputLocalPlayerSubsystem _asplayer_controller) "/Game/Characters/Input/IMC_Basic.IMC_Basic" 0 "(bIgnoreAllPressedKeysUntilRelease=True,bForceImmediately=False,bNotifyUserSettings=False)")
      (bind _returnvalue (UserInterface|CreateWidget "/Game/Programming/Blueprints/WBP_Stats.WBP_Stats_C"))
      (UserInterface|SetWidget (Variables|Default|GetHealth) _returnvalue)
      (bind _output_get (Variables|Default|SetWidgetRef _returnvalue))
      (UserInterface|Viewport|AddtoViewport _output_get 0)
      (GameplayAttributes|GetAttributeSet (Variables|Default|GetAbilitySystemComponent) "/Script/Proj.RushAttributeSet")
      (GameplayEffects|ApplyGameplayEffectToSelf :self (Variables|Default|GetAbilitySystemComponent) :GameplayEffectClass "/Game/Programming/Blueprints/GE_BasicStats.GE_BasicStats_C"))))

(fn ConstructionScript)