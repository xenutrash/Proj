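; Gameplay ability for Nixa's Water Burst, which fires a fan of burst projectiles in front of the avatar.
; On authority, it commits cooldown, caches rotation, disables avatar input and plays a sped-up montage with scaled root motion.
; The montage's WaterBurst gameplay event re-enables input and spawns owned projectiles at yaw steps set by Offset and Spread.
; EndAbility runs inside the spawn loop; montage interruption only prints, leaving input disabled.
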(event Ability|EventActivateAbility
  (bind _returnvalue (Ability|GetAvatarActorfromActorInfo))
  (bind _returnvalue_2 (Ability|GetAvatarActorfromActorInfo))
  (Ability|HasAuthority
    (:True
      (Development|PrintString (Utilities|String|ToString(Rotator) (Transformation|GetActorRotation (Ability|GetAvatarActorfromActorInfo))))
      (Ability|CommitAbilityCooldown false)
      (Variables|Default|SetRotation (Transformation|GetActorRotation _returnvalue_2))
      (Input|DisableInput _returnvalue_2 0)
      (|PlayMontageandWaitProxy "None" "/Game/Programming/Blueprints/Nixa/Animtest/AM_NixaWaterBurst.AM_NixaWaterBurst" 2.0 "None" true 5.0 0.0 false
        (:then
          (Ability|Tasks|WaitGameplayEvent "(TagName=\"Event.Montage.WaterBurst\")" 0
            (:EventReceived
              (Input|EnableInput _returnvalue_2 0)
              (for _index (range 1 (Variables|Default|GetProjectileCount))
                (bind _returnvalue_3 (Game|SpawnActorfromClass "/Game/Programming/Blueprints/Nixa/BP_NixaBurstProjectile.BP_NixaBurstProjectile_C" (Math|Transform|MakeTransform (+ (Transformation|GetActorLocation _returnvalue) (* (Transformation|GetActorForwardVector _returnvalue) "100.000000,100.000000,100.000000")) (Math|Rotator|CombineRotators (Math|Rotator|MakeRotator (.Roll (Math|Rotator|BreakRotator (Variables|Default|GetRotation))) 0.0 (+ (.Yaw (Math|Rotator|BreakRotator (Variables|Default|GetRotation))) (Variables|Default|Getoffset))) (* (Math|Rotator|MakeRotator 0.0 0.0 (Variables|Default|GetSpread)) _index)) "1.000000,1.000000,1.000000") "Undefined" "MultiplyWithRoot" 0 0))
                (Actor|SetOwner _returnvalue_3 (Ability|GetAvatarActorfromActorInfo))
                (Ability|EndAbility)))))
        (:OnInterrupted
          (Development|PrintString "DEN BLEV INTERUPPTED"))))))

(event Ability|EventOnEndAbility
  (params (bWasCancelled :type Boolean)))