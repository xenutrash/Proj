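; Player controller for rush characters that owns the local player's UI and session exit.
; BeginPlay adds input mapping and builds the stats, cooldown HUD and pause menu widgets, then links to the controlled BP_RushCharacter.
; Tick rotates that character, retrying the link when invalid.
; Events relay health, cooldowns, ultimate charge and HUD icons to widgets, and handle game over, input disabling, time dilation and session teardown to main menu.
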(event Custom|Health%20changed
  (params (HealthText :type Text) (HealthPercent :type Float%20%28double-precision%29))
  (Default|UpdateHealth (Variables|Default|GetWidget) HealthPercent HealthText))

(event Custom|EndClientSession
  (|DestroySession self
    (:then
      (Game|OpenLevel(byObjectReference) "/Game/Programming/Lobby/Maps/MainMenuMap.MainMenuMap"))))

(event Custom|PlayLoadingANimastionReverse
  (Default|PlayEverythingReverse (Variables|Default|GetLoadingScreen)))

(event Custom|EndGame
  (params (NewParam :type String))
  (bind _returnvalue (Class|ProjPlayerController|CreateGameOverWidget))
  (if _returnvalue
    (bind _aswpp_end_game_menu (Utilities|Casting|CastToWPP_EndGameMenu (Variables|Default|GetGameOverMenu)))
    (Default|SetWinnerText _aswpp_end_game_menu NewParam)))

(event Custom|SlowDownTime
  (params (TimeDilation :type Float%20%28single-precision%29))
  (Utilities|Time|SetGlobalTimeDilation TimeDilation))

(event Custom|Disable%20All%20Input
  (if (Pawn|IsLocalController)
    (Input|DisableInput (Pawn|GetControlledPawn) self)))

(event Custom|StartCooldownE
  (params (TimerE :type Integer))
  ;[1 1 1] Starts cooldown of interface
  (Default|StartCooldownE (Variables|Default|GetCooldownUI) TimerE))

(event Custom|StartCooldownQ
  (params (TimerQ :type Integer))
  ;[1 1 1] Starts cooldown of interface
  (Default|StartCooldownQ (Variables|Default|GetCooldownUI) TimerQ))

(event Custom|SetHudIConsEvent
  (params (CharacetrName :type Name) (SkinName :type Name))
  (bind _output_get (Variables|Default|SetHudName CharacetrName))
  (CallFunction|SetHUDIcons _output_get "None"))

(event Custom|StartCooldownSpace
  (params (TimerE :type Integer))
  ;[1 1 1] Starts cooldown of interface
  (Default|StartCooldownSpace (Variables|Default|GetCooldownUI) TimerE))

(event Custom|StartCoolDownM1
  ;[1 1 1] Starts cooldown of interface
  (Default|StartCoolDownM1 (Variables|Default|GetCooldownUI)))

(event Custom|AddUltimateCharge
  (params (ProgressUltimate :type Float%20%28double-precision%29))
  (Default|AddtoUltimate (Variables|Default|GetCooldownUI) ProgressUltimate))

(event Custom|ResetUltimate
  (Default|ResetUltimate (Variables|Default|GetCooldownUI)))

(event EventBeginPlay
  (bind _self self)
  (Utilities|FlowControl|Delay 0.2)
  (Input|AddMappingContext (PlayerController|LocalPlayerSubsystems|GetEnhancedInputLocalPlayerSubsystem (Game|GetPlayerController 0)) "/Game/Characters/Input/IMC_Basic.IMC_Basic" 0 "(bIgnoreAllPressedKeysUntilRelease=True,bForceImmediately=False,bNotifyUserSettings=False)")
  (if (Pawn|IsLocalController)
    (bind _returnvalue (UserInterface|CreateWidget "/Game/Programming/Blueprints/Widgets/WBP_Stats.WBP_Stats_C" self))
    (bind _output_get (Variables|Default|SetWidget _returnvalue))
    (bind _returnvalue_2 (UserInterface|CreateWidget "/Game/Programming/Blueprints/WBP_Cooldowns.WBP_Cooldowns_C"))
    (Default|AddHealthBarWidget _returnvalue_2 _output_get)
    (bind _output_get_2 (Variables|Default|SetCooldownUI _returnvalue_2))
    (UserInterface|Viewport|AddtoViewport _returnvalue_2 0)
    (CallFunction|SetHUDIcons (Variables|Default|GetHudName) "None")
    (bind _asbp_rush_character (Utilities|Casting|CastToBP_RushCharacter (Pawn|GetControlledPawn)))
    (bind _output_get_3 (Variables|Default|SetControlled%20Pawn _asbp_rush_character))
    (Variables|/Game/Programming/Blueprints/BP_RushCharacter.BP_RushCharacter_C|SetPlayerController _output_get_3 _self)
    (bind _returnvalue_3 (UserInterface|CreateWidget "/Game/Programming/Blueprints/Widgets/WBP_PauseMenu.WBP_PauseMenu_C" _self))
    (bind _output_get_4 (Variables|Default|SetPauseMenu _returnvalue_3))
    (Widget|SetVisibility _returnvalue_3 "Hidden")
    (UserInterface|Viewport|AddtoViewport _returnvalue_3 0)))

(event EventTick
  (params (DeltaSeconds :type Float%20%28single-precision%29))
  (Utilities|IsValid (Variables|Default|GetControlled%20Pawn)
    (:Is%20Valid
      (Default|RotateCharacter (Variables|Default|GetControlled%20Pawn)))
    (:Is%20Not%20Valid
      (if (Pawn|IsLocalController)
        (bind _asbp_rush_character (Utilities|Casting|CastToBP_RushCharacter (Pawn|GetControlledPawn)))
        (bind _output_get (Variables|Default|SetControlled%20Pawn _asbp_rush_character))
        (Variables|/Game/Programming/Blueprints/BP_RushCharacter.BP_RushCharacter_C|SetPlayerController _output_get self)))))

(event EventPossess
  (params (PossessedPawn :type Pawn%20Object%20Reference))
  (Utilities|FlowControl|Delay 1.0)
  (bind _asbp_rush_character (Utilities|Casting|CastToBP_RushCharacter PossessedPawn)
    (:then
      (Default|OnHealthChangedAllClients _asbp_rush_character))
    (:CastFailed
      (Development|PrintString "Not a rush character?"))))

(event Input|KeyboardEvents|T
  (params (Key :type Key%20Structure :default "None"))
  (:Pressed
    (CallFunction|PlayLoadingANimastionReverse)))

(event Input|KeyboardEvents|Tab
  (params (Key :type Key%20Structure :default "None"))
  (:Pressed
    (CallFunction|ShowPauseMenu)))

(fn ConstructionScript)

(fn SetHUDIcons
  (params (CharacterName :type Name) (SkinName :type Name))
  (if (Utilities|IsValid (Variables|Default|GetCooldownUI))
    (Default|SetHUDIcons (Variables|Default|GetCooldownUI) CharacterName SkinName)
    (else
      (Development|PrintString "No CoolDown GUI"))))

(fn ShowPauseMenu
  (if (Utilities|IsValid (Variables|Default|GetPauseMenu))
    _
    (else
      (bind _returnvalue (UserInterface|CreateWidget "/Game/Programming/Blueprints/Widgets/WBP_PauseMenu.WBP_PauseMenu_C" self))
      (bind _output_get (Variables|Default|SetPauseMenu _returnvalue))
      (Widget|SetVisibility _output_get "Hidden")
      (UserInterface|Viewport|AddtoViewport _output_get 0)))
  (Default|ShowPauseMenu (Variables|Default|GetPauseMenu)))