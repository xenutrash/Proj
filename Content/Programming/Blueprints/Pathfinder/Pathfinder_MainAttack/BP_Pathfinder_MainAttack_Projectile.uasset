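; Projectile actor for the Pathfinder main attack, handling hit detection on overlap while ignoring its owner.
; Hitting a Boss-tagged Rush character deals damage, charges the owner's ultimate and updates score; static mesh actors only trigger the impact.
; On impact it hides, disables further hits, plays Alchemist-named Niagara and audio effects, then destroys itself after a short delay.
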(event Custom|SpawnImpactEffect
  (Niagara|SpawnSystematLocation "/Game/Niagara/NS_Alchemist_BasicAttack_Impact.NS_Alchemist_BasicAttack_Impact" (Transformation|GetActorLocation)))

(event Collision|EventActorBeginOverlap
  (params (OtherActor :type Actor%20Object%20Reference))
  (bind _returnvalue (Components|GetOwner))
  (if (Variables|Default|GetCanHit)
    (if (not (== OtherActor (Components|GetOwner)))
      (if (Actor|ActorHasTag OtherActor "Boss")
        (bind _asbp_rush_character (Utilities|Casting|CastToBP_RushCharacter OtherActor))
        (Default|TakeDamage _asbp_rush_character (Variables|Default|GetDamage))
        (bind _asbp_rush_character_2 (Utilities|Casting|CastToBP_RushCharacter _returnvalue))
        (Default|ChargeUltimate _asbp_rush_character_2 (Variables|Default|GetUltCharge))
        (Default|UpdateScore _asbp_rush_character _returnvalue (Variables|Default|GetDamage))
        (else
          (Utilities|Casting|CastToStaticMeshActor OtherActor)))
      (Rendering|SetActorHiddenInGame true)
      (Variables|Default|SetCanHit false)
      (CallFunction|SpawnImpactEffect)
      (Class|FMODBlueprintStatics|PlayEventatLocation "/Game/FMOD/Events/InWorld/LocalPlayer/Hero/Alchemist/Local_Alchemist_MainAttackHit.Local_Alchemist_MainAttackHit" (Transformation|GetActorTransform))
      (Utilities|FlowControl|Delay 2.0)
      (Development|PrintString "Impact")
      (Actor|DestroyActor))))

(fn ConstructionScript)