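; Gameplay ability for the Pathfinder's main attack, which fires a projectile in time with a randomly chosen attack montage.
; Activation commits the cooldown and plays the montage; the server waits for an Attack.Basic gameplay event, then spawns the projectile at the head socket, facing the avatar's rotation.
; The ability ends after firing or when the montage finishes.
; An unused-in-graph helper removes attack-block tags with debug prints.
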(event Ability|EventActivateAbility
  (Ability|CommitAbilityCooldown false true)
  (|PlayMontageandWaitProxy "None" (.OutItem (Utilities|Array|Random (Variables|Default|GetAnimationArray))) 1.0 "None" false 1.0 0.0 false
    (:then
      (if (Networking|IsServer)
        (Ability|Tasks|WaitGameplayEvent "(TagName=\"Attack.Basic\")" 0
          (:EventReceived
            (CallFunction|SpawnProjectile)
            (Ability|EndAbility)))))
    (:OnCompleted
      (Ability|EndAbility :!label _label))
    (:OnBlendOut
      (goto _label))
    (:OnInterrupted
      (goto _label))
    (:OnCancelled
      (goto _label))))

(fn RemoveAttackBlock
  (bind _returnvalue (Ability|GameplayEffect|RemoveLooseGameplayTags (Ability|GetAvatarActorfromActorInfo) (GameplayTags|MakeGameplayTagContainerfromTag "(TagName=\"Attack.Block.All\")") true))
  (if _returnvalue
    (Development|PrintString "Removed?")
    (else
      (Development|PrintString "No remove?"))))

(fn SpawnProjectile
  (bind _returnvalue (Ability|GetAvatarActorfromActorInfo))
  (Game|SpawnActorfromClass "/Game/Programming/Blueprints/Pathfinder/Pathfinder_MainAttack/BP_Pathfinder_MainAttack_Projectile.BP_Pathfinder_MainAttack_Projectile_C" (Math|Transform|MakeTransform (Transformation|GetSocketLocation (Actor|GetComponentbyClass _returnvalue "/Script/Engine.SkeletalMeshComponent") "head") (Transformation|GetActorRotation _returnvalue) "1.000000,1.000000,1.000000") "Undefined" "MultiplyWithRoot" _returnvalue 0))