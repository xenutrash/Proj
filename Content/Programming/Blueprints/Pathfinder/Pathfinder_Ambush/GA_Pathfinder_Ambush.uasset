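; Pathfinder's Ambush gameplay ability, which marks the character's location and lets them teleport back to it within a time window.
; Activation commits only the cooldown and plays an ultimate attack montage.
; On the server, the Attack.Ultimate event saves the location and starts a wait for the confirm input event.
; Confirming teleports the Pathfinder to the saved spot and ends the ability; otherwise a delay ends it.
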(event Ability|EventActivateAbility
  (bind _asbp_pathfinder (Utilities|Casting|CastToBP_Pathfinder (Ability|GetAvatarActorfromActorInfo)))
  (Variables|Default|SetPathfinderCharacter _asbp_pathfinder)
  (Ability|CommitAbilityCooldown false true)
  (|PlayMontageandWaitProxy "None" "/Game/Animation/Alchemist/Montages/Anim_Alchemist_UltimateAttack_Montage.Anim_Alchemist_UltimateAttack_Montage" 1.0 "None" false 1.0 0.0 false
    (:then
      (if (Networking|IsServer)
        (Ability|Tasks|WaitGameplayEvent "(TagName=\"Attack.Ultimate\")" 0
          (:EventReceived
            (Variables|Default|SetSavedPosition (Transformation|GetActorLocation (Variables|Default|GetPathfinderCharacter)))
            (Ability|Tasks|WaitGameplayEvent "(TagName=\"Event.Input.Confirm\")" (Variables|Default|GetPathfinderCharacter) true
              (:then
                (Utilities|FlowControl|Delay 1e+01)
                (Ability|EndAbility))
              (:EventReceived
                (Transformation|SetActorLocation (Variables|Default|GetPathfinderCharacter) (Variables|Default|GetSavedPosition) false true)
                (Ability|EndAbility)))))))))