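; Pathfinder character Blueprint that maps basic, special, ultimate and dash input events to Gameplay Ability System activations.
; It mixes Pathfinder abilities (main attack, Ambush dash) with Slayer ones (Heal, Fairy Wings).
; Successful dash and special activations start cooldowns on player controller 0, while the ultimate requires a full attribute charge, then resets.
; "Multi" events handle montage stopping and actor visibility, and hiding the healthbar also hides the hitbox indicator.
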(event Custom|SetCharacterHiddenMulti
  (params (bNewHidden :type Boolean))
  ;[1 1 1] Toggle Visibility
  (Rendering|SetActorHiddenInGame bNewHidden)
  (CallFunction|ServeronHealthChanged))

(event Custom|SetCharacterHidden
  (params (bNewHidden :type Boolean))
  ;[1 1 1] Toggle Visibility
  (CallFunction|SetCharacterHiddenMulti bNewHidden))

(event Custom|StopAnimation
  (params (AnimMontage :type Anim%20Montage%20Object%20Reference))
  (CallFunction|StopAnimationMulti AnimMontage))

(event Custom|StopAnimationMulti
  (params (AnimMontage :type Anim%20Montage%20Object%20Reference))
  (Animation|StopAnimMontage AnimMontage))

(event EventHideHealthbar
  (|CallParentFunction)
  (Development|SetHiddeninGame (Variables|Default|GetHitboxIndicator) true false))

(event EventOnBasicAttack
  ;[1 1 1] Abilities
  (CallFunction|AbilityBasicAttack))

(event EventOnSpecialAttack
  ;[1 1 1] Abilities
  (CallFunction|AbilitySpecialAttack))

(event EventOnUltimateAttack
  ;[1 1 1] Abilities
  (CallFunction|AbilityUltimate)
  (Utilities|FlowControl|Delay 0.5)
  (Rendering|Material|SetOverlayMaterial (Variables|Character|GetMesh) 0 :!class /Script/Engine.MeshComponent))

(event EventOnDash
  ;[1 1 1] Abilities
  (CallFunction|AbilityDash))

(fn ConstructionScript
  (|CallParentFunction))

(fn AbilityDash
  (Ability|SendGameplayEventtoActor self "(TagName=\"Event.Input.Confirm\")")
  (bind _returnvalue (Abilities|TryActivateAbilitybyClass (Variables|Default|GetAbilitySystemComponent) "/Game/Programming/Blueprints/Pathfinder/Pathfinder_Ambush/GA_Pathfinder_Ambush.GA_Pathfinder_Ambush_C" true))
  (if _returnvalue
    (bind _asbp_proj_player_controller (Utilities|Casting|CastToBP_ProjPlayerController (Game|GetPlayerController 0)))
    (Default|StartCooldownSpace _asbp_proj_player_controller)))

(fn AbilityUltimate
  (if (<= 1e+02 (.ReturnValue (Class|AbilitySystemBlueprintLibrary|GetFloatAttributeBasefromAbilitySystemComponent (Variables|Default|GetAbilitySystemComponent) "(AttributeName=\"UltimateCharge\",Attribute=/Script/Proj.RushAttributeSet:UltimateCharge,AttributeOwner=\"/Script/CoreUObject.Class'/Script/Proj.RushAttributeSet'\")")))
    (Abilities|TryActivateAbilitybyClass (Variables|Default|GetAbilitySystemComponent) "/Game/Programming/Blueprints/Slayer/FairyWings/GA_Slayer_FairyWings.GA_Slayer_FairyWings_C" true)
    (CallFunction|ResetUltimate)))

(fn AbilitySpecialAttack
  (bind _returnvalue (Abilities|TryActivateAbilitybyClass (Variables|Default|GetAbilitySystemComponent) "/Game/Programming/Blueprints/Slayer/Heal/GA_Slayer_Heal.GA_Slayer_Heal_C" true))
  (if _returnvalue
    (bind _asbp_proj_player_controller (Utilities|Casting|CastToBP_ProjPlayerController (Game|GetPlayerController 0)))
    (Default|StartCooldownE _asbp_proj_player_controller)))

(fn AbilityBasicAttack
  (bind _returnvalue (Abilities|TryActivateAbilitybyClass (Variables|Default|GetAbilitySystemComponent) "/Game/Programming/Blueprints/Pathfinder/Pathfinder_MainAttack/GA_Pathfinder_MainAttack.GA_Pathfinder_MainAttack_C" true))
  (return _returnvalue))