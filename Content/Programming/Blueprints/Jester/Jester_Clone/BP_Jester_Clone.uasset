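; BP_Jester_Clone is the Jester's clone character, destroyed on spawn unless its owner is a BP_Jester.
; CloneMovement applies a supplied vector as a swept world offset and as movement velocity.
; Damage refreshes health on all clients; at zero it leaves the owner's clone list, plays a death montage and self-destructs.
; Ability functions activate GAS abilities, mostly Pathfinder and Slayer ones, with dash and special starting player-controller cooldowns.
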(event Custom|Testing
  ;[1 1 1] TESTING
  (CallFunction|TakeDamage -5.0))

(event Custom|CloneMovement
  (params (WorldVector :type Vector) (DeltaSeconds :type Float%20%28double-precision%29))
  (Transformation|AddActorWorldOffset (* WorldVector DeltaSeconds) true)
  (Variables|/Script/Engine.MovementComponent|SetVelocity (Variables|Character|GetCharacterMovement) WorldVector))

(event EventDeathEvent
  ;[1 1 1] Death event
  (Default|RemoveClone (Variables|Default|GetOwnerJester) self)
  (CallFunction|PlayAnimation "/Game/Animation/Alchemist/Montages/Anim_Alchemist_Death_Montage.Anim_Alchemist_Death_Montage")
  (Utilities|FlowControl|Delay 1.0)
  (Actor|DestroyActor))

(event EventTakeDamage
  (params (DamageAmount :type Float%20%28single-precision%29))
  ;[1 1 1] Take damage
  (|CallParentFunction DamageAmount)
  (CallFunction|OnHealthChangedAllClients)
  (if (<= (.ReturnValue (Class|AbilitySystemComponent|GetGameplayAttributeValue (Variables|Default|GetAbilitySystemComponent) "(AttributeName=\"Health\",Attribute=/Script/Proj.RushAttributeSet:Health,AttributeOwner=\"/Script/CoreUObject.Class'/Script/Proj.RushAttributeSet'\")")) 0.0)
    (CallFunction|DeathEvent)))

(event EventBeginPlay
  ;[1 1 1] Begin play
  (bind _asbp_jester (Utilities|Casting|CastToBP_Jester (Components|GetOwner))
    (:then
      (Variables|Default|SetOwnerJester _asbp_jester))
    (:CastFailed
      (Actor|DestroyActor))))

(fn ConstructionScript
  (|CallParentFunction))

(fn AbilityDash
  (Ability|SendGameplayEventtoActor self "(TagName=\"Event.Input.Confirm\")")
  (bind _returnvalue (Abilities|TryActivateAbilitybyClass (Variables|Default|GetAbilitySystemComponent) "/Game/Programming/Blueprints/Pathfinder/Pathfinder_Ambush/GA_Pathfinder_Ambush.GA_Pathfinder_Ambush_C" true))
  (if _returnvalue
    (bind _asbp_proj_player_controller (Utilities|Casting|CastToBP_ProjPlayerController (Game|GetPlayerController 0)))
    (Default|StartCooldownSpace _asbp_proj_player_controller)))

(fn AbilityUltimate
  (if (<= 1e+02 (.ReturnValue (Class|AbilitySystemBlueprintLibrary|GetFloatAttributeBasefromAbilitySystemComponent (Variables|Default|GetAbilitySystemComponent) "(AttributeName=\"UltimateCharge\",Attribute=/Script/Proj.RushAttributeSet:UltimateCharge,AttributeOwner=\"/Script/CoreUObject.Class'/Script/Proj.RushAttributeSet'\")")))
    _
    (else
      _))
  (Abilities|TryActivateAbilitybyClass (Variables|Default|GetAbilitySystemComponent) "/Game/Programming/Blueprints/Jester/Jester_Clone/GA_Jester_Clone.GA_Jester_Clone_C" true)
  (CallFunction|ResetUltimate))

(fn AbilitySpecialAttack
  (bind _returnvalue (Abilities|TryActivateAbilitybyClass (Variables|Default|GetAbilitySystemComponent) "/Game/Programming/Blueprints/Slayer/Heal/GA_Slayer_Heal.GA_Slayer_Heal_C" true))
  (if _returnvalue
    (bind _asbp_proj_player_controller (Utilities|Casting|CastToBP_ProjPlayerController (Game|GetPlayerController 0)))
    (Default|StartCooldownE _asbp_proj_player_controller)))

(fn AbilityBasicAttack
  (bind _returnvalue (Abilities|TryActivateAbilitybyClass (Variables|Default|GetAbilitySystemComponent) "/Game/Programming/Blueprints/Pathfinder/Pathfinder_MainAttack/GA_Pathfinder_MainAttack.GA_Pathfinder_MainAttack_C" true))
  (return _returnvalue))