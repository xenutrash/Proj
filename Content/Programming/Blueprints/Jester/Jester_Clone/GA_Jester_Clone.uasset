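; Gameplay ability that spawns a clone of the Jester character.
; On activation it commits the cooldown and captures the Jester's transform, then waits one second before spawning a BP_Jester_Clone at that saved position.
; The clone is owned and instigated by the Jester and registered in its Clones list before the ability ends.
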(event Ability|EventActivateAbility
  (bind _asbp_jester (Utilities|Casting|CastToBP_Jester (Ability|GetAvatarActorfromActorInfo)))
  (Variables|Default|SetJesterCharacter _asbp_jester)
  (Ability|CommitAbilityCooldown true true)
  (Variables|Default|SetPosition (Transformation|GetActorTransform (Variables|Default|GetJesterCharacter)))
  (Utilities|FlowControl|Delay 1.0)
  (bind _returnvalue (Game|SpawnActorfromClass "/Game/Programming/Blueprints/Jester/Jester_Clone/BP_Jester_Clone.BP_Jester_Clone_C" (Variables|Default|GetPosition) "AdjustIfPossibleButAlwaysSpawn" "MultiplyWithRoot" (Variables|Default|GetJesterCharacter) (Variables|Default|GetJesterCharacter)))
  (Default|AddtoClones (Variables|Default|GetJesterCharacter) _returnvalue)
  (Ability|EndAbility))