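; Playable Jester character that commands a list of clones mirroring its rotation, movement and taunts.
; Rotation, tick and taunt events extend the parent and forward to each clone; basic attack only calls the clones' Testing event.
; Dash, special and ultimate activate GAS abilities: borrowed Pathfinder Ambush, Slayer Heal, and Jester Clone.
; Dash and special start controller cooldowns on success, while the ultimate resets its charge regardless of activation.
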(event Custom|AddToClones
  (params (NewClone :type BP%20Jester%20Clone%20Object%20Reference%20%28by%20ref%29))
  (Utilities|Array|AddUnique (Variables|Default|GetClones) NewClone))

(event Custom|RemoveClone
  (params (Clone :type BP%20Jester%20Clone%20Object%20Reference%20%28by%20ref%29))
  (Utilities|Array|RemoveItem (Variables|Default|GetClones) Clone))

(event Custom|SetCharacterHiddenMulti
  (params (bNewHidden :type Boolean))
  ;[1 1 1] Toggle Visibility
  (Rendering|SetActorHiddenInGame bNewHidden)
  (CallFunction|ServeronHealthChanged))

(event Custom|SetCharacterHidden
  (params (bNewHidden :type Boolean))
  ;[1 1 1] Toggle Visibility
  (CallFunction|SetCharacterHiddenMulti bNewHidden))

(event Custom|StopAnimation
  (params (AnimMontage :type Anim%20Montage%20Object%20Reference))
  (CallFunction|StopAnimationMulti AnimMontage))

(event Custom|StopAnimationMulti
  (params (AnimMontage :type Anim%20Montage%20Object%20Reference))
  (Animation|StopAnimMontage AnimMontage))

(event EventHideHealthbar
  (|CallParentFunction)
  (Development|SetHiddeninGame (Variables|Default|GetHitboxIndicator) true false))

(event EventOnBasicAttack
  ;[1 1 1] Abilities
  (for _array_element (Variables|Default|GetClones)
    (Default|Testing _array_element)))

(event EventOnSpecialAttack
  ;[1 1 1] Abilities
  (CallFunction|AbilitySpecialAttack))

(event EventOnUltimateAttack
  ;[1 1 1] Abilities
  (CallFunction|AbilityUltimate)
  (Utilities|FlowControl|Delay 0.5)
  (Rendering|Material|SetOverlayMaterial (Variables|Character|GetMesh) 0 :!class /Script/Engine.MeshComponent))

(event EventMulticastRotation
  (params (NewRotation :type Rotator :default "0, 0, 0"))
  (|CallParentFunction NewRotation)
  (for _array_element (Variables|Default|GetClones)
    (Default|CallServerRotation _array_element NewRotation)))

(event EventOnDash
  ;[1 1 1] Abilities
  (CallFunction|AbilityDash))

(event EventOnTaunt
  (|CallParentFunction)
  (for _array_element (Variables|Default|GetClones)
    (Default|EmoteEvent _array_element)))

(event EventTick
  (params (DeltaSeconds :type Float%20%28single-precision%29))
  (|CallParentFunction DeltaSeconds)
  (for _array_element (Variables|Default|GetClones)
    (Default|CloneMovement _array_element (Pawn|Components|CharacterMovement|GetLastUpdateVelocity (Variables|Character|GetCharacterMovement)) DeltaSeconds)))

(fn ConstructionScript
  (|CallParentFunction))

(fn AbilityDash
  (Ability|SendGameplayEventtoActor self "(TagName=\"Event.Input.Confirm\")")
  (bind _returnvalue (Abilities|TryActivateAbilitybyClass (Variables|Default|GetAbilitySystemComponent) "/Game/Programming/Blueprints/Pathfinder/Pathfinder_Ambush/GA_Pathfinder_Ambush.GA_Pathfinder_Ambush_C" true))
  (if _returnvalue
    (bind _asbp_proj_player_controller (Utilities|Casting|CastToBP_ProjPlayerController (Game|GetPlayerController 0)))
    (Default|StartCooldownSpace _asbp_proj_player_controller)))

(fn AbilityUltimate
  (if (<= 1e+02 (.ReturnValue (Class|AbilitySystemBlueprintLibrary|GetFloatAttributeBasefromAbilitySystemComponent (Variables|Default|GetAbilitySystemComponent) "(AttributeName=\"UltimateCharge\",Attribute=/Script/Proj.RushAttributeSet:UltimateCharge,AttributeOwner=\"/Script/CoreUObject.Class'/Script/Proj.RushAttributeSet'\")")))
    _
    (else
      _))
  (Abilities|TryActivateAbilitybyClass (Variables|Default|GetAbilitySystemComponent) "/Game/Programming/Blueprints/Jester/Jester_Clone/GA_Jester_Clone.GA_Jester_Clone_C" true)
  (CallFunction|ResetUltimate))

(fn AbilitySpecialAttack
  (bind _returnvalue (Abilities|TryActivateAbilitybyClass (Variables|Default|GetAbilitySystemComponent) "/Game/Programming/Blueprints/Slayer/Heal/GA_Slayer_Heal.GA_Slayer_Heal_C" true))
  (if _returnvalue
    (bind _asbp_proj_player_controller (Utilities|Casting|CastToBP_ProjPlayerController (Game|GetPlayerController 0)))
    (Default|StartCooldownE _asbp_proj_player_controller)))

(fn AbilityBasicAttack
  (bind _returnvalue (Abilities|TryActivateAbilitybyClass (Variables|Default|GetAbilitySystemComponent) "/Game/Programming/Blueprints/Pathfinder/Pathfinder_MainAttack/GA_Pathfinder_MainAttack.GA_Pathfinder_MainAttack_C" true))
  (return _returnvalue))