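; Gameplay ability for raid boss Nixa's Flowing Tides attack: a dive, a pull on nearby pawns and a resurfacing strike.
; After the dive montage and move, a sphere trace gathers pawns, then a looping timer line-traces toward each.
; Traces hitting "Rock"-tagged actors only print; otherwise the target receives GA_TidePull and leaves the list.
; After a delay, remaining listed actors receive knockback events as Nixa resurfaces, attacks and ends the ability.
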(event Custom|Linetrace
  (bind _hit_actor (Variables|Default|GetHit%20Actor))
  (bind _as_bp_raidboss_nixa (Variables|Default|GetAs%20BP%20Raidboss%20Nixa))
  (for _array_element (Variables|Default|GetHit%20Actor)
    (bind _outhit (Collision|LineTraceForObjects "0, 0, 0" (Transformation|GetActorLocation _array_element) (Utilities|Array|MakeArray "ObjectTypeQuery3") false 0 "ForDuration"))
    (if true
      (Development|PrintString (Utilities|GetDisplayName (.HitActor (Collision|BreakHitResult _outhit))))
      (if (Actor|ActorHasTag (.HitActor (Collision|BreakHitResult _outhit)) "Rock")
        (Development|PrintString "You hit rock")
        (else
          (Utilities|IsValid (Ability|GetAbilitySystemComponent _array_element)
            (:Is%20Valid
              (Class|AbilitySystemComponent|GiveAbilityandActivateOnce (Ability|GetAbilitySystemComponent _array_element) "/Game/Programming/Blueprints/NixaRaidBoss/GA_TidePull.GA_TidePull_C" 0 -1)
              (Utilities|Array|RemoveItem _hit_actor _array_element)
              (Utilities|FlowControl|Delay 3.0)
              (for _array_element_2 _hit_actor
                (Ability|SendGameplayEventtoActor _array_element_2 "(TagName=\"Event.FlowingTides.Knockback\")")
                (Default|ActivateSubmergeVFX _as_bp_raidboss_nixa false)
                (Default|ToggleVisable _as_bp_raidboss_nixa)
                (Input|EnableInput (Ability|GetAvatarActorfromActorInfo) 0)
                (AI|Navigation|MovetoLocation "None" (Math|Vector|MakeVector 0.0 0.0 5e+02) 0.3
                  (:then
                    (|PlayMontageandWaitProxy "None" "/Game/Animation/Nixa/Montages/Attack_3_Montage.Attack_3_Montage" 2.0 "None" true 1.0 0.0 false
                      (:OnCompleted
                        (Ability|EndAbility)))))))))))))

(event Ability|EventActivateAbility
  (bind _returnvalue (Ability|GetAvatarActorfromActorInfo))
  (bind _returnvalue_2 (Transformation|GetActorLocation _returnvalue))
  (bind _asbp_raidboss_nixa (Utilities|Casting|CastToBP_RaidbossNixa (Ability|GetAvatarActorfromActorInfo)))
  (Variables|Default|SetAs%20BP%20Raidboss%20Nixa _asbp_raidboss_nixa)
  (|PlayMontageandWaitProxy "None" "/Game/Animation/Nixa/Montages/Dive_Montage.Dive_Montage" 0.3 "None" true 1.0 0.0 false
    (:OnCompleted
      (Default|ToggleVisable (Variables|Default|GetAs%20BP%20Raidboss%20Nixa))
      (Default|ActivateSubmergeVFX (Variables|Default|GetAs%20BP%20Raidboss%20Nixa) false)
      (AI|Navigation|MovetoLocation "None" (Math|Vector|MakeVector 0.0 0.0 (.Z (Math|Vector|BreakVector _returnvalue_2))) 1.5
        (:OnTargetLocationReached
          (Input|DisableInput _returnvalue 0)
          (Development|PrintString "Start ability")
          (bind _outhits (Collision|MultiSphereTraceForObjects _returnvalue_2 _returnvalue_2 1.4e+03 (Utilities|Array|MakeArray "ObjectTypeQuery3") false 0 "ForDuration"))
          (bind _array_element (Utilities|Array|ForEachLoopwithBreak _outhits)
            (:LoopBody
              (Utilities|Array|AddUnique (Variables|Default|GetHit%20Actor) (.HitActor (Collision|BreakHitResult _array_element))))
            (:Completed
              (Utilities|Time|SetTimerbyEvent (delegate Custom|Linetrace) 0.3 true))))))))

(event Ability|EventOnEndAbility
  (params (bWasCancelled :type Boolean)))