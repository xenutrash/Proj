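; TidePull Gameplay Ability in the Nixa raid boss folder that drags its avatar toward the world's XY origin, then launches it in a jump.
; A one-second MoveToLocation task keeps the avatar's height, with a short delay timing the root motion jump force.
; The jump negates the look-at rotator toward a fixed point above the origin, and the ability ends when it finishes.
; The FlowingTides knockback event listener only prints debug text.
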(event Ability|EventActivateAbility
  (Development|PrintString "TidePull Activated")
  (AI|Navigation|MovetoLocation "None" (Math|Vector|MakeVector 0.0 0.0 (.z (Transformation|GetActorLocation (Ability|GetAvatarActorfromActorInfo)))) 1.0
    (:then
      (Ability|Tasks|WaitGameplayEvent "(TagName=\"Event.FlowingTides.Knockback\")" 0
        (:then
          (Utilities|FlowControl|Delay 1.2))
        (:EventReceived
          (Development|PrintString "got event" true true "(R=1.000000,G=0.000000,B=0.136464,A=1.000000)" 2345.0)))
      (|ApplyRootMotionJumpForce "None" (Class|KismetMathLibrary|NegateRotator (Math|Rotator|FindLookatRotation (Transformation|GetActorLocation (Ability|GetAvatarActorfromActorInfo)) (Math|Vector|MakeVector 0.0 0.0 1e+02))) 1e+02 1.5e+02 1.0 0.0 false "MaintainLastRootMotionVelocity" "0, 0, 0" 0.0
        (:OnFinish
          (Ability|EndAbility))))))

(event Ability|EventOnEndAbility
  (params (bWasCancelled :type Boolean)))