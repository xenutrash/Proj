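; BP_Nixaa is the character Blueprint for Nixaa, a water-themed fighter whose abilities run through the Gameplay Ability System.
; Attack and dash events activate Waterburst, Whirlpool and Submerge by gameplay tag, with Waterburst using the boss main-attack tag.
; Tick copies the Speed attribute into max walk speed every frame.
; Basic attack (Bite) and move are empty, and taunt only prints a debug string.
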(event EventOnTaunt
  (Development|PrintString "Taunt"))

(event EventOnBasicAttack
  ;[1 1 1] Bite
)

(event EventBeginPlay)

(event EventTick
  (params (DeltaSeconds :type Float%20%28single-precision%29))
  ;[1 1 1] que?
  (Variables|/Script/Engine.CharacterMovementComponent|SetMaxWalkSpeed (Variables|Character|GetCharacterMovement) (.currentvalue (Variables|/Script/Proj.RushAttributeSet|GetSpeed (Variables|Default|GetAttributes)))))

(event EventOnSpecialAttack
  ;[1 1 1] Secondary E = Waterburst
  (Development|PrintString "WaterBurst")
  (Abilities|TryActivateAbilitiesbyTag (Variables|Default|GetAbilitySystemComponent) (GameplayTags|MakeLiteralGameplayTagContainer "(GameplayTags=((TagName=\"Attack.Boss.Main\")))") true))

(event EventOnUltimateAttack
  ;[1 1 1] Third Q = Whirlpool
  (Development|PrintString "Used whirlpool")
  (Abilities|TryActivateAbilitiesbyTag (Variables|Default|GetAbilitySystemComponent) (GameplayTags|MakeLiteralGameplayTagContainer "(GameplayTags=((TagName=\"Attack.Special\")))") true))

(event EventOnDash
  (Abilities|TryActivateAbilitiesbyTag (Variables|Default|GetAbilitySystemComponent) (GameplayTags|MakeLiteralGameplayTagContainer "(GameplayTags=((TagName=\"Attack.Submerge\")))") true))

(event EventOnMove)

(fn ConstructionScript
  (|CallParentFunction))