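; BP_NixaBurstProjectile is a projectile that damages players on overlap using the Gameplay Ability System.
; Its Box overlap event ignores other projectiles and only prints a debug message when it touches its owner.
; A player-tagged hit with a valid ability system component receives GE_TakeDamage, then the projectile destroys itself.
; Any other overlap destroys it without damage, while a player lacking that component leaves it intact.
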(event OnComponentBeginOverlap(Box)
  (params (OverlappedComponent :type Primitive%20Component%20Object%20Reference) (OtherActor :type Actor%20Object%20Reference) (OtherComp :type Primitive%20Component%20Object%20Reference) (OtherBodyIndex :type Integer) (bFromSweep :type Boolean) (SweepResult :type Hit%20Result%20Structure%20%28by%20ref%29))
  (bind _returnvalue (Ability|GetAbilitySystemComponent 0))
  (if (== OtherActor (Components|GetOwner))
    (Development|PrintString "I hit myself ")
    (elif (not (Actor|ActorHasTag "Projectile"))
      (if (Actor|ActorHasTag "player")
        (Utilities|IsValid _returnvalue
          (:Is%20Valid
            (GameplayEffects|ApplyGameplayEffectToSelf :self _returnvalue :GameplayEffectClass "/Game/Programming/Blueprints/GE_TakeDamage.GE_TakeDamage_C")
            (Actor|DestroyActor)))
        (else
          (Actor|DestroyActor))))))

(fn ConstructionScript)