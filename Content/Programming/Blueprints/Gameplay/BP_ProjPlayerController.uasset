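; Player controller for the rush character that owns the local player's HUD and end-game menu.
; On possess, the local controller creates stats and cooldown widgets, sets "Nixa" icons and links itself to the controlled character.
; Tick rotates that character locally, while events forward health and Q, E and Space cooldowns to the HUD, disable pawn input or show the winner.
; The input mapping context setup is left unconnected.
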(event Custom|Health%20changed
  (params (HealthText :type Text) (HealthPercent :type Float%20%28double-precision%29))
  (Default|UpdateHealth (Variables|Default|GetWidget) HealthPercent HealthText))

(event Custom|EndGame
  (params (NewParam :type String))
  (if (Pawn|IsLocalController)
    (bind _returnvalue (UserInterface|CreateWidget "/Game/Programming/Lobby/Widgets/WP_EndGameMenu.WP_EndGameMenu_C"))
    (Default|SetWinnerText _returnvalue NewParam)
    (UserInterface|Viewport|AddtoViewport _returnvalue 0)))

(event Custom|Disable%20All%20Input
  (if (Pawn|IsLocalController)
    (Input|DisableInput (Pawn|GetControlledPawn) self)))

(event Custom|StartCooldownE
  (params (TimerE :type Integer))
  ;[1 1 1] Starts cooldown of interface
  (Default|StartCooldownE (Variables|Default|GetCooldownUI) TimerE))

(event Custom|StartCooldownQ
  (params (TimerQ :type Integer))
  ;[1 1 1] Starts cooldown of interface
  (Default|StartCooldownQ (Variables|Default|GetCooldownUI) TimerQ))

(event Custom|StartCooldownSpace
  (params (TimerE :type Integer))
  ;[1 1 1] Starts cooldown of interface
  (Default|StartCooldownSpace (Variables|Default|GetCooldownUI) TimerE))

(event EventPossess
  (params (PossessedPawn :type Pawn%20Object%20Reference))
  (Development|PrintString "posses")
  (if (Pawn|IsLocalController)
    (bind _returnvalue (UserInterface|CreateWidget "/Game/Programming/Blueprints/Widgets/WBP_Stats.WBP_Stats_C"))
    (bind _output_get (Variables|Default|SetWidget _returnvalue))
    (bind _returnvalue_2 (UserInterface|CreateWidget "/Game/Programming/Blueprints/Widgets/WBP_Cooldowns.WBP_Cooldowns_C"))
    (Default|AddHealthBarWidget _returnvalue_2 _output_get)
    (bind _output_get_2 (Variables|Default|SetCooldownUI _returnvalue_2))
    (UserInterface|Viewport|AddtoViewport _returnvalue_2 0)
    (Default|SetHUDIcons _returnvalue_2 "Nixa" "None")
    (bind _asbp_rush_character (Utilities|Casting|CastToBP_RushCharacter (Game|Player|GetPlayerPawn 0)))
    (bind _output_get_3 (Variables|Default|SetControlled%20Pawn _asbp_rush_character))
    (Variables|/Game/Programming/Blueprints/BP_RushCharacter.BP_RushCharacter_C|SetPlayerController _output_get_3 self)))

(event EventTick
  (params (DeltaSeconds :type Float%20%28single-precision%29))
  (bind _controlled_pawn (Variables|Default|GetControlled%20Pawn))
  (Utilities|IsValid _controlled_pawn
    (:Is%20Valid
      (if (Pawn|IsLocalController)
        (Default|RotateCharacter _controlled_pawn)))))

(fn ConstructionScript)