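; BP_Water is a level-effect water plane whose material renders a whirlpool with a controllable position and radius.
; On BeginPlay it creates a dynamic instance of M_Water_Inst and applies it to the plane.
; Setter functions write the whirlpool's X/Y location and radius into scalar material parameters.
; AnimateRadius plays a timeline from the start to drive the radius, leaving its Time input unused.
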(event Custom|AnimateRadius
  (params (Time :type Float%20%28double-precision%29))
  (bind _radius (Timeline|RadiusTimeline PlayFromStart)
    (:Update
      (CallFunction|SetWhirlpoolRadius _radius))))

(event EventBeginPlay
  (bind _returnvalue (Rendering|Material|CreateDynamicMaterialInstance "/Game/Material/M_Water_Inst.M_Water_Inst" "Water" "None" :!class /Script/Engine.KismetMaterialLibrary))
  (bind _output_get (Variables|Default|SetWater%20Material _returnvalue))
  (Rendering|Material|SetMaterial (Variables|Default|GetWaterPlane) 0 _output_get))

(fn ConstructionScript)

(fn SetWhirlpoolLocation
  (params (Location :type Vector))
  (bind (_x _y) (Math|Vector|BreakVector Location))
  (bind _water_material (Variables|Default|GetWater%20Material))
  (Rendering|Material|SetScalarParameterValue _water_material "PosX" _x :!class /Script/Engine.MaterialInstanceDynamic)
  (Rendering|Material|SetScalarParameterValue _water_material "PosY" _y :!class /Script/Engine.MaterialInstanceDynamic))

(fn SetWhirlpoolRadius
  (params (Radius :type Float%20%28double-precision%29))
  (Rendering|Material|SetScalarParameterValue (Variables|Default|GetWater%20Material) "Radius" Radius :!class /Script/Engine.MaterialInstanceDynamic))