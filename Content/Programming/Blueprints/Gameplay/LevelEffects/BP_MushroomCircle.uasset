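; Mushroom circle level effect that, while active, grants ultimate charge to hero characters standing in it through homing Niagara wisps.
; StartCircle shows the effect and runs a looping timer that spawns a wisp for each overlapping hero without a ready ultimate, then fades out via timeline.
; Tick moves each mapped wisp toward its hero, adding charge and destroying it on arrival, with a charge sound for the local player.
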(event Custom|Start%20Circle
  (params (ApplyTime :type Float%20%28double-precision%29) (ActiveTime :type Float%20%28double-precision%29) (Float%20UltChargeToAdd :type Float%20%28double-precision%29))
  (Niagara|ResetSystem (Variables|Default|GetNS_Mushroomcircle))
  (Rendering|SetActorHiddenInGame false)
  (bind _returnvalue (Utilities|Time|SetTimerbyEvent (delegate Custom|SpawnWisp) ApplyTime true))
  (Utilities|FlowControl|Delay ActiveTime)
  (Utilities|Time|PauseTimerbyHandle _returnvalue)
  (bind _newtrack_0 (Timeline|Timeline PlayFromStart)
    (:Update
      (Niagara|SetNiagaraVariable(Float) (Variables|Default|GetNS_Mushroomcircle) "Alpha" _newtrack_0))
    (:Finished
      (Rendering|SetActorHiddenInGame true))))

(event Custom|AddUltCharge
  (params (Character :type BP%20Rush%20Character%20Object%20Reference))
  (Default|ChargeUltimate Character (stale Custom|Start%20Circle Float%20UltChargeToAdd))
  (if (Pawn|IsLocallyControlled Character)
    (Default|PlayEventAttachedLocally (Variables|/Game/Programming/Blueprints/BP_RushCharacter.BP_RushCharacter_C|GetSoundSystem Character) "/Game/FMOD/Events/NonWorld/Combat/Ultimate_Charge.Ultimate_Charge" (Variables|/Script/Engine.Actor|GetRootComponent Character) false)))

(event Custom|SpawnWisp
  (for _array_element (Variables|Default|GetCharactersInTheCircle)
    (if (not (Variables|/Game/Programming/Blueprints/BP_RushCharacter.BP_RushCharacter_C|GetUltimateReady _array_element))
      (bind _returnvalue (Niagara|SpawnSystematLocation "/Game/Niagara/NS_Wisp.NS_Wisp" "0.000000,0.000000,500.000000"))
      (Utilities|Map|Add (Variables|Default|GetComponents) _returnvalue _array_element))))

(event EventTick
  (params (DeltaSeconds :type Float%20%28single-precision%29))
  ;[1 1 1] Wisp follow player and give ult charge when near
  (bind _keys (Utilities|Map|Keys (Variables|Default|GetComponents)))
  (for _array_element _keys
    (bind (_close _location) (CallFunction|WispFollow _array_element (.Value (Utilities|Map|Find (Variables|Default|GetComponents) _array_element))))
    (if _close
      (bind _asbp_rush_character (Utilities|Casting|CastToBP_RushCharacter (.Value (Utilities|Map|Find (Variables|Default|GetComponents) _array_element))))
      (CallFunction|AddUltCharge _asbp_rush_character)
      (Niagara|SpawnSystematLocation "/Game/Niagara/Ns_Wisp_Disappear.Ns_Wisp_Disappear" (Transformation|GetActorLocation (.Value (Utilities|Map|Find (Variables|Default|GetComponents) _array_element))))
      (Utilities|Map|Remove (Variables|Default|GetComponents) _array_element)
      (Components|DestroyComponent _array_element)
      (else
        (Transformation|AddWorldOffset _array_element _location false false)))))

(event Collision|EventActorBeginOverlap
  (params (OtherActor :type Actor%20Object%20Reference))
  (if (Actor|ActorHasTag OtherActor "Hero")
    (bind _asbp_rush_character (Utilities|Casting|CastToBP_RushCharacter OtherActor))
    (Utilities|Array|AddUnique (Variables|Default|GetCharactersInTheCircle) _asbp_rush_character)))

(event Collision|EventActorEndOverlap
  (params (OtherActor :type Actor%20Object%20Reference))
  (if (Actor|ActorHasTag OtherActor "Hero")
    (bind _asbp_rush_character (Utilities|Casting|CastToBP_RushCharacter OtherActor))
    (Utilities|Array|RemoveItem (Variables|Default|GetCharactersInTheCircle) _asbp_rush_character)))

(fn ConstructionScript)

(fn WispFollow
  (params (Wisp :type Scene%20Component%20Object%20Reference) (CharacterToFollow :type Actor%20Object%20Reference))
  (bind _returnvalue (Transformation|GetActorLocation CharacterToFollow))
  (bind _returnvalue_2 (Transformation|GetWorldLocation Wisp))
  (return (<= (Math|Vector|VectorLength (- _returnvalue _returnvalue_2)) (Variables|Default|GetWispClose)) (* (* (Math|Vector|Normalize (Math|Vector|GetUnitDirection(Vector) _returnvalue_2 _returnvalue)) (Variables|Default|GetSpeedOfWisp)) (Utilities|Time|GetWorldDeltaSeconds))))