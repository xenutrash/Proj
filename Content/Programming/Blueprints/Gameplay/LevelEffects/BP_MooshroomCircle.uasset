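; BP_MooshroomCircle is a level-effect zone that periodically grants ultimate charge to heroes standing inside it for a limited time.
; Overlap events track BP_RushCharacters, though end overlap checks the Hero tag on itself rather than the other actor.
; StartCircle runs a looping timer for the active duration, then pauses it and clears the list.
; Each tick applies GE_SetMaxSpeed, despite its name, with an Attack.Ultimate SetByCaller magnitude.
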(event Custom|Start%20Circle
  (params (ApplyTime :type Float%20%28double-precision%29) (ActiveTime :type Float%20%28double-precision%29) (Float%20UltChargeToAdd :type Float%20%28double-precision%29))
  (bind _returnvalue (Utilities|Time|SetTimerbyEvent (delegate Custom|AddUltCharge) ApplyTime true))
  (Utilities|FlowControl|Delay ActiveTime)
  (Utilities|Time|PauseTimerbyHandle _returnvalue)
  (Utilities|Array|Clear (Variables|Default|GetCharactersInTheCircle)))

(event Custom|AddUltCharge
  (for _array_element (Variables|Default|GetCharactersInTheCircle)
    (bind _returnvalue (Ability|GameplayEffect|AssignTagSetbyCallerMagnitude (GameplayEffects|MakeOutgoingSpec :self (Variables|/Script/Proj.RushCharacter|GetAbilitySystemComponent _array_element) :GameplayEffectClass "/Game/Programming/Blueprints/GeneralAbilities/GE_SetMaxSpeed.GE_SetMaxSpeed_C") "(TagName=\"Attack.Ultimate\")" (stale Custom|Start%20Circle Float%20UltChargeToAdd)))
    (GameplayEffects|ApplyGameplayEffectSpecToSelf (Variables|/Script/Proj.RushCharacter|GetAbilitySystemComponent _array_element) _returnvalue)))

(event EventBeginPlay)

(event Collision|EventActorBeginOverlap
  (params (OtherActor :type Actor%20Object%20Reference))
  (if (Actor|ActorHasTag OtherActor "Hero")
    (bind _asbp_rush_character (Utilities|Casting|CastToBP_RushCharacter OtherActor))
    (Utilities|Array|AddUnique (Variables|Default|GetCharactersInTheCircle) _asbp_rush_character)
    (Development|PrintString "Player Entered the circle")))

(event EventTick
  (params (DeltaSeconds :type Float%20%28single-precision%29)))

(event Collision|EventActorEndOverlap
  (params (OtherActor :type Actor%20Object%20Reference))
  (if (Actor|ActorHasTag "Hero")
    (bind _asbp_rush_character (Utilities|Casting|CastToBP_RushCharacter OtherActor))
    (Utilities|Array|RemoveItem (Variables|Default|GetCharactersInTheCircle) _asbp_rush_character)
    (Development|PrintString "Player exited teh circle")))

(fn ConstructionScript)