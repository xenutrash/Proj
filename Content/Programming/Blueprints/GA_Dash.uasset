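; GA_Dash is a Gameplay Ability that dashes the avatar along its current horizontal movement direction.
; After committing, it spawns the NS_Hero_Dash effect at the avatar and applies a constant root motion force using the normalized XY velocity, with variable strength and duration.
; The avatar keeps the last root motion velocity when the force finishes and the ability ends; a failed commit cancels it.
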(event Ability|EventActivateAbility
  (bind _returnvalue (Ability|GetAvatarActorfromActorInfo))
  (bind _returnvalue_2 (Transformation|GetVelocity _returnvalue))
  (bind _returnvalue_3 (Ability|CommitAbility))
  (if _returnvalue_3
    (Variables|Default|SetDirection (Math|Vector|Normalize (Math|Vector|MakeVector (.x _returnvalue_2) (.y _returnvalue_2) 0.0)))
    (Niagara|SpawnSystematLocation "/Game/Niagara/NS_Hero_Dash.NS_Hero_Dash" (Transformation|GetActorLocation _returnvalue) (Transformation|GetActorRotation _returnvalue))
    (Ability|Tasks|ApplyRootMotionConstantForce "None" (Variables|Default|GetDirection) (Variables|Default|GetStrength) (Variables|Default|GetDuration) false 0 "MaintainLastRootMotionVelocity" (Transformation|GetVelocity (Ability|GetAvatarActorfromActorInfo))
      (:OnFinish
        (Ability|EndAbility)))
    (else
      (Ability|CancelAbility))))

(event Ability|EventOnEndAbility
  (params (bWasCancelled :type Boolean)))