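; BP_SoundSystem is a Blueprint that plays sound events at a world location, either locally or, as its event names indicate, on all clients.
; Each all-clients entry event forwards to a matching FromServer event, which calls PlayEventAtLocation with auto-play.
; The exclude-owner variant passes its Target along as Caller and skips playback where that equals the local player controller at index 0.
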(event Custom|Play%20Sound%20Locally
  (params (Event :type FMOD%20Event%20Object%20Reference) (Location :type Transform%20%28by%20ref%29))
  ;[1 1 1] Play sound locally
  (Class|FMODBlueprintStatics|PlayEventatLocation Event Location))

(event Custom|Play%20Sound%20All%20Clients
  (params (Event :type FMOD%20Event%20Object%20Reference) (Location :type Transform%20%28by%20ref%29))
  ;[1 1 1] Play sound on all clients
  (CallFunction|PlaySoundAllClientsfromServer Event Location))

(event Custom|Play%20Sound%20All%20Clients%20Exclude%20Owner
  (params (Event :type FMOD%20Event%20Object%20Reference) (Location :type Transform%20%28by%20ref%29) (Target :type Controller%20Object%20Reference))
  ;[1 1 1] Play sound on all clients but exclude the owner
  (CallFunction|PlaySoundAllClientsExcludeOwnerfromServer Event Location Target))

(event Custom|Play%20Sound%20All%20Clients%20Exclude%20Owner%20From%20Server
  (params (Event :type FMOD%20Event%20Object%20Reference) (Location :type Transform%20%28by%20ref%29) (Caller :type Controller%20Object%20Reference))
  ;[1 1 1] Play sound on all clients but exclude the owner
  (if (not (== Caller (Game|GetPlayerController 0)))
    (Class|FMODBlueprintStatics|PlayEventatLocation Event Location)))

(event Custom|Play%20Sound%20All%20Clients%20From%20Server
  (params (Event :type FMOD%20Event%20Object%20Reference) (Location :type Transform%20%28by%20ref%29))
  ;[1 1 1] Play sound on all clients
  (Class|FMODBlueprintStatics|PlayEventatLocation Event Location))