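; GA_Dash is a gameplay ability that dashes the avatar along its horizontal movement direction and applies an invincibility effect.
; On activation it commits the cooldown and plays a sped-up slide montage, then waits for the Movement.Dash gameplay event.
; That event triggers a constant root motion force and the invincibility effect.
; The ability ends when the force finishes or the montage blends out or is interrupted; dash VFX is left unwired.
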(event Ability|EventActivateAbility
  (bind _returnvalue (Ability|GetAvatarActorfromActorInfo))
  (bind _returnvalue_2 (Transformation|GetVelocity _returnvalue))
  (Ability|CommitAbilityCooldown false true)
  (|PlayMontageandWaitProxy "None" "/Game/TEMP/AM_Slide.AM_Slide" 2.0 "None" true 1.0 0.2 false
    (:then
      (Ability|Tasks|WaitGameplayEvent "(TagName=\"Movement.Dash\")" 0
        (:then
          (Variables|Default|SetDirection (Math|Vector|Normalize (Math|Vector|MakeVector (.x _returnvalue_2) (.y _returnvalue_2) 0.0)))
          (Ability|Tasks|ApplyRootMotionConstantForce "None" (Variables|Default|GetDirection) (Variables|Default|GetStrength) (Variables|Default|GetDuration) false 0 "MaintainLastRootMotionVelocity" (Transformation|GetVelocity _returnvalue)
            (:then
              (Ability|ApplyGameplayEffectToOwner "/Game/Programming/Blueprints/GeneralAbilities/GE_AddInvincibility.GE_AddInvincibility_C")
              (Development|PrintString "Successful Dash"))
            (:OnFinish
              (Ability|EndAbility))))))
    (:OnBlendOut
      (Ability|EndAbility :!label _label))
    (:OnInterrupted
      (goto _label))
    (:OnCancelled
      (goto _label))))

(event Ability|EventOnEndAbility
  (params (bWasCancelled :type Boolean))
  (Development|PrintString "End Dash"))