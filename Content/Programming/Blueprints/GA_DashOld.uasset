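; GA_DashOld is a hero dash gameplay ability, named as an older version.
; On activation it calls PlayMontage, then stores the avatar's normalized horizontal velocity as Direction.
; It spawns the NS_Hero_Dash Niagara effect at the avatar's location and rotation, then hands off to the parent activation.
; The graph applies no movement itself, and its OnEndAbility override is disabled.
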(event Ability|EventActivateAbility
  (bind _returnvalue (Ability|GetAvatarActorfromActorInfo))
  (bind _returnvalue_2 (Transformation|GetVelocity _returnvalue))
  (Animation|Montage|PlayMontage 0 0
    (:then
      (Variables|Default|SetDirection (Math|Vector|Normalize (Math|Vector|MakeVector (.x _returnvalue_2) (.y _returnvalue_2) 0.0)))
      (Niagara|SpawnSystematLocation "/Game/Niagara/NS_Hero_Dash.NS_Hero_Dash" (Transformation|GetActorLocation _returnvalue) (Transformation|GetActorRotation _returnvalue))
      (|CallParentFunction))))

(event Ability|EventOnEndAbility
  (params (bWasCancelled :type Boolean))
  (|CallParentFunction bWasCancelled) ; This node is disabled and will not be called.\nDrag off pins to build functionality.
)