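; GA_SmellingSalts is the Plague Doctor's Smelling Salts gameplay ability.
; It plays the AM_SmellingSalt montage and, on an Attack.Special gameplay event, spawns BP_SmellingSalt attached to the avatar's ik_hand_gun socket and commits the cooldown.
; The ability ends when the montage completes, blends out, is interrupted or is cancelled, and prints a debug message on end.
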(event Ability|EventActivateAbility
  (bind _returnvalue (Ability|GetAvatarActorfromActorInfo))
  (bind _returnvalue_2 (Actor|GetComponentbyClass _returnvalue "/Script/Engine.SkeletalMeshComponent"))
  (|PlayMontageandWaitProxy "None" "/Game/Characters/PlagueDoctor/PlaceHolders/AM_SmellingSalt.AM_SmellingSalt" 1.0 "None" true 1.0 0.0 false
    (:then
      (Ability|Tasks|WaitGameplayEvent "(TagName=\"Attack.Special\")" 0
        (:EventReceived
          (bind _returnvalue_3 (Game|SpawnActorfromClass "/Game/Programming/Blueprints/PlagueDoctor/SmellingSalts/BP_SmellingSalt.BP_SmellingSalt_C" (Math|Transform|MakeTransform (Transformation|GetSocketLocation _returnvalue_2 "ik_hand_gun") (Transformation|GetActorRotation _returnvalue) "1.000000,1.000000,1.000000") "Undefined" "MultiplyWithRoot" _returnvalue 0))
          (Transformation|AttachComponentToComponent _returnvalue_3 _returnvalue_2 "ik_hand_gun" "SnapToTarget" "SnapToTarget" "SnapToTarget" true)
          (Ability|CommitAbilityCooldown false true))))
    (:OnCompleted
      (Ability|EndAbility :!label _label))
    (:OnBlendOut
      (goto _label))
    (:OnInterrupted
      (goto _label))
    (:OnCancelled
      (goto _label))))

(event Ability|EventOnEndAbility
  (params (bWasCancelled :type Boolean))
  (Development|PrintString "Smelling Salts ended"))