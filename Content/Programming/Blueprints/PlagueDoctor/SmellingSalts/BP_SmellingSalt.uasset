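; BP_SmellingSalt is the Plague Doctor's smelling salts area actor, applying a gameplay effect to characters that enter its HitRange.
; Each overlapping actor is recorded so it is processed only once, and any RushCharacter receives GE_SmellingSaltOverTime through its ability system component.
; On BeginPlay it feeds its offset yaw into the placeholder Niagara effect's Rotation variable to orient the visuals.
; Debug prints report the rotation and effect results.
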(event OnComponentBeginOverlap(HitRange)
  (params (OverlappedComponent :type Primitive%20Component%20Object%20Reference) (OtherActor :type Actor%20Object%20Reference) (OtherComp :type Primitive%20Component%20Object%20Reference) (OtherBodyIndex :type Integer) (bFromSweep :type Boolean) (SweepResult :type Hit%20Result%20Structure%20%28by%20ref%29))
  (bind _actorshit (Variables|Default|GetActorsHit))
  (if (not (Utilities|Array|ContainsItem _actorshit OtherActor))
    (Utilities|Array|Add _actorshit OtherActor)
    (CallFunction|ApplyEffect OtherActor)))

(event Collision|EventActorBeginOverlap
  (params (OtherActor :type Actor%20Object%20Reference)))

(event EventTick
  (params (DeltaSeconds :type Float%20%28single-precision%29)))

(event EventBeginPlay
  (bind _returnvalue (Transformation|GetActorRotation))
  (bind _returnvalue_2 (- (.yaw _returnvalue) 9e+01))
  ;[1 1 1] Effect Rotation
  (Development|PrintString (Utilities|String|ToString(Float) _returnvalue_2))
  (Niagara|SetNiagaraVariable(Float) (Variables|Default|GetNS_SmellingSalts_PlaceHolder) "Rotation" _returnvalue_2))

(fn ConstructionScript)

(fn ApplyEffect
  (params (Object :type Object%20Object%20Reference))
  (bind _asrush_character (Utilities|Casting|CastToRushCharacter Object)
    (:then
      (GameplayEffects|ApplyGameplayEffectToSelf :self (Ability|GetAbilitySystemComponent _asrush_character) :GameplayEffectClass "/Game/Programming/Blueprints/PlagueDoctor/SmellingSalts/GE_SmellingSaltOverTime.GE_SmellingSaltOverTime_C")
      (Development|PrintString "Effect applied"))
    (:CastFailed
      (Development|PrintString "Not a RushCharacter"))))