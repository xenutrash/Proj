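; Gameplay ability GA_WaterBurst that spawns a BP_Projectile_Base at the avatar's location when activated.
; It traces 1000 units along the deprojected mouse direction on the Visibility channel, with persistent debug drawing.
; Spawn rotation is a look-at built from only the Z values of avatar and hit locations.
; CommitAbility is unconnected, pending a possible mana system, and the ability never calls EndAbility.
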(event Ability|EventActivateAbility
  (bind _returnvalue (Ability|GetAvatarActorfromActorInfo))
  (bind _returnvalue_2 (Game|GetPlayerController))
  (bind _returnvalue_3 (Transformation|GetActorLocation _returnvalue))
  (bind (_worldlocation _worlddirection) (Game|Player|ConvertMouseLocationToWorldSpace _returnvalue_2))
  (Class|WidgetLayoutLibrary|GetMousePositiononViewport)
  (bind _outhit (Collision|LineTraceByChannel _worldlocation (+ _worldlocation (* _worlddirection 1e+03)) "TraceTypeQuery1" false 0 "Persistent"))
  (Game|SpawnActorfromClass "/Game/Programming/Blueprints/BP_Projectile_Base.BP_Projectile_Base_C" (Math|Transform|MakeTransform (Math|Vector|MakeVector (.x _returnvalue_3) (.y _returnvalue_3) (.z _returnvalue_3)) (Math|Rotator|FindLookatRotation (Math|Conversions|ToVector(Float) (.z _returnvalue_3)) (Math|Conversions|ToVector(Float) (.z (.Location (Collision|BreakHitResult _outhit))))) "1.000000,1.000000,1.000000") "Undefined" "MultiplyWithRoot" _returnvalue 0))

(event Ability|EventOnEndAbility
  (params (bWasCancelled :type Boolean)))