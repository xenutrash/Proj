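; BP_Alchemist is the Alchemist character Blueprint, mapping its attack and dash events to Gameplay Ability System abilities.
; Basic attack, special attack and dash activate GA_AlchemistPrimaryFire, GA_SmellingSalts and GA_Dash by class through the AbilitySystemComponent.
; Each action prints a debug string, basic attack also prints its activation result, and ultimate only prints.
; BeginPlay, health changes and construction defer to the parent class.
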(event EventOnHealthChanged
  (params (DeltaValue :type Float%20%28single-precision%29) (EventTags :type Gameplay%20Tag%20Container%20Structure%20%28by%20ref%29))
  (|CallParentFunction DeltaValue EventTags))

(event EventBeginPlay
  (|CallParentFunction))

(event EventOnBasicAttack
  (Development|PrintString "Basic attack")
  (bind _returnvalue (Abilities|TryActivateAbilitybyClass (Variables|Default|GetAbilitySystemComponent) "/Game/Programming/Blueprints/Alchemist/PrimaryFire/GA_AlchemistPrimaryFire.GA_AlchemistPrimaryFire_C" true))
  (Development|PrintString (Utilities|String|ToString(Boolean) _returnvalue)))

(event EventOnSpecialAttack
  (Development|PrintString "Specialattack")
  (Abilities|TryActivateAbilitybyClass (Variables|Default|GetAbilitySystemComponent) "/Game/Programming/Blueprints/Alchemist/SmellingSalts/GA_SmellingSalts.GA_SmellingSalts_C" true))

(event EventOnUltimateAttack
  (Development|PrintString "Ultiamte attack"))

(event EventOnDash
  (Development|PrintString "Dash")
  (Abilities|TryActivateAbilitybyClass (Variables|Default|GetAbilitySystemComponent) "/Game/Programming/Blueprints/GA_Dash.GA_Dash_C" true))

(fn ConstructionScript
  (|CallParentFunction))