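; Gameplay Ability for the Slayer's three-step melee combo, playing one slash montage per activation based on the character's ComboCounter.
; It commits cooldown, then the server waits for an Attack.Basic event to advance the counter, sphere trace and end the ability.
; The first two hits trace short and wide, the third long and narrow.
; Unique Boss-tagged BP_RushCharacter hits take damage and charge the Slayer's ultimate.
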(event Ability|EventActivateAbility
  (bind _asbp_slayer (Utilities|Casting|CastToBP_Slayer (Ability|GetAvatarActorfromActorInfo)))
  (Variables|Default|SetSlayerCharacter _asbp_slayer)
  (Ability|CommitAbilityCooldown false true)
  (|PlayMontageandWaitProxy "None" (Utilities|Select :Index (Variables|/Game/Programming/Blueprints/Slayer/BP_Slayer.BP_Slayer_C|GetComboCounter (Variables|Default|GetSlayerCharacter)) :Option%200 "/Game/Animation/Slayer/Animations/Slash_1_Montage.Slash_1_Montage" :Option%201 "/Game/Animation/Slayer/Animations/Slash_2_Montage.Slash_2_Montage" :Option%202 "/Game/Animation/Slayer/Animations/Slash_3_Montage.Slash_3_Montage") 1.0 "None" true 1.0 0.0 false
    (:then
      (if (Networking|IsServer)
        (Ability|Tasks|WaitGameplayEvent "(TagName=\"Attack.Basic\")" 0 true
          (:EventReceived
            (switch int (Variables|/Game/Programming/Blueprints/Slayer/BP_Slayer.BP_Slayer_C|GetComboCounter (Variables|Default|GetSlayerCharacter))
              (:0
                (Variables|/Game/Programming/Blueprints/Slayer/BP_Slayer.BP_Slayer_C|SetComboCounter (Variables|Default|GetSlayerCharacter) 1)
                (CallFunction|FirstandSecondAttackSphere :!label _label))
              (:1
                (Variables|/Game/Programming/Blueprints/Slayer/BP_Slayer.BP_Slayer_C|SetComboCounter (Variables|Default|GetSlayerCharacter) 2)
                (goto _label))
              (:2
                (Variables|/Game/Programming/Blueprints/Slayer/BP_Slayer.BP_Slayer_C|SetComboCounter (Variables|Default|GetSlayerCharacter) 0)
                (CallFunction|ThirdAttackSphere)))
            ;[1 1 1] Should be removed when animations come
            (Ability|EndAbility)))))
    (:OnCompleted
      (Ability|EndAbility :!label _label_2))
    (:OnBlendOut
      (goto _label_2))
    (:OnInterrupted
      (goto _label_2))
    (:OnCancelled
      (goto _label_2))))

(fn ProcessHitActors
  (params (Array :type Array%20of%20Hit%20Result%20Structures))
  (for _array_element Array
    (Utilities|Array|AddUnique (Variables|Default|GetHitActors) (.HitActor (Collision|BreakHitResult _array_element))))
  (for _array_element_2 (Variables|Default|GetHitActors)
    (if (Actor|ActorHasTag _array_element_2 "Boss")
      (bind _asbp_rush_character (Utilities|Casting|CastToBP_RushCharacter _array_element_2))
      (Default|TakeDamage _asbp_rush_character (Variables|Default|GetDamage))
      (bind _asbp_slayer (Utilities|Casting|CastToBP_Slayer (Ability|GetAvatarActorfromActorInfo)))
      (Default|ChargeUltimate _asbp_slayer (Variables|Default|GetUltCharge))))
  (return))

(fn FirstandSecondAttackSphere
  (bind _returnvalue (Ability|GetAvatarActorfromActorInfo))
  (bind _returnvalue_2 (Transformation|GetActorLocation _returnvalue))
  (bind _returnvalue_3 (Transformation|GetActorForwardVector _returnvalue))
  (bind _returnvalue_4 (* _returnvalue_3 80))
  (bind _returnvalue_5 (* _returnvalue_3 200))
  (bind _returnvalue_6 (+ _returnvalue_2 _returnvalue_4))
  (bind _returnvalue_7 (+ _returnvalue_2 _returnvalue_5))
  (bind _outhits (Collision|MultiSphereTraceForObjects (Math|Vector|MakeVector (.x _returnvalue_6) (.y _returnvalue_6) (- (.z _returnvalue_6) 5e+01)) (Math|Vector|MakeVector (.x _returnvalue_7) (.y _returnvalue_7) (- (.z _returnvalue_7) 5e+01)) 1e+02 (Utilities|Array|MakeArray "ObjectTypeQuery3") false 0 "ForDuration"))
  (CallFunction|ProcessHitActors _outhits))

(fn ThirdAttackSphere
  (bind _returnvalue (Ability|GetAvatarActorfromActorInfo))
  (bind _returnvalue_2 (Transformation|GetActorLocation _returnvalue))
  (bind _returnvalue_3 (Transformation|GetActorForwardVector _returnvalue))
  (bind _returnvalue_4 (* _returnvalue_3 80))
  (bind _returnvalue_5 (* _returnvalue_3 400))
  (bind _returnvalue_6 (+ _returnvalue_2 _returnvalue_4))
  (bind _returnvalue_7 (+ _returnvalue_2 _returnvalue_5))
  (bind _outhits (Collision|MultiSphereTraceForObjects (Math|Vector|MakeVector (.x _returnvalue_6) (.y _returnvalue_6) (- (.z _returnvalue_6) 5e+01)) (Math|Vector|MakeVector (.x _returnvalue_7) (.y _returnvalue_7) (- (.z _returnvalue_7) 5e+01)) 5e+01 (Utilities|Array|MakeArray "ObjectTypeQuery3") false 0 "ForDuration"))
  (CallFunction|ProcessHitActors _outhits))