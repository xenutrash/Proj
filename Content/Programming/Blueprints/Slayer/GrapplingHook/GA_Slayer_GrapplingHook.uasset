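; Gameplay ability for the Slayer's grappling hook, which plays a throw montage and spawns the hook actor.
; It force-commits the cooldown on activation and ends when the montage completes, blends out, is interrupted or is cancelled.
; On the server only, it waits once for a Movement.Dash gameplay event, then spawns BP_Slayer_GrapplingHook at the avatar's head socket, facing the actor's rotation.
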(event Ability|EventActivateAbility
  (bind _returnvalue (Ability|GetAvatarActorfromActorInfo))
  (Ability|CommitAbilityCooldown false true)
  (|PlayMontageandWaitProxy "None" "/Game/Programming/Blueprints/Alchemist/PlaceHolders/AM_ThrowAttack.AM_ThrowAttack" 1.0 "None" false 1.0 0.0 false
    (:then
      (if (Networking|IsServer)
        (Ability|Tasks|WaitGameplayEvent "(TagName=\"Movement.Dash\")" 0 true
          (:EventReceived
            (Game|SpawnActorfromClass "/Game/Programming/Blueprints/Slayer/GrapplingHook/BP_Slayer_GrapplingHook.BP_Slayer_GrapplingHook_C" (Math|Transform|MakeTransform (Transformation|GetSocketLocation (Actor|GetComponentbyClass _returnvalue "/Script/Engine.SkeletalMeshComponent") "head") (Transformation|GetActorRotation _returnvalue) "1.000000,1.000000,1.000000") "Undefined" "MultiplyWithRoot" _returnvalue 0)))))
    (:OnCompleted
      (Ability|EndAbility :!label _label))
    (:OnBlendOut
      (goto _label))
    (:OnInterrupted
      (goto _label))
    (:OnCancelled
      (goto _label))))