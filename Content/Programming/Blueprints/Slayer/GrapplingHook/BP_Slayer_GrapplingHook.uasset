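; Slayer's grappling hook projectile, which drags the Slayer to terrain or pulls Hero-tagged actors toward the Slayer.
; Separate terrain and ally overlap components classify the hit, stop the projectile and play montages and sounds; a short timeout counts as a miss.
; Tick then applies the matching drag or flies the hook back using per-frame world offsets.
; Getting close cancels the hook and detaches the line, while hits also self-destroy after a delay.
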(event OnComponentBeginOverlap(TerrainHook)
  (params (OverlappedComponent :type Primitive%20Component%20Object%20Reference) (OtherActor :type Actor%20Object%20Reference) (OtherComp :type Primitive%20Component%20Object%20Reference) (OtherBodyIndex :type Integer) (bFromSweep :type Boolean) (SweepResult :type Hit%20Result%20Structure%20%28by%20ref%29))
  (bind _valid (CallFunction|CompareActorHit OtherActor))
  (if _valid
    (if (not (Actor|ActorHasTag (Variables|Default|GetTargetHit) "Hero"))
      (CallFunction|PlaySound "/Game/FMOD/Events/InWorld/LocalPlayer/Hero/Slayer/Local_Slayer_GrapplingHookHit.Local_Slayer_GrapplingHookHit" "/Game/FMOD/Events/InWorld/NonLocalPlayer/Hero/Slayer/NonLocal_Slayer_GrapplingHookHit.NonLocal_Slayer_GrapplingHookHit" "Hook")
      (Default|PlayAnimation (Variables|Default|GetSlayer%20Character) "/Game/Animation/Slayer/NewFolder/Slayer_Hook_Slide_Montage.Slayer_Hook_Slide_Montage")
      (Variables|Default|SetTargetHitName "Terrain")
      (Default|EventInstanceSetParameter (Variables|/Game/Programming/Blueprints/BP_RushCharacter.BP_RushCharacter_C|GetSoundSystem (Variables|Default|GetSlayer%20Character)) "GrapplingHookHit" 0.0 (Utilities|String|MakeLiteralString "Hook"))
      (Variables|Default|SetTarget (Transformation|GetWorldLocation (Variables|Default|GetTerrainHook)))
      (CallFunction|StopHook)
      (Utilities|FlowControl|Delay 3.0)
      (Actor|DestroyActor))))

(event OnComponentBeginOverlap(AlliesHook)
  (params (OverlappedComponent :type Primitive%20Component%20Object%20Reference) (OtherActor :type Actor%20Object%20Reference) (OtherComp :type Primitive%20Component%20Object%20Reference) (OtherBodyIndex :type Integer) (bFromSweep :type Boolean) (SweepResult :type Hit%20Result%20Structure%20%28by%20ref%29))
  (bind _valid (CallFunction|CompareActorHit OtherActor))
  (if _valid
    (if (Actor|ActorHasTag (Variables|Default|GetTargetHit) "Hero")
      (CallFunction|PlaySound "/Game/FMOD/Events/InWorld/LocalPlayer/Hero/Slayer/Local_Slayer_GrapplingHookHit.Local_Slayer_GrapplingHookHit" "/Game/FMOD/Events/InWorld/NonLocalPlayer/Hero/Slayer/NonLocal_Slayer_GrapplingHookHit.NonLocal_Slayer_GrapplingHookHit" "Hook")
      (Default|PlayAnimation (Variables|Default|GetSlayer%20Character) "/Game/Animation/Slayer/NewFolder/Slayer_Hook_Pull_Montage.Slayer_Hook_Pull_Montage")
      (Variables|Default|SetTargetHitName "Hero")
      (Default|EventInstanceSetParameter (Variables|/Game/Programming/Blueprints/BP_RushCharacter.BP_RushCharacter_C|GetSoundSystem (Variables|Default|GetSlayer%20Character)) "GrapplingHookHit" 1.0 (Utilities|String|MakeLiteralString "Hook"))
      (CallFunction|StopHook)
      (Utilities|FlowControl|Delay 3.0)
      (Actor|DestroyActor))))

(event Custom|CancelHook
  ;[1 1 1] Cancel the hook
  (if (not (Variables|Default|GetCancelled))
    (Variables|Default|SetCancelled true)
    (Default|StopAnimation (Variables|Default|GetSlayer%20Character) "/Game/Animation/Slayer/NewFolder/Slayer_Hook_Slide_Montage.Slayer_Hook_Slide_Montage")
    (Default|StopAnimation (Variables|Default|GetSlayer%20Character) "/Game/Animation/Slayer/NewFolder/Slayer_Hook_Hold_Montage.Slayer_Hook_Hold_Montage")
    (CallFunction|DetachLinetoGrappling)
    (Default|EventInstanceAttachedStop (Variables|/Game/Programming/Blueprints/BP_RushCharacter.BP_RushCharacter_C|GetSoundSystem (Variables|Default|GetSlayer%20Character)) "GrapplingHook")
    (Actor|DestroyActor)))

(event Custom|AttachLineToGrappling
  ;[1 1 1] Attach and detach grappling
  (CallFunction|AttachLinetoGrapplingMulti))

(event Custom|AttachLineToGrapplingMulti
  ;[1 1 1] Attach and detach grappling
  (Default|AttachGrappling (Variables|Default|GetSlayer%20Character) (Variables|Default|GetTerrainHook)))

(event Custom|DetachLineToGrappling
  ;[1 1 1] Attach and detach grappling
  (CallFunction|DetachLinetoGrapplingMulti))

(event Custom|DetachLineToGrapplingMulti
  ;[1 1 1] Attach and detach grappling
  (Default|DetachGrappling (Variables|Default|GetSlayer%20Character)))

(event EventBeginPlay
  (bind _asbp_slayer (Utilities|Casting|CastToBP_Slayer (Components|GetOwner)))
  (Variables|Default|SetSlayer%20Character _asbp_slayer)
  (CallFunction|AttachLinetoGrappling)
  (CallFunction|PlaySoundAttached "GrapplingHook" "/Game/FMOD/Events/InWorld/LocalPlayer/Hero/Slayer/Local_Slayer_GrapplingHook.Local_Slayer_GrapplingHook" "/Game/FMOD/Events/InWorld/NonLocalPlayer/Hero/Slayer/NonLocal_Slayer_GrapplingHookHit.NonLocal_Slayer_GrapplingHookHit")
  (Utilities|FlowControl|Delay 0.05)
  (Variables|/Script/Engine.PrimitiveComponent|SetbGenerateOverlapEvents (Variables|Default|GetTerrainHook) true)
  (Variables|/Script/Engine.PrimitiveComponent|SetbGenerateOverlapEvents (Variables|Default|GetAlliesHook) true)
  (Utilities|FlowControl|Delay 0.4)
  (if (not (Variables|Default|GetHitSomething))
    (CallFunction|StopHook)
    (Variables|Default|SetSpeed 4e+03)))

(event EventTick
  (params (DeltaSeconds :type Float%20%28single-precision%29))
  (if (Variables|Default|GetHitSomething)
    (Default|EventInstanceAttatchedSetParameter (Variables|/Game/Programming/Blueprints/BP_RushCharacter.BP_RushCharacter_C|GetSoundSystem (Variables|Default|GetSlayer%20Character)) "GrapplingHook" 1.0 "GrapplingHook")
    (switch string (Variables|Default|GetTargetHitName)
      (:Default
        (CallFunction|ReturnHooktoPlayer))
      (:Hero
        (CallFunction|DragHeroTowardsPlayer)
        (CallFunction|ReturnHooktoPlayerHitHero))
      (:Terrain
        (CallFunction|DragTowardsTerrain)))))

(fn ConstructionScript)

(fn DragTowardsTerrain
  (bind _returnvalue (Components|GetOwner))
  (bind _returnvalue_2 (Transformation|GetActorLocation _returnvalue))
  (if (Variables|Default|GetTooClose)
    (CallFunction|CancelHook)
    (else
      (Variables|Default|SetTooClose (<= (Math|Vector|VectorLength (- (Variables|Default|GetTarget) _returnvalue_2)) (Variables|Default|GetClose)))
      (Transformation|AddActorWorldOffset _returnvalue (* (* (Math|Vector|Normalize (Math|Vector|GetUnitDirection(Vector) _returnvalue_2 (Variables|Default|GetTarget))) (Variables|Default|GetSpeed)) (Utilities|Time|GetWorldDeltaSeconds))))))

(fn DragHeroTowardsPlayer
  (bind _returnvalue (Components|GetOwner))
  (bind _returnvalue_2 (Transformation|GetActorLocation _returnvalue))
  (Variables|Default|SetTarget (Transformation|GetActorLocation (Variables|Default|GetTargetHit)))
  (if (Variables|Default|GetTooClose)
    (CallFunction|CancelHook)
    (else
      (Variables|Default|SetTooClose (<= (Math|Vector|VectorLength (- (Variables|Default|GetTarget) _returnvalue_2)) (Variables|Default|GetClose)))
      (Transformation|AddActorWorldOffset (Variables|Default|GetTargetHit) (* (Math|Vector|Normalize (Math|Vector|GetUnitDirection(Vector) (Variables|Default|GetTarget) _returnvalue_2)) (Variables|Default|GetSpeed) (Utilities|Time|GetWorldDeltaSeconds)) false true))))

(fn ReturnHooktoPlayer
  (bind _returnvalue (Transformation|GetActorLocation))
  (bind _slayer_character (Variables|Default|GetSlayer%20Character))
  (bind _returnvalue_2 (Transformation|GetActorLocation _slayer_character))
  (if (Variables|Default|GetTooClose)
    (CallFunction|CancelHook)
    (else
      (Variables|Default|SetTooClose (<= (Math|Vector|VectorLength (- _returnvalue _returnvalue_2)) (Variables|Default|GetClose)))
      (Transformation|AddActorWorldOffset self (* (* (Math|Vector|Normalize (Math|Vector|GetUnitDirection(Vector) _returnvalue _returnvalue_2)) (Variables|Default|GetSpeed)) (Utilities|Time|GetWorldDeltaSeconds))))))

(fn ReturnHooktoPlayerHitHero
  (bind _self self)
  (Utilities|IsValid _self
    (:Is%20Valid
      (Transformation|AddActorWorldOffset _self (* (* (Math|Vector|Normalize (Math|Vector|GetUnitDirection(Vector) (Transformation|GetActorLocation) (Transformation|GetActorLocation (Variables|Default|GetSlayer%20Character)))) (Variables|Default|GetSpeed)) (Utilities|Time|GetWorldDeltaSeconds)) false true))))

(fn PlaySoundAttached
  (params (NameOfKey :type String) (Local :type FMOD%20Event%20Object%20Reference) (NonLocal :type FMOD%20Event%20Object%20Reference))
  (Default|PlayEventAttachedLocally (Variables|/Game/Programming/Blueprints/BP_RushCharacter.BP_RushCharacter_C|GetSoundSystem (Variables|Default|GetSlayer%20Character)) Local (Variables|Transformation|GetRootComponent) true NameOfKey)
  (Default|PlayEventAttachedAllClientsExcludeOwner (Variables|/Game/Programming/Blueprints/BP_RushCharacter.BP_RushCharacter_C|GetSoundSystem (Variables|Default|GetSlayer%20Character)) NonLocal (Variables|Transformation|GetRootComponent) (Components|GetOwner) true NameOfKey))

(fn StopHook
  (bind _projectilemovement (Variables|Default|GetProjectileMovement))
  (Variables|Default|SetHitSomething true)
  (Variables|/Script/Engine.ProjectileMovementComponent|SetInitialSpeed _projectilemovement 0.0)
  (Variables|/Script/Engine.ProjectileMovementComponent|SetMaxSpeed _projectilemovement 0.0)
  (Components|Movement|StopMovementImmediately _projectilemovement)
  (Variables|/Script/Engine.MovementComponent|SetVelocity _projectilemovement "0, 0, 0"))

(fn PlaySound
  (params (Local :type FMOD%20Event%20Object%20Reference) (NonLocal :type FMOD%20Event%20Object%20Reference) (NameOfKey :type String))
  (bind _terrainhook (Variables|Default|GetTerrainHook))
  (bind _returnvalue (Transformation|GetWorldLocation _terrainhook))
  (bind _returnvalue_2 (Math|Conversions|ToTransform(Vector) _returnvalue))
  (Default|PlaySoundLocally (Variables|/Game/Programming/Blueprints/BP_RushCharacter.BP_RushCharacter_C|GetSoundSystem (Variables|Default|GetSlayer%20Character)) Local _returnvalue_2 true NameOfKey)
  (Default|PlaySoundAllClientsExcludeOwner (Variables|/Game/Programming/Blueprints/BP_RushCharacter.BP_RushCharacter_C|GetSoundSystem (Variables|Default|GetSlayer%20Character)) NonLocal _returnvalue_2 (Game|GetPlayerController 0) true NameOfKey))

(fn CompareActorHit
  (params (TargetHit :type Actor%20Object%20Reference))
  (if (not (Variables|Default|GetHitSomething))
    (Variables|Default|SetTargetHit TargetHit)
    (if (not (== (Variables|Default|GetTargetHit) self))
      (if (== (Variables|Default|GetTargetHit) (Components|GetOwner))
        (return false)
        (else
          (return true))))))