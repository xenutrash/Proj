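; Slayer spin attack gameplay ability that repeatedly damages bosses around the avatar and charges the Slayer's ultimate.
; Activation commits the cooldown and plays a montage, ending the ability when it finishes or is interrupted.
; On the server, an Attack.Special event starts a looping timer that sphere-traces for pawns.
; Hits accumulate uniquely in HitActors, which is never cleared here, and every Boss-tagged entry is damaged each tick.
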(event Custom|DoDamage
  (bind _returnvalue (Ability|GetAvatarActorfromActorInfo))
  (bind _returnvalue_2 (Transformation|GetActorLocation _returnvalue))
  (bind _outhits (Collision|MultiSphereTraceForObjects _returnvalue_2 _returnvalue_2 2.5e+02 (Utilities|Array|MakeArray "ObjectTypeQuery3") false 0 "ForDuration"))
  (CallFunction|ProcessHitActors _outhits))

(event Ability|EventActivateAbility
  (Ability|CommitAbilityCooldown false true)
  (|PlayMontageandWaitProxy "None" "/Game/Programming/Blueprints/Alchemist/PlaceHolders/AM_SmellingSalt.AM_SmellingSalt" 1.0 "None" true 1.0 0.0 false
    (:then
      (if (Networking|IsServer)
        (Ability|Tasks|WaitGameplayEvent "(TagName=\"Attack.Special\")" 0 true
          (:EventReceived
            (Utilities|Time|SetTimerbyEvent (delegate Custom|DoDamage) 0.5 true)))))
    (:OnCompleted
      (Ability|EndAbility :!label _label))
    (:OnBlendOut
      (goto _label))
    (:OnInterrupted
      (goto _label))
    (:OnCancelled
      (goto _label))))

(fn ProcessHitActors
  (params (Array :type Array%20of%20Hit%20Result%20Structures))
  (for _array_element Array
    (Utilities|Array|AddUnique (Variables|Default|GetHitActors) (.HitActor (Collision|BreakHitResult _array_element))))
  (for _array_element_2 (Variables|Default|GetHitActors)
    (if (Actor|ActorHasTag _array_element_2 "Boss")
      (bind _asbp_rush_character (Utilities|Casting|CastToBP_RushCharacter _array_element_2))
      (Default|TakeDamage _asbp_rush_character (Variables|Default|GetDamage))
      (bind _asbp_slayer (Utilities|Casting|CastToBP_Slayer (Ability|GetAvatarActorfromActorInfo)))
      (Default|ChargeUltimate _asbp_slayer (Variables|Default|GetUltCharge)))))