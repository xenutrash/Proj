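; BP_Slayer is the Slayer character Blueprint, mapping attack and dash events to Gameplay Ability System abilities.
; Basic, special and dash events activate main attack, spin attack and grappling hook abilities, with debug prints.
; Dash also starts a cooldown on player controller 0, regardless of activation success.
; BeginPlay adds max health, while the ultimate only prints after an attribute threshold check, activating no ability.
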(event EventOnHealthChanged
  (params (DeltaValue :type Float%20%28single-precision%29) (EventTags :type Gameplay%20Tag%20Container%20Structure%20%28by%20ref%29))
  (|CallParentFunction DeltaValue EventTags))

(event EventBeginPlay
  (CallFunction|AddtoMaxHealth 1e+02)
  (|CallParentFunction))

(event EventOnBasicAttack
  (Development|PrintString "Basic attack")
  (Abilities|TryActivateAbilitybyClass (Variables|Default|GetAbilitySystemComponent) "/Game/Programming/Blueprints/Slayer/MainAttack/GA_Slayer_MainAttack.GA_Slayer_MainAttack_C" true))

(event EventOnSpecialAttack
  (Development|PrintString "Specialattack")
  (Abilities|TryActivateAbilitybyClass (Variables|Default|GetAbilitySystemComponent) "/Game/Programming/Blueprints/Slayer/SpinAttack/GA_Slayer_SpinAttack.GA_Slayer_SpinAttack_C" true))

(event EventOnUltimateAttack
  (if (<= 1e+02 (.ReturnValue (Class|AbilitySystemBlueprintLibrary|GetFloatAttributeBasefromAbilitySystemComponent (Variables|Default|GetAbilitySystemComponent) "(AttributeName=\"UltimateCharge\",Attribute=/Script/Proj.RushAttributeSet:UltimateCharge,AttributeOwner=\"/Script/CoreUObject.Class'/Script/Proj.RushAttributeSet'\")")))
    (Development|PrintString "Ultiamte attack")))

(event EventOnDash
  (Development|PrintString "Dash")
  (Abilities|TryActivateAbilitybyClass (Variables|Default|GetAbilitySystemComponent) "/Game/Programming/Blueprints/Slayer/GrapplingHook/GA_Slayer_GrapplingHook.GA_Slayer_GrapplingHook_C" true)
  (bind _asbp_proj_player_controller (Utilities|Casting|CastToBP_ProjPlayerController (Game|GetPlayerController 0)))
  (Default|StartCooldownSpace _asbp_proj_player_controller))

(fn ConstructionScript
  (|CallParentFunction))