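; Gameplay ability for the Slayer's self-heal, restoring health over time during a heal montage.
; On activation it lowers max speed, forces the cooldown and plays the montage.
; On the server, the first Attack.Special gameplay event starts a looping timer that repeatedly adds HealAmount to current health.
; The montage completing, blending out or being interrupted or cancelled ends the ability, which restores speed and pauses the timer.
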(event Custom|Heal%20Over%20Time
  (Default|AddtoCurrentHealth (Variables|Default|GetSlayerCharacter) (Variables|Default|GetHealAmount)))

(event Ability|EventActivateAbility
  (bind _asbp_slayer (Utilities|Casting|CastToBP_Slayer (Ability|GetAvatarActorfromActorInfo)))
  (Variables|Default|SetSlayerCharacter _asbp_slayer)
  (Default|AddtoMaxSpeed (Variables|Default|GetSlayerCharacter) -3e+02)
  (Ability|CommitAbilityCooldown false true)
  (|PlayMontageandWaitProxy "None" "/Game/Animation/Slayer/Heal_white_Montage.Heal_white_Montage" 1.0 "None" true 1.0 0.0 false
    (:then
      (if (Networking|IsServer)
        (Ability|Tasks|WaitGameplayEvent "(TagName=\"Attack.Special\")" 0 true
          (:EventReceived
            (bind _returnvalue (Utilities|Time|SetTimerbyEvent (delegate Custom|Heal%20Over%20Time) 0.2 true))
            (Variables|Default|SetHealTimerHandle _returnvalue)))))
    (:OnCompleted
      (Ability|EndAbility :!label _label))
    (:OnBlendOut
      (goto _label))
    (:OnInterrupted
      (goto _label))
    (:OnCancelled
      (goto _label))))

(event Ability|EventOnEndAbility
  (params (bWasCancelled :type Boolean))
  (bind _healtimerhandle (Variables|Default|GetHealTimerHandle))
  (Default|AddtoMaxSpeed (Variables|Default|GetSlayerCharacter) 3e+02)
  (if (Utilities|Time|IsValidTimerHandle _healtimerhandle)
    (Utilities|Time|PauseTimerbyHandle _healtimerhandle)))