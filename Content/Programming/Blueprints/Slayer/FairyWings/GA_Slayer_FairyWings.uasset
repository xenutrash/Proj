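; Slayer's Fairy Wings ultimate ability, a targeted leap that teleports the character to a mouse-chosen spot and smashes the area.
; A jump montage plays and, on the Attack.Ultimate event, the locally controlled client spawns a mouse-location actor and waits for a confirm input event.
; Confirming teleports at current height, shows wings and, after a short delay, spawns smash VFX and sphere-traces pawns, damaging unique Boss-tagged BP_RushCharacters.
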(event Custom|TeleportCharacter
  (params (NewLocation :type Vector))
  (Transformation|SetActorLocation (Variables|Default|GetSlayer%20Character) NewLocation false true))

(event Custom|ImpactDamage
  (CallFunction|TeleporttoMouseLocation)
  (Default|ToggleWings (Variables|Default|GetSlayer%20Character) true)
  (Utilities|FlowControl|Delay 0.1)
  (Niagara|SpawnSystematLocation "/Game/Niagara/NS_SlayerUltimateSmash.NS_SlayerUltimateSmash" (Transformation|GetActorLocation (Variables|Default|GetSlayer%20Character)) "0, 0, 0" "1.000000,1.000000,1.000000" true true "AutoRelease")
  (bind _outhits (CallFunction|FindCharactersinRadius))
  (CallFunction|ProcessHitActors _outhits)
  (Ability|EndAbility))

(event Ability|EventActivateAbility
  (bind _asbp_slayer (Utilities|Casting|CastToBP_Slayer (Ability|GetAvatarActorfromActorInfo)))
  (Variables|Default|SetSlayer%20Character _asbp_slayer)
  (|PlayMontageandWaitProxy "None" "/Game/Animation/Slayer/Ult_Jump_Montage.Ult_Jump_Montage" 1.0 "None" true 1.0 0.0 false
    (:then
      (Ability|Tasks|WaitGameplayEvent "(TagName=\"Attack.Ultimate\")" 0 true
        (:EventReceived
          (if (Pawn|IsLocallyControlled (Variables|Default|GetSlayer%20Character))
            (bind _returnvalue (Game|SpawnActorfromClass "/Game/Programming/Blueprints/Slayer/FairyWings/BP_Slayer_MouseLocation.BP_Slayer_MouseLocation_C" (Transformation|GetActorTransform (Variables|Default|GetSlayer%20Character)) "Undefined" "MultiplyWithRoot" (Variables|Default|GetSlayer%20Character) (Variables|Default|GetSlayer%20Character)))
            (Variables|Default|SetMouse%20Position _returnvalue)
            (Ability|Tasks|WaitGameplayEvent "(TagName=\"Event.Input.Confirm\")" (Variables|Default|GetSlayer%20Character) true
              (:EventReceived
                (Development|PrintString "KALLAS")
                (CallFunction|ImpactDamage)))))))))

(fn TeleporttoMouseLocation
  (bind _mouse_position (Variables|Default|GetMouse%20Position))
  (bind _teleportlocation (Variables|/Game/Programming/Blueprints/Slayer/FairyWings/BP_Slayer_MouseLocation.BP_Slayer_MouseLocation_C|GetTeleportLocation _mouse_position))
  (Pawn|IsLocallyControlled
    (:True
      (CallFunction|TeleportCharacter (Math|Vector|MakeVector (.x _teleportlocation) (.y _teleportlocation) (.z (Transformation|GetActorLocation (Variables|Default|GetSlayer%20Character)))))
      (Actor|DestroyActor (Variables|Default|GetMouse%20Position)))))

(fn ProcessHitActors
  (params (Array :type Array%20of%20Hit%20Result%20Structures))
  (for _array_element Array
    (Utilities|Array|AddUnique (Variables|Default|GetHitActors) (.HitActor (Collision|BreakHitResult _array_element))))
  (for _array_element_2 (Variables|Default|GetHitActors)
    (if (Actor|ActorHasTag _array_element_2 "Boss")
      (bind _asbp_rush_character (Utilities|Casting|CastToBP_RushCharacter _array_element_2))
      (Default|TakeDamage _asbp_rush_character (Variables|Default|GetDamage)))))

(fn FindCharactersinRadius
  (bind _slayer_character (Variables|Default|GetSlayer%20Character))
  (bind _returnvalue (Transformation|GetActorLocation _slayer_character))
  (bind _outhits (Collision|MultiSphereTraceForObjects _returnvalue _returnvalue (Variables|Default|GetDamageRadius) (Utilities|Array|MakeArray "ObjectTypeQuery3") false 0 "ForDuration"))
  (return _outhits))