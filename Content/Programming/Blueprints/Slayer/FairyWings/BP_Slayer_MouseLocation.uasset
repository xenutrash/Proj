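; Cursor-following actor in the Slayer's FairyWings folder that tracks a valid teleport location for its owner.
; While active with a local player controller, Tick projects the mouse onto a horizontal plane below the owner and moves the actor there via SetLocationMulti.
; Two debug-drawn line traces then update TeleportLocation only over WorldDynamic "Ground" with no WorldStatic hit, otherwise keeping the last valid spot.
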(event Custom|SetLocation
  (params (NewLocation :type Vector))
  (CallFunction|SetLocationMulti NewLocation))

(event Custom|SetLocationMulti
  (params (NewLocation :type Vector))
  (Transformation|SetActorLocation NewLocation false true))

(event EventBeginPlay
  (bind _returnvalue (Components|GetOwner))
  (bind _returnvalue_2 (Game|GetInstigatorController _returnvalue))
  (Utilities|IsValid _returnvalue_2
    (:Is%20Valid
      (if (Pawn|IsLocalController _returnvalue_2)
        (bind _asplayer_controller (Utilities|Casting|CastToPlayerController _returnvalue_2))
        (Variables|Default|SetController _asplayer_controller)
        (Variables|Default|SetTeleportLocation (Transformation|GetActorLocation (Components|GetOwner)))))))

(event EventTick
  (params (DeltaSeconds :type Float%20%28single-precision%29))
  (Utilities|IsValid (Variables|Default|GetController)
    (:Is%20Valid
      (if (Variables|Default|GetActive)
        (CallFunction|CalculateMouseLocation)
        (CallFunction|SetLocation (Variables|Default|GetMouseLocation))
        (CallFunction|CheckTeleportAvailability)))))

(fn ConstructionScript)

(fn CalculateMouseLocation
  (bind _returnvalue (Components|GetOwner))
  (bind _controller (Variables|Default|GetController))
  (bind (_worldlocation _worlddirection) (Game|Player|ConvertMouseLocationToWorldSpace _controller))
  (bind _rootcomponent (Variables|/Script/Engine.Actor|GetRootComponent _returnvalue))
  (bind _returnvalue_2 (Transformation|GetWorldLocation _rootcomponent))
  (Variables|Default|SetMouseLocation (.Intersection (Class|KismetMathLibrary|LinePlaneIntersectionOriginNormal _worldlocation (+ _worldlocation (* _worlddirection 1e+04)) (Math|Vector|MakeVector (.x _returnvalue_2) (.y _returnvalue_2) (+ (.z _returnvalue_2) -1.5e+02)) "0.000000,0.000000,1.000000")))
  (return))

(fn CheckTeleportAvailability
  (bind (_start _end) (Utilities|CalculatePositionforCheck))
  (bind (_start_2 _end_2) (Utilities|CalculatePositionforCheck))
  (bind _outhit (Collision|LineTraceForObjects _start _end (Utilities|Array|MakeArray (Utilities|Enum|LiteralenumEObjectTypeQuery "ObjectTypeQuery2")) false 0 "ForDuration"))
  (Utilities|IsValid (.hitactor _outhit)
    (:Is%20Valid
      (if (Actor|ActorHasTag (.hitactor _outhit) "Ground")
        (bind _returnvalue (Collision|LineTraceForObjects _start_2 _end_2 (Utilities|Array|MakeArray (Utilities|Enum|LiteralenumEObjectTypeQuery "ObjectTypeQuery1")) false 0 "ForDuration"))
        (if (not _returnvalue)
          (Variables|Default|SetTeleportLocation (Variables|Default|GetMouseLocation)))))))