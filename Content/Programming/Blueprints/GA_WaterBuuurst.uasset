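; Gameplay ability that fires a fan-shaped burst of BP_ProjectileBase projectiles toward the cursor.
; On activation it rotates the avatar to face the Visibility hit under the instigator's cursor.
; A loop spawns ProjectileCount projectiles ahead of the avatar, yawing each by Offset plus an index-scaled Spread.
; EndAbility runs inside the loop body without any CommitAbility call, and OnEndAbility only prints a debug string.
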(event Ability|EventActivateAbility
  (bind _returnvalue (Ability|GetAvatarActorfromActorInfo))
  (bind _returnvalue_2 (Ability|GetAvatarActorfromActorInfo))
  (bind _returnvalue_3 (Transformation|GetActorRotation _returnvalue))
  (bind (_roll _pitch _yaw) (Math|Rotator|BreakRotator _returnvalue_3))
  (Transformation|SetActorRotation _returnvalue (Math|Rotator|FindLookatRotation (Transformation|GetActorLocation (Ability|GetAvatarActorfromActorInfo)) (.location (.HitResult (Game|Player|GetHitResultUnderCursorbyChannel (Pawn|GetLocalViewingPlayerController (Variables|/Script/Engine.Actor|GetInstigator (Ability|GetAvatarActorfromActorInfo))) "TraceTypeQuery1" true)))))
  (for _index (range 1 (Variables|Default|GetProjectileCount))
    (Game|SpawnActorfromClass "/Game/Programming/Blueprints/BP_ProjectileBase.BP_ProjectileBase_C" (Math|Transform|MakeTransform (+ (Transformation|GetActorLocation _returnvalue_2) (* (Transformation|GetActorForwardVector _returnvalue_2) "100.000000,100.000000,100.000000")) (Math|Rotator|CombineRotators (Math|Rotator|MakeRotator _roll _pitch (+ _yaw (Variables|Default|Getoffset))) (* (Math|Rotator|MakeRotator 0.0 0.0 (Variables|Default|GetSpread)) _index)) "1.000000,1.000000,1.000000") "Undefined" "MultiplyWithRoot" 0 0)
    (Ability|EndAbility)))

(event Ability|EventOnEndAbility
  (params (bWasCancelled :type Boolean))
  (Development|PrintString "Hello"))