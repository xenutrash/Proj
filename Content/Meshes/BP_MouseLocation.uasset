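; Mouse location marker actor that follows the owning player's cursor in the world, with a Niagara effect as its visual.
; BeginPlay caches the PlayerController from the owner's instigator and stores the owner's location as TeleportLocation.
; Tick deprojects the mouse and teleports the actor to where that ray meets a horizontal plane below the owner's root.
; Custom events show the Niagara effect and destroy the actor.
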(event Custom|Destory%20Mouse%20Actor
  (Actor|DestroyActor))

(event Custom|SetVisableOwningPlayerOnly
  (Rendering|SetVisibility (Variables|Default|GetNiagara) true false))

(event EventTick
  (params (DeltaSeconds :type Float%20%28single-precision%29))
  (bind _returnvalue (Components|GetOwner))
  (bind _as_player_controller (Variables|Default|GetAs%20Player%20Controller))
  (bind (_worldlocation _worlddirection) (Game|Player|ConvertMouseLocationToWorldSpace _as_player_controller))
  (bind _rootcomponent (Variables|/Script/Engine.Actor|GetRootComponent _returnvalue))
  (bind _returnvalue_2 (Transformation|GetWorldLocation _rootcomponent))
  (Utilities|IsValid (Variables|Default|GetAs%20Player%20Controller)
    (:Is%20Valid
      (Transformation|SetActorLocation (.Intersection (Class|KismetMathLibrary|LinePlaneIntersectionOriginNormal _worldlocation (+ _worldlocation (* _worlddirection 1e+04)) (Math|Vector|MakeVector (.x _returnvalue_2) (.y _returnvalue_2) (+ (.z _returnvalue_2) -1.5e+02)) "0.000000,0.000000,1.000000")) false true))))

(event EventBeginPlay
  (bind _asplayer_controller (Utilities|Casting|CastToPlayerController (Game|GetInstigatorController (Components|GetOwner))))
  (Variables|Default|SetAs%20Player%20Controller _asplayer_controller)
  (Variables|Default|SetTeleportLocation (Transformation|GetActorLocation (Components|GetOwner))))

(fn ConstructionScript)